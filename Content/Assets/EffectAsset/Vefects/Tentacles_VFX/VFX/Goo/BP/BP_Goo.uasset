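; BP_Goo is an interactive tentacle goo blob that wakes when the player enters its sphere or box sensor and can be exploded with E.
; Activation fires random line traces and spawns a BP_Spline to each hit on an "Anchorable" actor, while timelines animate the goo material's displacement and noise.
; Leaving removes the splines and reverses the animation; exploding also shrinks the mesh, spawns Niagara and sound, then destroys the actor.
; The construction script configures collision shape and the normal or dark variant.
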(event OnComponentBeginOverlap(Col)
  (params (OverlappedComponent :type Primitive%20Component%20Object%20Reference) (OtherActor :type Actor%20Object%20Reference) (OtherComp :type Primitive%20Component%20Object%20Reference) (OtherBodyIndex :type Integer) (bFromSweep :type Boolean) (SweepResult :type Hit%20Result%20Structure%20%28by%20ref%29))
  (bind _defaultsceneroot (Variables|Default|GetDefaultSceneRoot))
  (bind _goomatdyn (Variables|Default|GetgooMatDyn))
  (bind _checksradius (Variables|Default|GetchecksRadius))
  (bind _loopsafe (Variables|Default|GetloopSafe))
  (bind _returnvalue (Utilities|String|ToString(Integer) _loopsafe))
  (bind _returnvalue_2 (Transformation|GetWorldLocation _defaultsceneroot))
  (bind _returnvalue_3 (* _checksradius -1.0))
  (if (== OtherActor (Game|Player|GetPlayerPawn 0))
    (if (Variables|Default|GetcolCanActivate)
      (Variables|Default|SetcolCanActivate false)
      (if (not (Variables|Default|GetcolActivated))
        (Variables|Default|SetcolActivated true)
        (if (not (Variables|Default|GetdeactivateSeq))
          (Utilities|FlowControl|Sequence
            (:then_0
              (Variables|Default|SetloopForChecks true)
              (Variables|Default|SetnumberChecks (Math|Random|RandomIntegerinRange (Variables|Default|GetminChecks) (Variables|Default|GetmaxChecks)))
              (Variables|Default|SetcurrentTryCheckNumber 0)
              (Variables|Default|SetcurrentSuccessCheckNumber 0)
              (while (Variables|Default|GetloopForChecks)
                (if (>= (Variables|Default|GetcurrentTryCheckNumber) (Variables|Default|GetloopSafe))
                  (Variables|Default|SetloopForChecks false)
                  (if (== (Variables|Default|GetcurrentSuccessCheckNumber) 0)
                    (Development|PrintString (Utilities|String|Append "No surfaces found in " _returnvalue " tries!"))
                    (else
                      (Development|PrintString (Utilities|String|Append (Utilities|String|ToString(Integer) (Variables|Default|GetcurrentSuccessCheckNumber)) " surfaces found in " _returnvalue " tries!"))))
                  (else
                    (bind (_outhit _returnvalue_4) (Collision|LineTraceForObjects _returnvalue_2 (+ _returnvalue_2 (Math|Vector|MakeVector (Math|Random|RandomFloatinRange _returnvalue_3 _checksradius) (Math|Random|RandomFloatinRange _returnvalue_3 _checksradius) (Math|Random|RandomFloatinRange _returnvalue_3 _checksradius))) (Utilities|Array|MakeArray "ObjectTypeQuery1" "ObjectTypeQuery2") false 0 (Variables|Default|GetDraw%20Debug%20Type) true "(R=1.000000,G=0.000000,B=0.000000,A=1.000000)" "(R=0.000000,G=1.000000,B=0.000000,A=1.000000)" 2.0))
                    (Variables|Default|SetcurrentTryCheckNumber (+ (Variables|Default|GetcurrentTryCheckNumber) 1))
                    (if _returnvalue_4
                      (if (!= (.HitActor (Collision|BreakHitResult _outhit)) (Game|Player|GetPlayerPawn 0))
                        (if (Actor|ActorHasTag (.HitActor (Collision|BreakHitResult _outhit)) "Anchorable")
                          (if (>= (Variables|Default|GetcurrentSuccessCheckNumber) (Variables|Default|GetnumberChecks))
                            (Variables|Default|SetloopForChecks false)
                            (else
                              (Variables|Default|SetcurrentSuccessCheckNumber (+ (Variables|Default|GetcurrentSuccessCheckNumber) 1))
                              (bind _returnvalue_5 (Game|SpawnActorfromClass "/Game/Assets/EffectAsset/Vefects/Tentacles_VFX/VFX/Goo/BP/BP_Spline.BP_Spline_C" (Math|Transform|MakeTransform (Transformation|GetWorldLocation (Variables|Default|GetDefaultSceneRoot))) "Undefined" "OverrideRootScale" 0 0))
                              (Utilities|Array|Add (Variables|Default|GetspawnedActorsArray) _returnvalue_5)
                              (Default|SetPoints _returnvalue_5 "0, 0, 0" (.ImpactPoint (Collision|BreakHitResult _outhit)) (Variables|Default|GetGoo%20Type))))))))))
              (Variables|Default|SetcolCanActivate true))
            (:then_1
              (bind _newtrack_0 (Timeline|Timeline_0 Play)
                (:Update
                  (Rendering|Material|SetScalarParameterValue _goomatdyn "WPO Intensity" (Math|Float|Lerp 33.0 123.0 _newtrack_0) :!class /Script/Engine.MaterialInstanceDynamic)
                  (Rendering|Material|SetScalarParameterValue _goomatdyn "Noise Tex Pan Intensity" (Math|Float|Lerp -1.0 2.0 _newtrack_0) :!class /Script/Engine.MaterialInstanceDynamic)
                  (Rendering|Material|SetScalarParameterValue _goomatdyn "Noise Tex Scale Intensity" (Math|Float|Lerp 1.0 1.0 _newtrack_0) :!class /Script/Engine.MaterialInstanceDynamic)
                  (Rendering|Material|SetScalarParameterValue _goomatdyn "WPO Sine Intensity" (Math|Float|Lerp 2e+01 1e+01 _newtrack_0) :!class /Script/Engine.MaterialInstanceDynamic))))
            (:then_2
              (Input|EnableInput (Game|GetPlayerController 0)))
            (:then_3
              (Components|Activation|Activate (Variables|Default|GetPS_Goo_Up) false))
            (:then_4
              (Audio|SpawnSoundatLocation "/Game/Assets/EffectAsset/Vefects/Tentacles_VFX/Audio/SFX_Vefects_Tentacles_Body_Activation_01_Cue.SFX_Vefects_Tentacles_Body_Activation_01_Cue" (Transformation|GetActorLocation) "0, 0, 0" 1.0 1.0 0.0 0 0))))))))

(event OnComponentEndOverlap(Col)
  (params (OverlappedComponent :type Primitive%20Component%20Object%20Reference) (OtherActor :type Actor%20Object%20Reference) (OtherComp :type Primitive%20Component%20Object%20Reference) (OtherBodyIndex :type Integer))
  (bind _goomatdyn (Variables|Default|GetgooMatDyn))
  (bind _spawnedactorsarray (Variables|Default|GetspawnedActorsArray))
  (if (Variables|Default|GetcolCanActivate)
    (Variables|Default|SetcolCanActivate false)
    (if (Variables|Default|GetcolActivated)
      (Variables|Default|SetcolActivated false)
      (if (not (Variables|Default|GetdeactivateSeq))
        (Utilities|FlowControl|Sequence
          (:then_0
            (for _array_element (Variables|Default|GetspawnedActorsArray)
              (Default|Destroy _array_element))
            (bind _arrayindex (Utilities|Array|ReverseforEachLoop _spawnedactorsarray)
              (:LoopBody
                (Utilities|Array|RemoveIndex _spawnedactorsarray _arrayindex))
              (:Completed
                (Variables|Default|SetcolCanActivate true))))
          (:then_1
            (bind _newtrack_0 (Timeline|Timeline_0 Reverse)
              (:Update
                (Rendering|Material|SetScalarParameterValue _goomatdyn "WPO Intensity" (Math|Float|Lerp 33.0 123.0 _newtrack_0) :!class /Script/Engine.MaterialInstanceDynamic)
                (Rendering|Material|SetScalarParameterValue _goomatdyn "Noise Tex Pan Intensity" (Math|Float|Lerp -1.0 2.0 _newtrack_0) :!class /Script/Engine.MaterialInstanceDynamic)
                (Rendering|Material|SetScalarParameterValue _goomatdyn "Noise Tex Scale Intensity" (Math|Float|Lerp 1.0 1.0 _newtrack_0) :!class /Script/Engine.MaterialInstanceDynamic)
                (Rendering|Material|SetScalarParameterValue _goomatdyn "WPO Sine Intensity" (Math|Float|Lerp 2e+01 1e+01 _newtrack_0) :!class /Script/Engine.MaterialInstanceDynamic))))
          (:then_2
            (Input|DisableInput (Game|GetPlayerController 0)))
          (:then_3
            (Components|Activation|Deactivate (Variables|Default|GetPS_Goo_Up)))
          (:then_4
            (Audio|SpawnSoundatLocation "/Game/Assets/EffectAsset/Vefects/Tentacles_VFX/Audio/SFX_Vefects_Tentacles_Body_Activation_01_Cue.SFX_Vefects_Tentacles_Body_Activation_01_Cue" (Transformation|GetActorLocation) "0, 0, 0" 1.0 1.0 0.0 0 0)))))))

(event OnComponentBeginOverlap(ColCube)
  (params (OverlappedComponent :type Primitive%20Component%20Object%20Reference) (OtherActor :type Actor%20Object%20Reference) (OtherComp :type Primitive%20Component%20Object%20Reference) (OtherBodyIndex :type Integer) (bFromSweep :type Boolean) (SweepResult :type Hit%20Result%20Structure%20%28by%20ref%29))
  (bind _defaultsceneroot (Variables|Default|GetDefaultSceneRoot))
  (bind _goomatdyn (Variables|Default|GetgooMatDyn))
  (bind _checksradius (Variables|Default|GetchecksRadius))
  (bind _loopsafe (Variables|Default|GetloopSafe))
  (bind _returnvalue (Utilities|String|ToString(Integer) _loopsafe))
  (bind _returnvalue_2 (Transformation|GetWorldLocation _defaultsceneroot))
  (bind _returnvalue_3 (* _checksradius -1.0))
  (if (== OtherActor (Game|Player|GetPlayerPawn 0))
    (if (Variables|Default|GetcolCanActivate)
      (Variables|Default|SetcolCanActivate false)
      (if (not (Variables|Default|GetcolActivated))
        (Variables|Default|SetcolActivated true)
        (if (not (Variables|Default|GetdeactivateSeq))
          (Utilities|FlowControl|Sequence
            (:then_0
              (Variables|Default|SetloopForChecks true)
              (Variables|Default|SetnumberChecks (Math|Random|RandomIntegerinRange (Variables|Default|GetminChecks) (Variables|Default|GetmaxChecks)))
              (Variables|Default|SetcurrentTryCheckNumber 0)
              (Variables|Default|SetcurrentSuccessCheckNumber 0)
              (while (Variables|Default|GetloopForChecks)
                (if (>= (Variables|Default|GetcurrentTryCheckNumber) (Variables|Default|GetloopSafe))
                  (Variables|Default|SetloopForChecks false)
                  (if (== (Variables|Default|GetcurrentSuccessCheckNumber) 0)
                    (Development|PrintString (Utilities|String|Append "No surfaces found in " _returnvalue " tries!"))
                    (else
                      (Development|PrintString (Utilities|String|Append (Utilities|String|ToString(Integer) (Variables|Default|GetcurrentSuccessCheckNumber)) " surfaces found in " _returnvalue " tries!"))))
                  (else
                    (bind (_outhit _returnvalue_4) (Collision|LineTraceForObjects _returnvalue_2 (+ _returnvalue_2 (Math|Vector|MakeVector (Math|Random|RandomFloatinRange _returnvalue_3 _checksradius) (Math|Random|RandomFloatinRange _returnvalue_3 _checksradius) (Math|Random|RandomFloatinRange _returnvalue_3 _checksradius))) (Utilities|Array|MakeArray "ObjectTypeQuery1" "ObjectTypeQuery2") false 0 (Variables|Default|GetDraw%20Debug%20Type) true "(R=1.000000,G=0.000000,B=0.000000,A=1.000000)" "(R=0.000000,G=1.000000,B=0.000000,A=1.000000)" 2.0))
                    (Variables|Default|SetcurrentTryCheckNumber (+ (Variables|Default|GetcurrentTryCheckNumber) 1))
                    (if _returnvalue_4
                      (if (!= (.HitActor (Collision|BreakHitResult _outhit)) (Game|Player|GetPlayerPawn 0))
                        (if (Actor|ActorHasTag (.HitActor (Collision|BreakHitResult _outhit)) "Anchorable")
                          (if (>= (Variables|Default|GetcurrentSuccessCheckNumber) (Variables|Default|GetnumberChecks))
                            (Variables|Default|SetloopForChecks false)
                            (else
                              (Variables|Default|SetcurrentSuccessCheckNumber (+ (Variables|Default|GetcurrentSuccessCheckNumber) 1))
                              (bind _returnvalue_5 (Game|SpawnActorfromClass "/Game/Assets/EffectAsset/Vefects/Tentacles_VFX/VFX/Goo/BP/BP_Spline.BP_Spline_C" (Math|Transform|MakeTransform (Transformation|GetWorldLocation (Variables|Default|GetDefaultSceneRoot))) "Undefined" "OverrideRootScale" 0 0))
                              (Utilities|Array|Add (Variables|Default|GetspawnedActorsArray) _returnvalue_5)
                              (Default|SetPoints _returnvalue_5 "0, 0, 0" (.ImpactPoint (Collision|BreakHitResult _outhit)) (Variables|Default|GetGoo%20Type))))))))))
              (Variables|Default|SetcolCanActivate true))
            (:then_1
              (bind _newtrack_0 (Timeline|Timeline_0 Play)
                (:Update
                  (Rendering|Material|SetScalarParameterValue _goomatdyn "WPO Intensity" (Math|Float|Lerp 33.0 123.0 _newtrack_0) :!class /Script/Engine.MaterialInstanceDynamic)
                  (Rendering|Material|SetScalarParameterValue _goomatdyn "Noise Tex Pan Intensity" (Math|Float|Lerp -1.0 2.0 _newtrack_0) :!class /Script/Engine.MaterialInstanceDynamic)
                  (Rendering|Material|SetScalarParameterValue _goomatdyn "Noise Tex Scale Intensity" (Math|Float|Lerp 1.0 1.0 _newtrack_0) :!class /Script/Engine.MaterialInstanceDynamic)
                  (Rendering|Material|SetScalarParameterValue _goomatdyn "WPO Sine Intensity" (Math|Float|Lerp 2e+01 1e+01 _newtrack_0) :!class /Script/Engine.MaterialInstanceDynamic))))
            (:then_2
              (Input|EnableInput (Game|GetPlayerController 0)))
            (:then_3
              (Components|Activation|Activate (Variables|Default|GetPS_Goo_Up) false))
            (:then_4
              (Audio|SpawnSoundatLocation "/Game/Assets/EffectAsset/Vefects/Tentacles_VFX/Audio/SFX_Vefects_Tentacles_Body_Activation_01_Cue.SFX_Vefects_Tentacles_Body_Activation_01_Cue" (Transformation|GetActorLocation) "0, 0, 0" 1.0 1.0 0.0 0 0))))))))

(event OnComponentEndOverlap(ColCube)
  (params (OverlappedComponent :type Primitive%20Component%20Object%20Reference) (OtherActor :type Actor%20Object%20Reference) (OtherComp :type Primitive%20Component%20Object%20Reference) (OtherBodyIndex :type Integer))
  (bind _goomatdyn (Variables|Default|GetgooMatDyn))
  (bind _spawnedactorsarray (Variables|Default|GetspawnedActorsArray))
  (if (Variables|Default|GetcolCanActivate)
    (Variables|Default|SetcolCanActivate false)
    (if (Variables|Default|GetcolActivated)
      (Variables|Default|SetcolActivated false)
      (if (not (Variables|Default|GetdeactivateSeq))
        (Utilities|FlowControl|Sequence
          (:then_0
            (for _array_element (Variables|Default|GetspawnedActorsArray)
              (Default|Destroy _array_element))
            (bind _arrayindex (Utilities|Array|ReverseforEachLoop _spawnedactorsarray)
              (:LoopBody
                (Utilities|Array|RemoveIndex _spawnedactorsarray _arrayindex))
              (:Completed
                (Variables|Default|SetcolCanActivate true))))
          (:then_1
            (bind _newtrack_0 (Timeline|Timeline_0 Reverse)
              (:Update
                (Rendering|Material|SetScalarParameterValue _goomatdyn "WPO Intensity" (Math|Float|Lerp 33.0 123.0 _newtrack_0) :!class /Script/Engine.MaterialInstanceDynamic)
                (Rendering|Material|SetScalarParameterValue _goomatdyn "Noise Tex Pan Intensity" (Math|Float|Lerp -1.0 2.0 _newtrack_0) :!class /Script/Engine.MaterialInstanceDynamic)
                (Rendering|Material|SetScalarParameterValue _goomatdyn "Noise Tex Scale Intensity" (Math|Float|Lerp 1.0 1.0 _newtrack_0) :!class /Script/Engine.MaterialInstanceDynamic)
                (Rendering|Material|SetScalarParameterValue _goomatdyn "WPO Sine Intensity" (Math|Float|Lerp 2e+01 1e+01 _newtrack_0) :!class /Script/Engine.MaterialInstanceDynamic))))
          (:then_2
            (Input|DisableInput (Game|GetPlayerController 0)))
          (:then_3
            (Components|Activation|Deactivate (Variables|Default|GetPS_Goo_Up)))
          (:then_4
            (Audio|SpawnSoundatLocation "/Game/Assets/EffectAsset/Vefects/Tentacles_VFX/Audio/SFX_Vefects_Tentacles_Body_Activation_01_Cue.SFX_Vefects_Tentacles_Body_Activation_01_Cue" (Transformation|GetActorLocation) "0, 0, 0" 1.0 1.0 0.0 0 0)))))))

(event EventBeginPlay
  (Audio|Components|Audio|Play (Variables|Default|GetSFX) (Math|Random|RandomFloatinRange 0.0 18.0)))

(event Input|KeyboardEvents|E
  (params (Key :type Key%20Structure))
  (bind _goomatdyn (Variables|Default|GetgooMatDyn))
  (bind _spawnedactorsarray (Variables|Default|GetspawnedActorsArray))
  (:Pressed
    (if (Variables|Default|GetcolActivated)
      (Variables|Default|SetdeactivateSeq true)
      (if (not (Variables|Default|GetdestroySeqActive))
        (Variables|Default|SetdestroySeqActive true)
        (Utilities|FlowControl|Sequence
          (:then_0
            (Utilities|FlowControl|Sequence
              (:then_0
                (if (!= (Variables|Default|GetcurrentSuccessCheckNumber) 0)
                  (for _array_element (Variables|Default|GetspawnedActorsArray)
                    (Default|Destroy _array_element))
                  (bind _arrayindex (Utilities|Array|ReverseforEachLoop _spawnedactorsarray)
                    (:LoopBody
                      (Utilities|Array|RemoveIndex _spawnedactorsarray _arrayindex))
                    (:Completed
                      (Variables|Default|SetcolCanActivate true)))))
              (:then_1
                (Variables|Default|SetcurrentScale (Transformation|GetWorldScale (Variables|Default|GetSphere)))
                (bind (_direction _newtrack_0 _newtrack_1) (Timeline|Timeline_1 ReverseFromEnd)
                  (:Update
                    (Rendering|Material|SetScalarParameterValue _goomatdyn "WPO Intensity" (Math|Float|Lerp 0.0 123.0 _newtrack_0) :!class /Script/Engine.MaterialInstanceDynamic)
                    (Rendering|Material|SetScalarParameterValue _goomatdyn "Noise Tex Pan Intensity" (Math|Float|Lerp 0.0 2.0 _newtrack_0) :!class /Script/Engine.MaterialInstanceDynamic)
                    (Rendering|Material|SetScalarParameterValue _goomatdyn "Noise Tex Scale Intensity" (Math|Float|Lerp 1.0 1.0 _newtrack_0) :!class /Script/Engine.MaterialInstanceDynamic)
                    (Rendering|Material|SetScalarParameterValue _goomatdyn "WPO Sine Intensity" (Math|Float|Lerp 0.0 1e+01 _newtrack_0) :!class /Script/Engine.MaterialInstanceDynamic)
                    (Transformation|SetRelativeScale3D (Variables|Default|GetSphere) (* (Variables|Default|GetcurrentScale) _newtrack_1)))))))
          (:then_1
            (Utilities|FlowControl|Delay 0.17)
            (Niagara|SpawnSystematLocation (Variables|Default|GetGoo%20Explode%20Niagara) (Transformation|GetWorldLocation (Variables|Default|GetSphere)))
            (Utilities|FlowControl|Delay 0.1)
            (Actor|DestroyActor))
          (:then_2
            (Audio|SpawnSoundatLocation "/Game/Assets/EffectAsset/Vefects/Tentacles_VFX/Audio/SFX_Vefects_Tentacles_Body_Explode_01_Cue.SFX_Vefects_Tentacles_Body_Explode_01_Cue" (Transformation|GetActorLocation) "0, 0, 0" 1.0 1.0 0.0 0 0))
          (:then_3
            (Components|Activation|Deactivate (Variables|Default|GetSFX))))))))

(fn ConstructionScript
  (bind _blockcolcube (Variables|Default|GetblockColCube))
  (bind _ns_goo_drips (Variables|Default|GetNS_Goo_Drips))
  (bind _ns_goo_up (Variables|Default|GetNS_Goo_Up))
  (bind _blockcol (Variables|Default|GetblockCol))
  (Utilities|FlowControl|Sequence
    (:then_0
      (if (Variables|Default|GetcubeCol?)
        (Components|Box|SetBoxExtent _blockcolcube (Variables|Default|GetcubeColExtent) true)
        (Components|Box|SetBoxExtent (Variables|Default|GetColCube) (Variables|Default|GetsenseCubeColExtent) true)
        (Components|DestroyComponent _blockcol)
        (else
          (Components|Sphere|SetSphereRadius _blockcol (Variables|Default|GetblockColRadius) true)
          (Components|Sphere|SetSphereRadius (Variables|Default|GetCol) (Variables|Default|GetsenseColRadius) true)
          (Components|DestroyComponent _blockcolcube))))
    (:then_1
      (switch int (Variables|Default|GetGoo%20Type)
        (:Default
          (Variables|Default|SetGoo%20Material "/Game/Assets/EffectAsset/Vefects/Tentacles_VFX/VFX/Goo/Materials/MI_VFX_Goo_01.MI_VFX_Goo_01" :!label _label)
          (Class|NiagaraComponent|SetAsset _ns_goo_up "/Game/Assets/EffectAsset/Vefects/Tentacles_VFX/VFX/Goo/Particles/NS_Goo_Up.NS_Goo_Up" true)
          (Class|NiagaraComponent|SetAsset _ns_goo_drips "/Game/Assets/EffectAsset/Vefects/Tentacles_VFX/VFX/Goo/Particles/NS_Goo_Drips.NS_Goo_Drips" true)
          (Variables|Default|SetGoo%20Explode%20Niagara "/Game/Assets/EffectAsset/Vefects/Tentacles_VFX/VFX/Goo/Particles/NS_Goo_Explode.NS_Goo_Explode"))
        (:1
          (goto _label))
        (:2
          (Variables|Default|SetGoo%20Material "/Game/Assets/EffectAsset/Vefects/Tentacles_VFX/VFX/Goo/Materials/MI_VFX_Goo_Dark_02.MI_VFX_Goo_Dark_02")
          (Class|NiagaraComponent|SetAsset _ns_goo_up "/Game/Assets/EffectAsset/Vefects/Tentacles_VFX/VFX/Goo/Particles/NS_Goo_Up_Dark.NS_Goo_Up_Dark" true)
          (Class|NiagaraComponent|SetAsset _ns_goo_drips "/Game/Assets/EffectAsset/Vefects/Tentacles_VFX/VFX/Goo/Particles/NS_Goo_Drips_Dark.NS_Goo_Drips_Dark" true)
          (Variables|Default|SetGoo%20Explode%20Niagara "/Game/Assets/EffectAsset/Vefects/Tentacles_VFX/VFX/Goo/Particles/NS_Goo_Explode_Dark.NS_Goo_Explode_Dark")))
      (bind _returnvalue (Rendering|Material|CreateDynamicMaterialInstance (Variables|Default|GetGoo%20Material) "None" "None" :!class /Script/Engine.KismetMaterialLibrary))
      (Variables|Default|SetgooMatDyn _returnvalue)
      (Rendering|Material|SetMaterial (Variables|Default|GetSphere) 0 (Variables|Default|GetgooMatDyn))
      (Rendering|Material|SetScalarParameterValue (Variables|Default|GetgooMatDyn) "WPO Intensity" 33.0 :!class /Script/Engine.MaterialInstanceDynamic)
      (Rendering|Material|SetScalarParameterValue (Variables|Default|GetgooMatDyn) "Noise Tex Pan Intensity" -1.0 :!class /Script/Engine.MaterialInstanceDynamic)
      (Rendering|Material|SetScalarParameterValue (Variables|Default|GetgooMatDyn) "Noise Tex Scale Intensity" 1.0 :!class /Script/Engine.MaterialInstanceDynamic)
      (Rendering|Material|SetScalarParameterValue (Variables|Default|GetgooMatDyn) "WPO Sine Intensity" 2e+01 :!class /Script/Engine.MaterialInstanceDynamic))))