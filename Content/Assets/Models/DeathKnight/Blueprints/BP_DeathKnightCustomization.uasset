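; Death Knight character Blueprint that toggles modular armor and accessory pieces such as helmets, horns, shoulder armor, belts, skulls and knives.
; The Construction Script passes each skeletal mesh part and its boolean flag to a shared helper function.
; Enabled parts follow the main Mesh through Leader Pose and become visible, while disabled parts are hidden.
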(fn ConstructionScript
  (bind _mesh (Variables|Character|GetMesh))
  (CallFunction|SetMasterPoseComponent (Variables|Components|GetSK_Сollar) _mesh (Variables|Customization|GetDK_Сollar))
  (CallFunction|SetMasterPoseComponent (Variables|Components|GetSK_Visor) _mesh (Variables|Customization|GetDK_Visor))
  (CallFunction|SetMasterPoseComponent (Variables|Components|GetSK_Skull_Belt) _mesh (Variables|Customization|GetDK_Skull_Belt))
  (CallFunction|SetMasterPoseComponent (Variables|Components|GetSK_Armor_Belt) _mesh (Variables|Customization|GetDK_Armor_Belt))
  (CallFunction|SetMasterPoseComponent (Variables|Components|GetSK_Cloth) _mesh (Variables|Customization|GetDK_Cloth))
  (CallFunction|SetMasterPoseComponent (Variables|Components|GetSK_Element) _mesh (Variables|Customization|GetDK_Element))
  (CallFunction|SetMasterPoseComponent (Variables|Components|GetSK_Knife_Leg) _mesh (Variables|Customization|GetDK_Knife_Leg))
  (CallFunction|SetMasterPoseComponent (Variables|Components|GetSK_Skull_Leg) _mesh (Variables|Customization|GetDK_Skull_Leg))
  (CallFunction|SetMasterPoseComponent (Variables|Components|GetSK_Skull_Torso) _mesh (Variables|Customization|GetDK_Skull_Torso))
  (CallFunction|SetMasterPoseComponent (Variables|Components|GetSK_Helmet_1) _mesh (Variables|Customization|GetDK_Helmet_1))
  (CallFunction|SetMasterPoseComponent (Variables|Components|GetSK_Helmet_2) _mesh (Variables|Customization|GetDK_Helmet_2))
  (CallFunction|SetMasterPoseComponent (Variables|Components|GetSK_Helmet_2_Horns) _mesh (Variables|Customization|GetDK_Helmet_2_Horns))
  (CallFunction|SetMasterPoseComponent (Variables|Components|GetSK_Helmet_3) _mesh (Variables|Customization|GetDK_Helmet_3))
  (CallFunction|SetMasterPoseComponent (Variables|Components|GetSK_Helmet_3_Horns) _mesh (Variables|Customization|GetDK_Helmet_3_Horns))
  (CallFunction|SetMasterPoseComponent (Variables|Default|GetSK_Helmet_4) _mesh (Variables|Customization|GetDK_Helmet_4))
  (CallFunction|SetMasterPoseComponent (Variables|Components|GetSK_Knife_Arm) _mesh (Variables|Customization|GetDK_Knife_Arm))
  (CallFunction|SetMasterPoseComponent (Variables|Components|GetSK_Arm_Armor) _mesh (Variables|Customization|GetDK_Arm_Armor))
  (CallFunction|SetMasterPoseComponent (Variables|Components|GetSK_Skull_Shoulder) _mesh (Variables|Customization|GetDK_Skull_Shoulder))
  (CallFunction|SetMasterPoseComponent (Variables|Components|GetSK_Shoulder_Armor_3) _mesh (Variables|Customization|GetDK_Shoulder_Armor_3))
  (CallFunction|SetMasterPoseComponent (Variables|Components|GetSK_Shoulder_Armor_2) _mesh (Variables|Customization|GetDK_Shoulder_Armor_2))
  (CallFunction|SetMasterPoseComponent (Variables|Default|GetSK_Shoulder_Armor_1) _mesh (Variables|Customization|GetDK_Shoulder_Armor_1))
  (CallFunction|SetMasterPoseComponent (Variables|Components|GetSK_Knife_Shoulder) _mesh (Variables|Customization|GetDK_Knife_Shoulder)))

(fn SetMasterPoseComponent
  (params (Target :type Skinned%20Mesh%20Component%20Object%20Reference) (NewMasterBoneComponent :type Skinned%20Mesh%20Component%20Object%20Reference) (Condition :type Boolean))
  (if Condition
    (Components|SkinnedMesh|SetLeaderPoseComponent Target NewMasterBoneComponent false false)
    (Rendering|SetVisibility Target true false)
    (else
      (Rendering|SetVisibility Target false false)))
  (return))