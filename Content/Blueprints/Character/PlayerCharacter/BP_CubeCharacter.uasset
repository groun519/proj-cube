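; BP_CubeCharacter is the player character, handling class setup, overhead UI and cosmetic ability effects.
; BeginPlay retries until PlayerState is valid, then picks Ranger or Healer from hardcoded player names and grants abilities.
; Events drive timed weapon swaps, pose-copied trails, dynamic-material emissive flashes and a Motion Warping facing target.
; Tick feeds attribute values to the health bar, while box overlaps fade actors in and out through BI_FadeInterface.
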(event OnComponentBeginOverlap(Box)
  (params (OverlappedComponent :type Primitive%20Component%20Object%20Reference) (OtherActor :type Actor%20Object%20Reference) (OtherComp :type Primitive%20Component%20Object%20Reference) (OtherBodyIndex :type Integer) (bFromSweep :type Boolean) (SweepResult :type Hit%20Result%20Structure%20%28by%20ref%29))
  ;[1 1 1] FadeActor
  (if (Utilities|DoesObjectImplementInterface OtherActor "/Game/Blueprints/FadeActor/BI_FadeInterface.BI_FadeInterface_C")
    (Class|BIFadeInterface|FadeOut(Message) OtherActor)))

(event OnComponentEndOverlap(Box)
  (params (OverlappedComponent :type Primitive%20Component%20Object%20Reference) (OtherActor :type Actor%20Object%20Reference) (OtherComp :type Primitive%20Component%20Object%20Reference) (OtherBodyIndex :type Integer))
  ;[1 1 1] FadeActor
  (if (Utilities|DoesObjectImplementInterface OtherActor "/Game/Blueprints/FadeActor/BI_FadeInterface.BI_FadeInterface_C")
    (Class|BIFadeInterface|Fadein(Message) OtherActor)))

(event Custom|EmissiveCharacter
  (params (Color :type Linear%20Color%20Structure) (Emissive :type Float%20%28double-precision%29) (Time :type Float%20%28double-precision%29))
  ;[1 1 1] Character Emissive Event
  (Utilities|FlowControl|Sequence
    (:then_0
      (for (_array_element _array_index) (Rendering|Material|GetMaterials (Variables|Character|GetMesh))
        (bind _returnvalue (Rendering|Material|CreateDynamicMaterialInstance (Variables|Character|GetMesh) _array_index _array_element "None" :!class /Script/Engine.PrimitiveComponent))
        (Utilities|Array|Add (Variables|Default|GetMIDArr) _returnvalue)
        (Rendering|Material|SetVectorParameterValue _returnvalue "Color" Color :!class /Script/Engine.MaterialInstanceDynamic)
        (Rendering|Material|SetScalarParameterValue _returnvalue "Emissive" Emissive :!class /Script/Engine.MaterialInstanceDynamic))
      (Utilities|FlowControl|Delay Time)
      (for _array_element_2 (Variables|Default|GetMIDArr)
        (Rendering|Material|SetVectorParameterValue :self _array_element_2 :ParameterName "Color" :!class /Script/Engine.MaterialInstanceDynamic)
        (Rendering|Material|SetScalarParameterValue _array_element_2 "Emissive" 0.0 :!class /Script/Engine.MaterialInstanceDynamic)))))

(event Custom|SetAbilityWeaponMesh
  (params (NewMesh :type Skeletal%20Mesh%20Object%20Reference) (Duration :type Float%20%28single-precision%29))
  ;[1 1 1] Set Ability Weapon Mesh (비용 문제로 폐기. 오른쪽 3개 노드만 비슷하게 가져가면 됨.)
  (bind _ascombat_interface (Utilities|Casting|CastToCombatInterface self))
  (Class|CombatInterface|ChangeWeapon _ascombat_interface NewMesh)
  (Utilities|FlowControl|Delay Duration)
  (Class|CombatInterface|ResetWeapon _ascombat_interface))

(event Custom|SpawnTrail
  (params (Color :type Linear%20Color%20Structure))
  ;[1 1 1] Spawn Trail Event
  (bind _returnvalue (Game|SpawnActorfromClass "/Game/Blueprints/Character/PlayerCharacter/BP_CharacterTrail.BP_CharacterTrail_C" (Transformation|GetWorldTransform (Variables|Character|GetMesh)) "AlwaysSpawn" "MultiplyWithRoot" 0 0))
  (Default|CopyPose _returnvalue (Variables|Character|GetMesh))
  (Default|SetColor _returnvalue Color))

(event Custom|UpdateFacingTarget
  (params (Target :type Vector%20%28by%20ref%29))
  ;[1 1 1] Facing Target
  (Class|MotionWarpingComponent|AddorUpdateWarpTargetfromLocation (Variables|Default|GetMotionWarping) "FacingTarget" Target))

(event EventBeginPlay
  ;[1 1 1] 플레이어 이름 설정 및 텍스트로 띄우기
  (Utilities|FlowControl|Delay 0.2 :!label _label)
  (if (Utilities|IsValid (Variables|Default|GetPlayerState))
    (bind _asoverhead_widget (Utilities|Casting|CastToOverheadWidget (UserInterface|GetUserWidgetObject (Variables|Default|GetOverheadWidget))))
    (bind _returnvalue (Class|OverheadWidget|ShowPlayerName _asoverhead_widget self))
    ;[1 1 1] 클래스 설정
    (if (Utilities|Enum|Equal(Enum) _returnvalue "Beom")
      (Variables|Default|SetCharacterClass "Ranger")
      (Class|CubeCharacterBase|AddCharacterAbilities)
      (elif (Utilities|Enum|Equal(Enum) _returnvalue "poppy04")
        (Variables|Default|SetCharacterClass "Healer")
        (Class|CubeCharacterBase|AddCharacterAbilities)
        (else
          (Variables|Default|SetCharacterClass "Ranger")
          (Class|CubeCharacterBase|AddCharacterAbilities)
          (Class|CombatInterface|SetBaseWeapon "/Game/Blueprints/AbilitySystem/Character/Abilities/FireStaff/MagicStick1.MagicStick1" (Math|Transform|MakeTransform "0.000000,4.000000,-30.000000" "0, 0, 0" "0.500000,0.500000,0.500000")))))
    (else
      (goto _label))))

(event EventTick
  (params (DeltaSeconds :type Float%20%28single-precision%29))
  ;[1 1 1] HP Bar
  (Utilities|FlowControl|Sequence
    (:then_0
      (bind _aswbp_player_health_bar (Utilities|Casting|CastToWBP_PlayerHealthBar (UserInterface|GetUserWidgetObject (Variables|Default|GetHealthBar))))
      (Default|SetPercent _aswbp_player_health_bar (.ReturnValue (Ability|Attribute|GetFloatAttribute self "(AttributeName=\"Health\",Attribute=/Script/P_Cube.CubeAttributeSet:Health,AttributeOwner=\"/Script/CoreUObject.Class'/Script/P_Cube.CubeAttributeSet'\")")) (.ReturnValue (Ability|Attribute|GetFloatAttribute self "(AttributeName=\"MaxHealth\",Attribute=/Script/P_Cube.CubeAttributeSet:MaxHealth,AttributeOwner=\"/Script/CoreUObject.Class'/Script/P_Cube.CubeAttributeSet'\")"))))))

(fn ConstructionScript)