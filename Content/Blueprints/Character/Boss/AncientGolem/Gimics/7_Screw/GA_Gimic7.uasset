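; Gameplay ability for the Ancient Golem boss's seventh gimmick, a Screw attack aimed at a nearby player.
; On activation it plays the fourth attack montage from the golem with reduced root-motion translation and starts a wait for that montage's gameplay event.
; The wait's immediate output, not the event, finds the nearest player and spawns a Screw hitbox at the golem, yawed toward them.
; The graph never ends the ability.
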(event Ability|EventActivateAbility
  (bind _returnvalue (Ability|GetAvatarActorfromActorInfo))
  (bind _asbp_ancient_golem (Utilities|Casting|CastToBP_AncientGolem (Ability|GetAvatarActorfromActorInfo)))
  (Variables|Default|SetBPAncientGolem _asbp_ancient_golem)
  (bind _returnvalue_2 (Class|CombatInterface|GetAttackMontages(Message) (Ability|GetAvatarActorfromActorInfo)))
  (for (_array_element _array_index) _returnvalue_2
    (if (== _array_index 3)
      (bind _output_get (Variables|Default|SetTaggedMontage _array_element))
      (|PlayMontageandWaitProxy "None" (.Montage (Utilities|Struct|BreakTaggedMontage _output_get)) 1.0 "None" true 0.15 0.0 false
        (:then
          (Ability|Tasks|WaitGameplayEvent (.MontageTag (Utilities|Struct|BreakTaggedMontage _output_get)) 0 true
            (:then
              (bind _returnvalue_3 (Class|CubeActiveSkill|FindNearestActorsbyTag "Player" (Transformation|GetActorLocation (Ability|GetAvatarActorfromActorInfo)) 1e+03 1 false))
              (for _array_element_2 _returnvalue_3
                (Class|CubeActiveSkill|SpawnHitBox "Screw" "ScrewDamage" (Math|Transform|MakeTransform (Transformation|GetActorLocation _returnvalue) (Math|Rotator|MakeRotator 0.0 0.0 (.Yaw (Math|Rotator|BreakRotator (Math|Rotator|FindLookatRotation (Transformation|GetActorLocation (Ability|GetAvatarActorfromActorInfo)) (Transformation|GetActorLocation _array_element_2)))))) false 0 _returnvalue)))))))))

(event Ability|EventOnEndAbility
  (params (bWasCancelled :type Boolean)))