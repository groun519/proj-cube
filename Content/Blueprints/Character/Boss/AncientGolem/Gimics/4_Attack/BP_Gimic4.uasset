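; BP_Gimic4 is a short-lived hitbox actor for an Ancient Golem boss attack gimmick.
; On BeginPlay it configures its Box as a hitbox, snaps onto the actor returned by GetInstigatorPlayer and spawns a fixed-size warning square.
; Timed delays enable overlap events on the box partway through the warning, then destroy the actor.
; Overlap response is not handled in this graph.
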(event EventBeginPlay
  (Class|CubeHitbox|SetHitboxCollision (Variables|Default|GetBox))
  (Transformation|AttachActorToActor (Class|CubeHitActor|GetInstigatorPlayer) "None" "SnapToTarget" "SnapToTarget" "SnapToTarget" true)
  (Class|CubeHitActor|SpawnWarningSquare 513.0 12.3 2.6 1.35)
  (Utilities|FlowControl|Delay 0.4)
  (Variables|/Script/Engine.PrimitiveComponent|SetbGenerateOverlapEvents (Variables|Default|GetBox) true)
  (Utilities|FlowControl|Delay 1.0)
  (Actor|DestroyActor))

(fn ConstructionScript)