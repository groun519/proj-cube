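; Gameplay ability for the Ancient Golem boss's fourth gimmick attack, apparently a dash.
; Plays the fourth attack montage with reduced root motion and, on its tagged event, flashes the body emissive and spawns a dash hitbox yawed toward the nearest player in range.
; Inside that player loop, four chained montage events spawn progressively brighter trails; the last ends the ability after a short delay, so it never ends without a target.
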(event Ability|EventActivateAbility
  (bind _returnvalue (Ability|GetAvatarActorfromActorInfo))
  (bind _asbp_ancient_golem (Utilities|Casting|CastToBP_AncientGolem (Ability|GetAvatarActorfromActorInfo)))
  (Variables|Default|SetBPAncientGolem _asbp_ancient_golem)
  (bind _returnvalue_2 (Class|CombatInterface|GetAttackMontages(Message) (Ability|GetAvatarActorfromActorInfo)))
  (for (_array_element _array_index) _returnvalue_2
    (if (== _array_index 3)
      (bind _output_get (Variables|Default|SetTaggedMontage _array_element))
      (|PlayMontageandWaitProxy "None" (.Montage (Utilities|Struct|BreakTaggedMontage _output_get)) 1.0 "None" true 0.15 0.0 false
        (:then
          (Ability|Tasks|WaitGameplayEvent (.MontageTag (Utilities|Struct|BreakTaggedMontage _output_get)) 0 true
            (:EventReceived
              (Default|EmissiveCharacter (Variables|Default|GetBPAncientGolem) "(R=0.000000,G=31.672691,B=100.000000,A=1.000000)" 1e+03 0.25)
              (Utilities|FlowControl|Delay 0.25)
              (Default|EmissiveCharacter (Variables|Default|GetBPAncientGolem) "(R=0.000000,G=31.672691,B=100.000000,A=1.000000)" 5e+01 0.5)
              (bind _returnvalue_3 (Class|CubeActiveSkill|FindNearestActorsbyTag "Player" (Transformation|GetActorLocation (Ability|GetAvatarActorfromActorInfo)) 1e+03 1 false))
              (for _array_element_2 _returnvalue_3
                (Class|CubeActiveSkill|SpawnHitBox "DashHitBox" "DashDamage" (Math|Transform|MakeTransform (Transformation|GetActorLocation _returnvalue) (Math|Rotator|MakeRotator 0.0 0.0 (.Yaw (Math|Rotator|BreakRotator (Math|Rotator|FindLookatRotation (Transformation|GetActorLocation (Ability|GetAvatarActorfromActorInfo)) (Transformation|GetActorLocation _array_element_2)))))) false _returnvalue 0)
                ;[1 1 1] 트레일 생성
                (Ability|Tasks|WaitGameplayEvent "(TagName=\"Event.Montage.Gimic4.Trail.1\")" 0 true
                  (:EventReceived
                    (Default|SpawnTrail (Variables|Default|GetBPAncientGolem) "(R=2.000000,G=0.386304,B=0.331250,A=1.000000)")
                    (Ability|Tasks|WaitGameplayEvent "(TagName=\"Event.Montage.Gimic4.Trail.2\")" 0 true
                      (:EventReceived
                        (Default|SpawnTrail (Variables|Default|GetBPAncientGolem) "(R=5.000000,G=0.829774,B=0.687500,A=1.000000)")
                        (Ability|Tasks|WaitGameplayEvent "(TagName=\"Event.Montage.Gimic4.Trail.3\")" 0 true
                          (:EventReceived
                            (Default|SpawnTrail (Variables|Default|GetBPAncientGolem) "(R=10.000000,G=1.251412,B=0.952940,A=1.000000)")
                            (Ability|Tasks|WaitGameplayEvent "(TagName=\"Event.Montage.Gimic4.Trail.4\")" 0 true
                              (:EventReceived
                                (Default|SpawnTrail (Variables|Default|GetBPAncientGolem) "(R=15.000000,G=1.877118,B=1.429410,A=1.000000)")
                                (Utilities|FlowControl|Delay 0.5)
                                (Ability|EndAbility)))))))))))))))))

(event Ability|EventOnEndAbility
  (params (bWasCancelled :type Boolean)))