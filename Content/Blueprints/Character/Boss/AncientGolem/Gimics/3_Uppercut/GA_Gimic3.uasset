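; Gameplay ability for the Ancient Golem boss's third gimmick, an uppercut attack aimed at a nearby player.
; It plays the avatar's third attack montage and waits for that montage's gameplay event tag.
; On that event it searches for the nearest player, turns the boss toward them through CombatInterface, and spawns the uppercut hitbox in front of the boss, lowered and yawed toward the target.
; The ability ends on the Gimic3 end montage event.
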(event Ability|EventActivateAbility
  (bind _returnvalue (Class|CombatInterface|GetAttackMontages(Message) (Ability|GetAvatarActorfromActorInfo)))
  (for (_array_element _array_index) _returnvalue
    (if (== _array_index 2)
      (bind _output_get (Variables|Default|SetTaggedMontage _array_element))
      (|PlayMontageandWaitProxy "None" (.Montage (Utilities|Struct|BreakTaggedMontage _output_get)) 1.0 "None" true 1.0 0.0 false
        (:then
          (Ability|Tasks|WaitGameplayEvent (.MontageTag (Utilities|Struct|BreakTaggedMontage _output_get)) 0 true
            (:EventReceived
              ;[1 1 1] 플레이어 탐색
              (bind _returnvalue_2 (Class|CubeActiveSkill|FindNearestActorsbyTag "Player" (Transformation|GetActorLocation (Ability|GetAvatarActorfromActorInfo)) 5e+03 1 true))
              (for _array_element_2 _returnvalue_2
                ;[1 1 1] 대상이 유효하다면
                (Utilities|IsValid _array_element_2
                  (:Is%20Valid
                    ;[1 1 1] 방향 바라보기
                    (Variables|Default|SetHitboxLocation (+ (* (Math|Vector|Normalize (Math|Rotator|GetRotationXVector (Math|Rotator|MakeRotator 0.0 0.0 (.Yaw (Math|Rotator|BreakRotator (Math|Rotator|FindLookatRotation (Transformation|GetActorLocation (Ability|GetAvatarActorfromActorInfo)) (Transformation|GetActorLocation _array_element_2))))))) 3.5e+02) (Transformation|GetActorLocation (Ability|GetAvatarActorfromActorInfo))))
                    (bind _ascombat_interface (Utilities|Casting|CastToCombatInterface (Ability|GetAvatarActorfromActorInfo)))
                    (Class|CombatInterface|UpdateFacingTarget _ascombat_interface (Transformation|GetActorLocation _array_element_2))
                    (Class|CubeActiveSkill|SpawnHitBox "UppercutHitbox" "UppercutDamage" (Math|Transform|MakeTransform (- (+ (* (Math|Vector|Normalize (Math|Rotator|GetRotationXVector (Math|Rotator|MakeRotator 0.0 0.0 (.Yaw (Math|Rotator|BreakRotator (Math|Rotator|FindLookatRotation (Transformation|GetActorLocation (Ability|GetAvatarActorfromActorInfo)) (Transformation|GetActorLocation _array_element_2))))))) 3.5e+02) (Transformation|GetActorLocation (Ability|GetAvatarActorfromActorInfo))) "0.000000,0.000000,200.000000") (Math|Rotator|MakeRotator 0.0 0.0 (.Yaw (Math|Rotator|BreakRotator (Math|Rotator|FindLookatRotation (Transformation|GetActorLocation (Ability|GetAvatarActorfromActorInfo)) (Transformation|GetActorLocation _array_element_2)))))) false 0 0)
                    (Ability|Tasks|WaitGameplayEvent "(TagName=\"Event.Montage.Gimic3.End\")" 0 true
                      (:EventReceived
                        (Ability|EndAbility)))))))))))))