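; Timed hitbox actor for the Ancient Golem boss's Gimic 3 (Uppercut) attack, with a growing indicator before the hit.
; BeginPlay configures the Box collision and offsets it along Y.
; Tick grows the flattened PullObj toward twice the Box's X/Y scale over MaxTime, then enables Box overlap events and destroys the actor after a 0.1-second delay.
; A PullObj movement node is left unconnected.
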(event EventBeginPlay
  (Class|CubeHitbox|SetHitboxCollision (Variables|Default|GetBox))
  (Variables|Default|SetYawRot 0.0)
  (Variables|Default|SetRollRot 0.0)
  (Variables|Default|SetPitchRot 0.0)
  (Variables|Default|SetPullObjStartLoc (Variables|/Script/Engine.SceneComponent|GetRelativeLocation (Variables|Default|GetPullObj)))
  (Transformation|SetRelativeLocation (Variables|Default|GetBox) (+ (Transformation|GetWorldLocation (Variables|Default|GetBox)) "0.000000,500.000000,0.000000") false true))

(event EventTick
  (params (DeltaSeconds :type Float%20%28single-precision%29))
  (bind _box (Variables|Default|GetBox))
  (bind _returnvalue (Transformation|GetWorldScale _box))
  (if (> (Variables|Default|GetTime) (Variables|Default|GetMaxTime))
    (Variables|/Script/Engine.PrimitiveComponent|SetbGenerateOverlapEvents (Variables|Default|GetBox) true)
    (Utilities|FlowControl|Delay 0.1)
    (Actor|DestroyActor)
    (else
      (Variables|Default|SetTime (+ (Variables|Default|GetTime) DeltaSeconds))
      (Transformation|SetWorldScale3D (Variables|Default|GetPullObj) (Math|Vector|MakeVector (* (Variables|Default|GetTime) (/ (* (.x _returnvalue) 2.0) (Variables|Default|GetMaxTime))) (* (Variables|Default|GetTime) (/ (* (.y _returnvalue) 2.0) (Variables|Default|GetMaxTime))) 0.1)))))

(fn ConstructionScript)