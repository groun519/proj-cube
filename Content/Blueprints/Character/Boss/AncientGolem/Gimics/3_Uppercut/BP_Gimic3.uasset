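; BP_Gimic3 is the uppercut gimmick hazard for the Ancient Golem boss: a telegraphed box area that strikes after a delay.
; On BeginPlay it sets up the Box hitbox collision and spawns a warning square sized from the box extent.
; When the two-second warning ends, it enables overlap events on the box for a brief window, then destroys itself.
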(event EventBeginPlay
  (bind _box (Variables|Default|GetBox))
  (bind _returnvalue (Components|Box|GetScaledBoxExtent _box))
  (bind (_x _y) (Math|Vector|BreakVector _returnvalue))
  (Class|CubeHitbox|SetHitboxCollision (Variables|Default|GetBox))
  (Class|CubeHitActor|SpawnWarningSquare 0.0 0.0 (/ _x 5e+01) (/ _y 5e+01) 2.0)
  (Utilities|FlowControl|Delay 2.0)
  (Variables|/Script/Engine.PrimitiveComponent|SetbGenerateOverlapEvents (Variables|Default|GetBox) true)
  (Utilities|FlowControl|Delay 0.05)
  (Actor|DestroyActor))

(fn ConstructionScript)