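; BP_Gimic7 is an Ancient Golem boss gimmick that runs as a timed area with a growing indicator.
; Each Tick scales the flat Sec component with elapsed time, sized from the ProceduralMesh scale and three times longer in X than Y.
; Past MaxTime, it turns on the mesh's overlap events and destroys itself after a brief delay.
; The procedural mesh and hitbox collision setup is disconnected and never runs.
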(event EventBeginPlay)

(event EventTick
  (params (DeltaSeconds :type Float%20%28single-precision%29))
  (if (> (Variables|Default|GetTime) (Variables|Default|GetMaxTime))
    (Variables|/Script/Engine.PrimitiveComponent|SetbGenerateOverlapEvents (Variables|Default|GetProceduralMesh) true)
    (Utilities|FlowControl|Delay 0.1)
    (Actor|DestroyActor)
    (else
      (Variables|Default|SetTime (+ (Variables|Default|GetTime) DeltaSeconds))
      (Transformation|SetWorldScale3D (Variables|Default|GetSec) (Math|Vector|MakeVector (* (* (Variables|Default|GetTime) (/ (* (.x (Transformation|GetWorldScale (Variables|Default|GetProceduralMesh))) 1.17) (Variables|Default|GetMaxTime))) 3.0) (* (Variables|Default|GetTime) (/ (* (.x (Transformation|GetWorldScale (Variables|Default|GetProceduralMesh))) 1.17) (Variables|Default|GetMaxTime))) 0.1)))))

(fn ConstructionScript)