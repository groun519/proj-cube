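; BP_Gimic4 is the hitbox actor for the Ancient Golem boss's dash gimmick.
; On BeginPlay it sets up box collision, snaps onto the actor returned by GetInstigatorPlayer and spawns a square ground warning.
; After a short telegraph it spawns a Niagara wind effect behind itself and enables the box's overlap events, then destroys itself a second later.
; No overlap response is defined in this graph.
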(event EventBeginPlay
  (Class|CubeHitbox|SetHitboxCollision (Variables|Default|GetBox))
  (Transformation|AttachActorToActor (Class|CubeHitActor|GetInstigatorPlayer) "None" "SnapToTarget" "SnapToTarget" "SnapToTarget" true)
  (Class|CubeHitActor|SpawnWarningSquare 513.0 12.3 2.6 0.75)
  (Utilities|FlowControl|Delay 0.5)
  (Utilities|FlowControl|Delay 0.2)
  (Niagara|SpawnSystematLocation "/Game/Blueprints/Character/Boss/AncientGolem/BossAsset/NS_BossDash_Wind.NS_BossDash_Wind" (+ (* (Transformation|GetActorForwardVector) -7.5e+02) (Transformation|GetActorLocation)) (Transformation|GetActorRotation) "3.000000,3.000000,3.000000")
  (Variables|/Script/Engine.PrimitiveComponent|SetbGenerateOverlapEvents (Variables|Default|GetBox) true)
  (Utilities|FlowControl|Delay 1.0)
  (Actor|DestroyActor))

(fn ConstructionScript)