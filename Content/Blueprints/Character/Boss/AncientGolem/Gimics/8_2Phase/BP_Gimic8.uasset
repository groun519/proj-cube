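; BP_Gimic8 is a short-lived Ancient Golem phase 2 boss gimmick that telegraphs and then fires a circular shockwave.
; On BeginPlay it registers its sphere as the hitbox and spawns a warning circle scaled from that sphere's radius.
; After a delay slightly longer than the warning, it enables overlap events, spawns the shockwave Niagara effect and destroys itself moments later, leaving only a brief hit window.
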(event EventBeginPlay
  ;[1 1 1] 히트박스 지정
  (Class|CubeHitbox|SetHitboxCollision (Variables|Default|GetSphere))
  ;[1 1 1] 위험 범위 이펙트 생성
  (Class|CubeHitActor|SpawnWarningCircle (/ (Components|Sphere|GetScaledSphereRadius (Variables|Default|GetSphere)) 5e+01) 2.0)
  ;[1 1 1] 콜리전 충돌 끄기
  (Utilities|FlowControl|Delay 2.3)
  (Variables|/Script/Engine.PrimitiveComponent|SetbGenerateOverlapEvents (Variables|Default|GetSphere) true)
  ;[1 1 1] 이펙트 생성 후 디스트로이
  (Niagara|SpawnSystematLocation "/Game/Blueprints/Character/Boss/AncientGolem/BossAsset/NS_ShockWave_Boss.NS_ShockWave_Boss" (Transformation|GetActorLocation) "0, 0, 0" "1.225000,1.225000,1.225000")
  (Utilities|FlowControl|Delay 0.05)
  (Actor|DestroyActor))

(fn ConstructionScript)