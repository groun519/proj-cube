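; Gameplay ability for the Ancient Golem boss's Gimic 8 attack: a leap out of sight followed by a landing slam.
; It faces the combat target and plays the eighth attack montage, whose gameplay events drive three stages.
; Jump raises the boss through a recursive delay loop and hides it; the montage's tag event teleports it above a nearby "Center"-tagged actor and spawns a damage hitbox.
; Land restores visibility, walking and overlaps, then ends the ability.
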(event Custom|JumpLoop
  (bind _bpancientgolem (Variables|Default|GetBPAncientGolem))
  ;[0.07292 1 0.143] 점프 재귀 루프
  (if (Variables|Default|GetbIsJumping)
    (Transformation|SetActorRelativeLocation _bpancientgolem (+ (Transformation|GetActorLocation _bpancientgolem) "0.000000,0.000000,50.000000") false true)
    (Utilities|FlowControl|Delay 0.01)
    (CallFunction|JumpLoop)))

(event Ability|EventActivateAbility
  ;[1 1 1] AncientGolem으로 캐스팅
  ; (유니티의 GetComponent와 유사한, 객체 접근)
  (bind _asbp_ancient_golem_2 (Utilities|Casting|CastToBP_AncientGolem (Ability|GetAvatarActorfromActorInfo)))
  (bind _output_get (Variables|Default|SetBPAncientGolem _asbp_ancient_golem_2))
  ;[1 1 1] Facing
  (bind _returnvalue (Class|CombatInterface|GetCombatTarget(Message) _output_get))
  (Class|CombatInterface|UpdateFacingTarget(Message) _output_get (Transformation|GetActorLocation _returnvalue))
  ;[1 1 1] 사용할 몽타주 선정 (보스 캐릭터의 배열에 할당되어져 있는 몽타주를 가져옴.
  (bind _returnvalue_2 (Class|CombatInterface|GetAttackMontages(Message) (Variables|Default|GetBPAncientGolem)))
  (for (_array_element _array_index) _returnvalue_2
    (if (== _array_index 7)
      ;[1 1 1] 해당 몽타주 재생
      (bind _output_get_2 (Variables|Default|SetTaggedMontage _array_element))
      (|PlayMontageandWaitProxy "None" (.Montage (Utilities|Struct|BreakTaggedMontage _output_get_2)) 1.0 "None" true 1.0 0.0 false
        (:then
          (Utilities|FlowControl|Sequence
            (:then_0
              ;[1 1 1] 태그 바인딩
              (Ability|Tasks|WaitGameplayEvent "(TagName=\"Event.Montage.Gimic8.Jump\")" 0 true
                (:EventReceived
                  ;[1 1 1] 점프 이벤트 호출 (Jump Loop로 Is Jumping이 true일 동안 재귀반복하게 만듬.)
                  (Variables|Default|SetbIsJumping true)
                  (CallFunction|JumpLoop)
                  (Utilities|FlowControl|Delay 1.0)
                  ;[1 0.3641 0.07292] 보스의 모습을 숨김.
                  (Rendering|SetActorHiddenInGame (Variables|Default|GetBPAncientGolem) true)
                  (Pawn|Components|CharacterMovement|DisableMovement (Variables|/Script/Engine.Character|GetCharacterMovement (Variables|Default|GetBPAncientGolem)))
                  ;[1 1 1] Is Jumping을 true로 만들어 JumpLoop 이벤트트의 루프를 빠져나옴.
                  (Variables|Default|SetbIsJumping false))))
            (:then_1
              ;[1 1 1] 가장 가까운 플레이어 4명을 탐색
              (Ability|Tasks|WaitGameplayEvent (.MontageTag (Utilities|Struct|BreakTaggedMontage _output_get_2)) 0 true
                (:EventReceived
                  (bind _returnvalue_3 (Class|CubeActiveSkill|FindNearestActorsbyTag "Center" (Transformation|GetActorLocation (Variables|Default|GetBPAncientGolem)) 5e+03 1 true))
                  (for (_array_element_2 _array_index_2) _returnvalue_3
                    (if (== _array_index_2 0)
                      ;[1 0.3641 0.07292] 보스를 해당 플레이어 위치로 이동시키고, 콜리전을 비활성화시킴.
                      (Transformation|SetActorRelativeLocation (Variables|Default|GetBPAncientGolem) (+ (Transformation|GetActorLocation _array_element_2) "0.000000,0.000000,390.000000") false true)
                      (Variables|/Script/Engine.PrimitiveComponent|SetbGenerateOverlapEvents (Variables|/Script/Engine.Character|GetMesh (Variables|Default|GetBPAncientGolem)) false)
                      ;[0.09375 0.3083 1] 히트박스 생성
                      (Class|CubeActiveSkill|SpawnHitBox "JumpHitbox" "JumpDamage" (Math|Transform|MakeTransform (Transformation|GetActorLocation (Variables|Default|GetBPAncientGolem)) (Transformation|GetActorRotation (Variables|Default|GetBPAncientGolem))) false 0 0))))))
            (:then_2
              ;[1 0.3641 0.07292] 보스의 모습을 다시 보이게 함.
              (Ability|Tasks|WaitGameplayEvent "(TagName=\"Event.Montage.Gimic8.Land\")" 0 true
                (:EventReceived
                  (Rendering|SetActorHiddenInGame (Variables|Default|GetBPAncientGolem) false)
                  (Pawn|Components|CharacterMovement|SetMovementMode (Variables|/Script/Engine.Character|GetCharacterMovement (Variables|Default|GetBPAncientGolem)) "MOVE_Walking" 0)
                  (Variables|/Script/Engine.PrimitiveComponent|SetbGenerateOverlapEvents (Variables|/Script/Engine.Character|GetMesh (Variables|Default|GetBPAncientGolem)) true)
                  ;[1 1 1] 사운드 재생 후 어빌리티 종료.
                  (Audio|PlaySound2D 0 1.0 1.0 0.0 0 0)
                  (Utilities|FlowControl|Delay 0.5)
                  (Ability|EndAbility))))))))))

(fn FindNearestPlayer
  (LocalVariables|SetClosestActor 0)
  (LocalVariables|SetClosestDistance 9999999999.0)
  (bind _outactors (Actor|GetAllActorswithTag "Player"))
  (for _array_element _outactors
    (bind _returnvalue (Class|CombatInterface|IsDead(Message) _array_element))
    (if (not _returnvalue)
      (bind _output_get (LocalVariables|SetActor _array_element))
      (bind _output_get_2 (LocalVariables|SetCalculatedDistance (Transformation|GetDistanceTo _output_get (LocalVariables|GetActor))))
      (if (< _output_get_2 (LocalVariables|GetClosestDistance))
        (LocalVariables|SetClosestDistance (LocalVariables|GetCalculatedDistance))
        (bind _output_get_3 (LocalVariables|SetClosestActor (LocalVariables|GetActor)))
        (return (Transformation|GetActorLocation _output_get_3))))))