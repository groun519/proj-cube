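; Gameplay ability for the Ancient Golem boss's second gimmick, a "Razer" projectile attack at a nearby player.
; It plays the second attack montage and waits once for that montage's gameplay event tag.
; On the event it finds the nearest tagged player within range, turns to face them and spawns the projectile from the montage's socket, aimed along the forward vector.
; The FindNearestPlayer helper is unused, and EndAbility is never called.
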(event Ability|EventActivateAbility
  (bind _returnvalue (Ability|GetAvatarActorfromActorInfo))
  (bind _returnvalue_2 (Class|CombatInterface|GetAttackMontages(Message) (Ability|GetAvatarActorfromActorInfo)))
  (bind (_array_element _array_index) (Utilities|Array|ForEachLoopwithBreak _returnvalue_2)
    (:LoopBody
      (if (== _array_index 1)
        (bind _output_get (Variables|Default|SetTaggedMontage _array_element))
        (|PlayMontageandWaitProxy "None" (.Montage (Utilities|Struct|BreakTaggedMontage _output_get)) 1.0 "None" true 1.0 0.0 false
          (:then
            (Ability|Tasks|WaitGameplayEvent (.MontageTag (Utilities|Struct|BreakTaggedMontage _output_get)) 0 true
              (:EventReceived
                ;[1 1 1] 플레이어 탐색 (1차)
                (bind _returnvalue_3 (Class|CubeActiveSkill|FindNearestActorsbyTag "Player" (Transformation|GetActorLocation (Ability|GetAvatarActorfromActorInfo)) 3e+03 1 true))
                (for _array_element_2 _returnvalue_3
                  ;[1 1 1] 방향 바라보기
                  (Utilities|IsValid _array_element_2
                    (:Is%20Valid
                      (bind _ascombat_interface (Utilities|Casting|CastToCombatInterface (Ability|GetAvatarActorfromActorInfo)))
                      (Class|CombatInterface|UpdateFacingTarget _ascombat_interface (Transformation|GetActorLocation _array_element_2))
                      (Class|CubeActiveSkill|SpawnProjectile "Razer" "Rax" (+ (Transformation|GetActorForwardVector _returnvalue) (Transformation|GetActorLocation _returnvalue)) (.SocketTag (Utilities|Struct|BreakTaggedMontage _output_get)) true 0.0 false 0.0 0 false 0 "(bUseMultipleProjectilesFeacher=False,ProjectileSpread=90.000000,MaxNumProjectiles=5)" "(bUseHomingFeacher=False,HomingAccelerationMin=1600.000000,HomingAccelerationMax=3200.000000)"))))))))))))

(event Ability|EventOnEndAbility
  (params (bWasCancelled :type Boolean)))

(fn FindNearestPlayer
  (LocalVariables|SetClosestActor 0)
  (LocalVariables|SetClosestDistance 9999999999.0)
  (bind _outactors (Actor|GetAllActorswithTag "Player"))
  (for _array_element _outactors
    (bind _output_get (LocalVariables|SetActor _array_element))
    (bind _output_get_2 (LocalVariables|SetCalculatedDistance (Transformation|GetDistanceTo _output_get (LocalVariables|GetActor))))
    (if (< _output_get_2 (LocalVariables|GetClosestDistance))
      (LocalVariables|SetClosestDistance (LocalVariables|GetCalculatedDistance))
      (bind _output_get_3 (LocalVariables|SetClosestActor (LocalVariables|GetActor)))
      (return (Transformation|GetActorLocation _output_get_3)))))