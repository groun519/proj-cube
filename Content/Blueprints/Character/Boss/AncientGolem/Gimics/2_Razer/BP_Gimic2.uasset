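; BP_Gimic2 is a projectile actor for the Ancient Golem boss's second gimmick (Razer), fired horizontally toward a nearby player.
; On BeginPlay it raises itself 250 units, then sphere-overlaps for actors tagged Player.
; Each match sets the ProjectileMovement velocity along the look-at yaw with pitch zeroed, so the last match wins.
; The direction is set once, with no later homing.
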(event EventBeginPlay
  (bind _self self)
  (bind _self_2 self)
  (bind _returnvalue (Transformation|GetActorLocation _self_2))
  (Transformation|SetActorRelativeLocation _self (+ (Transformation|GetActorLocation _self) "0.000000,0.000000,250.000000"))
  (Variables|Default|SetFirestLoc _returnvalue)
  (bind _outactors (Collision|SphereOverlapActors _returnvalue 1e+03 (Variables|Default|GetObject%20Types) 0))
  (for _array_element _outactors
    (if (Actor|ActorHasTag _array_element "Player")
      (Variables|/Script/Engine.MovementComponent|SetVelocity (Variables|Default|GetProjectileMovement) (* (Math|Rotator|GetRotationXVector (Math|Rotator|MakeRotator (.Roll (Math|Rotator|BreakRotator (Math|Rotator|FindLookatRotation (Variables|Default|GetFirestLoc) (Transformation|GetActorLocation _array_element)))) 0.0 (.Yaw (Math|Rotator|BreakRotator (Math|Rotator|FindLookatRotation (Variables|Default|GetFirestLoc) (Transformation|GetActorLocation _array_element)))))) 3e+03)))))

(fn ConstructionScript)