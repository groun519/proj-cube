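; Timed area-attack actor for the Ancient Golem boss's jump gimmick, with a growing indicator that leads into a shockwave.
; BeginPlay configures the Sphere as a hitbox, then Tick scales the flattened Sec component up over MaxTime in proportion to the Sphere's size.
; Once time runs out, it spawns the shockwave Niagara effect, enables Sphere overlap events and destroys itself after a brief delay.
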(event EventBeginPlay
  (Class|CubeHitbox|SetHitboxCollision (Variables|Default|GetSphere))
  (Variables|Default|SetYawRot 0.0)
  (Variables|Default|SetRollRot 0.0)
  (Variables|Default|SetPitchRot 0.0)
  (Transformation|SetRelativeLocation (Variables|Default|GetSphere) (Transformation|GetWorldLocation (Variables|Default|GetSphere)) false true))

(event EventTick
  (params (DeltaSeconds :type Float%20%28single-precision%29))
  (if (> (Variables|Default|GetTime) (Variables|Default|GetMaxTime))
    (Niagara|SpawnSystematLocation "/Game/Blueprints/Character/Boss/AncientGolem/BossAsset/NS_ShockWave_Boss.NS_ShockWave_Boss" (Transformation|GetActorLocation) "0, 0, 0" "1.500000,1.500000,1.500000")
    (Variables|/Script/Engine.PrimitiveComponent|SetbGenerateOverlapEvents (Variables|Default|GetSphere) true)
    (Utilities|FlowControl|Delay 0.1)
    (Actor|DestroyActor)
    (else
      (Variables|Default|SetTime (+ (Variables|Default|GetTime) DeltaSeconds))
      (Transformation|SetWorldScale3D (Variables|Default|GetSec) (Math|Vector|MakeVector (* (Variables|Default|GetTime) (/ (* (.x (Transformation|GetWorldScale (Variables|Default|GetSphere))) 1e+01) (Variables|Default|GetMaxTime))) (* (Variables|Default|GetTime) (/ (* (.x (Transformation|GetWorldScale (Variables|Default|GetSphere))) 1e+01) (Variables|Default|GetMaxTime))) 0.1)))))

(fn ConstructionScript)