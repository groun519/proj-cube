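; Gameplay ability for the Ancient Golem boss's first gimmick: a leap that crashes down on a player.
; It faces the combat target and plays the first attack montage, whose gameplay events pace each phase.
; A recursive Delay loop lifts the boss before hiding it, then it teleports to the nearest player within range and spawns a damage hitbox.
; The Land event unhides it, plays a sound and ends the ability; FindNearestPlayer is not called here.
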(event Custom|JumpLoop
  (bind _returnvalue (Ability|GetAvatarActorfromActorInfo))
  (if (Variables|Default|GetbIsJumping)
    (Transformation|SetActorRelativeLocation _returnvalue (+ (Transformation|GetActorLocation _returnvalue) "0.000000,0.000000,50.000000") false true)
    (Utilities|FlowControl|Delay 0.01)
    (CallFunction|JumpLoop)))

(event Ability|EventActivateAbility
  (bind _returnvalue (Ability|GetAvatarActorfromActorInfo))
  (bind _returnvalue_2 (Ability|GetAvatarActorfromActorInfo))
  (bind _returnvalue_3 (Class|CombatInterface|GetCombatTarget(Message) _returnvalue_2))
  (Class|CombatInterface|UpdateFacingTarget(Message) _returnvalue_2 (Transformation|GetActorLocation _returnvalue_3))
  (bind _returnvalue_4 (Class|CombatInterface|GetAttackMontages(Message) (Ability|GetAvatarActorfromActorInfo)))
  (for (_array_element _array_index) _returnvalue_4
    (if (== _array_index 0)
      (bind _output_get (Variables|Default|SetTaggedMontage _array_element))
      (|PlayMontageandWaitProxy "None" (.Montage (Utilities|Struct|BreakTaggedMontage _output_get)) 1.0 "None" true 1.0 0.0 false
        (:then
          (Ability|Tasks|WaitGameplayEvent "(TagName=\"Event.Montage.Gimic1.Jump\")" 0 true
            (:EventReceived
              (Variables|Default|SetbIsJumping true)
              (CallFunction|JumpLoop)
              (Utilities|FlowControl|Delay 1.0)
              (Rendering|SetActorHiddenInGame (Ability|GetAvatarActorfromActorInfo) true)
              (Variables|Default|SetbIsJumping false)
              (Ability|Tasks|WaitGameplayEvent (.MontageTag (Utilities|Struct|BreakTaggedMontage _output_get)) 0 true
                (:EventReceived
                  (bind _returnvalue_5 (Class|CubeActiveSkill|FindNearestActorsbyTag "Player" (Transformation|GetActorLocation (Ability|GetAvatarActorfromActorInfo)) 6e+03 1 false))
                  (for _array_element_2 _returnvalue_5
                    (Transformation|SetActorRelativeLocation (Ability|GetAvatarActorfromActorInfo) (Transformation|GetActorLocation _array_element_2) false true)
                    (Class|CubeActiveSkill|SpawnHitBox "JumpHitbox" "JumpDamage" (Math|Transform|MakeTransform (Transformation|GetActorLocation _returnvalue) (Transformation|GetActorRotation _returnvalue)) false 0 0)
                    (Ability|Tasks|WaitGameplayEvent "(TagName=\"Event.Montage.Gimic1.Land\")" 0 true
                      (:EventReceived
                        (Rendering|SetActorHiddenInGame (Ability|GetAvatarActorfromActorInfo) false)
                        (Audio|PlaySound2D 0 1.0 1.0 0.0 0 0)
                        (Utilities|FlowControl|Delay 0.2)
                        (Ability|EndAbility)))))))))))))

(event Ability|EventOnEndAbility
  (params (bWasCancelled :type Boolean)))

(fn FindNearestPlayer
  (LocalVariables|SetClosestActor 0)
  (LocalVariables|SetClosestDistance 9999999999.0)
  (bind _outactors (Actor|GetAllActorswithTag "Player"))
  (for _array_element _outactors
    (bind _returnvalue (Class|CombatInterface|IsDead(Message) _array_element))
    (if (not _returnvalue)
      (bind _output_get (LocalVariables|SetActor _array_element))
      (bind _output_get_2 (LocalVariables|SetCalculatedDistance (Transformation|GetDistanceTo _output_get (LocalVariables|GetActor))))
      (if (< _output_get_2 (LocalVariables|GetClosestDistance))
        (LocalVariables|SetClosestDistance (LocalVariables|GetCalculatedDistance))
        (bind _output_get_3 (LocalVariables|SetClosestActor (LocalVariables|GetActor)))
        (return (Transformation|GetActorLocation _output_get_3))))))