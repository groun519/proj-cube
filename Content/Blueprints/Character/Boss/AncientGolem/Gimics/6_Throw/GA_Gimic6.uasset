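; Gameplay ability for the Ancient Golem boss's sixth gimmick, a rock throw at a nearby player.
; It plays the golem's fifth attack montage, using gameplay events to show the held Rock mesh, then hide it on release.
; On release it updates facing toward the combat target, finds the nearest tagged player within range, spawns the projectile at their location and ends after a short delay.
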(event Ability|EventActivateAbility
  (bind _returnvalue (Ability|GetAvatarActorfromActorInfo))
  (bind _asbp_ancient_golem (Utilities|Casting|CastToBP_AncientGolem2 (Ability|GetAvatarActorfromActorInfo)))
  (Variables|Default|SetBPAncientGolem _asbp_ancient_golem)
  (bind _returnvalue_2 (Class|CombatInterface|GetAttackMontages(Message) (Ability|GetAvatarActorfromActorInfo)))
  (bind (_array_element _array_index) (Utilities|Array|ForEachLoopwithBreak _returnvalue_2)
    (:LoopBody
      (if (== _array_index 4)
        (bind _output_get (Variables|Default|SetTaggedMontage _array_element))
        (|PlayMontageandWaitProxy "None" (.Montage (Utilities|Struct|BreakTaggedMontage _output_get)) 1.0 "None" true 1.0 0.0 false
          (:then
            (Utilities|FlowControl|Sequence
              (:then_0
                (Ability|Tasks|WaitGameplayEvent "(TagName=\"Event.Montage.Gimic6.Rock\")" 0 true
                  (:EventReceived
                    (Rendering|SetVisibility (Variables|/Game/Blueprints/Character/Boss/AncientGolem/BP_AncientGolem2.BP_AncientGolem2_C|GetRock (Variables|Default|GetBPAncientGolem)) true false))))
              (:then_1
                (Ability|Tasks|WaitGameplayEvent (.MontageTag (Utilities|Struct|BreakTaggedMontage _output_get)) 0 true
                  (:EventReceived
                    (Rendering|SetVisibility (Variables|/Game/Blueprints/Character/Boss/AncientGolem/BP_AncientGolem2.BP_AncientGolem2_C|GetRock (Variables|Default|GetBPAncientGolem)) false false)
                    (bind _returnvalue_3 (Class|CombatInterface|GetCombatTarget(Message) _returnvalue))
                    (Class|CombatInterface|UpdateFacingTarget(Message) _returnvalue (Transformation|GetActorLocation _returnvalue_3))
                    (bind _returnvalue_4 (Class|CubeActiveSkill|FindNearestActorsbyTag "Player" (Transformation|GetActorLocation (Ability|GetAvatarActorfromActorInfo)) 3e+03 1 true))
                    (for _array_element_2 _returnvalue_4
                      (Class|CubeActiveSkill|SpawnProjectile "Gimic6" "Gimic6" (Transformation|GetActorLocation _array_element_2) (.SocketTag (Utilities|Struct|BreakTaggedMontage _output_get)) false 0.0 false 0.0 0 false 0 "(bUseMultipleProjectilesFeacher=False,ProjectileSpread=90.000000,NumProjectiles=1,MaxNumProjectiles=1,UpgradeProjectiles=1)" "(bUseHomingFeacher=False,HomingAccelerationMin=1600.000000,HomingAccelerationMax=3200.000000,HomingTarget=None)")
                      (Utilities|FlowControl|Delay 0.2)
                      (Ability|EndAbility))))))))))))

(event Ability|EventOnEndAbility
  (params (bWasCancelled :type Boolean)))