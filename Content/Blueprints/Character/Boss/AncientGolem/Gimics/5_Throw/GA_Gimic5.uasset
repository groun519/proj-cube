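; Gameplay ability for the Ancient Golem boss's fifth gimmick, a throw attack that launches a projectile at a nearby player.
; It plays the avatar's fifth attack montage and waits for that montage's gameplay event.
; On the event, it updates facing toward the combat target, spawns the projectile from the montage's socket at the nearest tagged player, then ends after a short delay.
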(event Ability|EventActivateAbility
  (bind _returnvalue (Ability|GetAvatarActorfromActorInfo))
  (bind _returnvalue_2 (Class|CombatInterface|GetAttackMontages(Message) (Ability|GetAvatarActorfromActorInfo)))
  (bind (_array_element _array_index) (Utilities|Array|ForEachLoopwithBreak _returnvalue_2)
    (:LoopBody
      (if (== _array_index 4)
        (bind _output_get (Variables|Default|SetTaggedMontage _array_element))
        (|PlayMontageandWaitProxy "None" (.Montage (Utilities|Struct|BreakTaggedMontage _output_get)) 1.0 "None" true 1.0 0.0 false
          (:then
            (Ability|Tasks|WaitGameplayEvent (.MontageTag (Utilities|Struct|BreakTaggedMontage _output_get)) 0 true
              (:EventReceived
                (bind _returnvalue_3 (Class|CombatInterface|GetCombatTarget(Message) _returnvalue))
                (Class|CombatInterface|UpdateFacingTarget(Message) _returnvalue (Transformation|GetActorLocation _returnvalue_3))
                (bind _returnvalue_4 (Class|CubeActiveSkill|FindNearestActorsbyTag "Player" (Transformation|GetActorLocation (Ability|GetAvatarActorfromActorInfo)) 3e+03 1 true))
                (for _array_element_2 _returnvalue_4
                  (Class|CubeActiveSkill|SpawnProjectile "Gimic5" "Gimic5" (Transformation|GetActorLocation _array_element_2) (.SocketTag (Utilities|Struct|BreakTaggedMontage _output_get)) false 0.0 false 0.0 0 false 0)
                  (Utilities|FlowControl|Delay 0.2)
                  (Ability|EndAbility))))))))))

(event Ability|EventOnEndAbility
  (params (bWasCancelled :type Boolean)))