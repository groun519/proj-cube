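; Ancient Golem boss ability that plays a random attack montage for a leap attack: rise, vanish, reappear at a player and fire a projectile.
; Chained montage gameplay events drive the jump, teleport with projectile spawn, and landing unhide.
; JumpLoop raises the golem through timed recursive teleports until it hides.
; FindNearestPlayer measures each actor against itself and returns inside the loop, so it yields the first tagged player, not the nearest.
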(event Custom|JumpLoop
  (bind _returnvalue (Ability|GetAvatarActorfromActorInfo))
  (if (Variables|Default|GetbIsJumping)
    (Transformation|SetActorRelativeLocation _returnvalue (+ (Transformation|GetActorLocation _returnvalue) "0.000000,0.000000,50.000000") false true)
    (Utilities|FlowControl|Delay 0.01)
    (CallFunction|JumpLoop)))

(event Ability|EventActivateAbility
  (bind _returnvalue (Ability|GetAvatarActorfromActorInfo))
  (bind _returnvalue_2 (Class|CombatInterface|GetCombatTarget(Message) _returnvalue))
  (Class|CombatInterface|UpdateFacingTarget(Message) _returnvalue (Transformation|GetActorLocation _returnvalue_2))
  (bind _returnvalue_3 (Class|CombatInterface|GetAttackMontages(Message) (Ability|GetAvatarActorfromActorInfo)))
  (bind _output_get (Variables|Default|SetTaggedMontage (Class|CubeDamageGameplayAbility|GetRandomTaggedMontagefromArray _returnvalue_3)))
  (|PlayMontageandWaitProxy "None" (.Montage (Utilities|Struct|BreakTaggedMontage _output_get)) 1.0 "None" true 1.0 0.0 false
    (:then
      (Ability|Tasks|WaitGameplayEvent "(TagName=\"Event.Montage.Gimic1.Jump\")" 0 true
        (:EventReceived
          (Variables|Default|SetbIsJumping true)
          (CallFunction|JumpLoop)
          (Utilities|FlowControl|Delay 1.0)
          (Rendering|SetActorHiddenInGame (Ability|GetAvatarActorfromActorInfo) true)
          (Variables|Default|SetbIsJumping false)
          (Ability|Tasks|WaitGameplayEvent (.MontageTag (Utilities|Struct|BreakTaggedMontage _output_get)) 0 true
            (:EventReceived
              (bind _nearestplayerloc (CallFunction|FindNearestPlayer))
              (Transformation|SetActorRelativeLocation (Ability|GetAvatarActorfromActorInfo) _nearestplayerloc false true)
              (Class|CubeProjectileSkill|SpawnProjectile (Transformation|GetActorLocation (Ability|GetAvatarActorfromActorInfo)) (.SocketTag (Utilities|Struct|BreakTaggedMontage _output_get)) false 0.0)
              (Ability|Tasks|WaitGameplayEvent "(TagName=\"Event.Montage.Gimic1.Land\")" 0 true
                (:EventReceived
                  (Rendering|SetActorHiddenInGame (Ability|GetAvatarActorfromActorInfo) false))))))))))

(event Ability|EventOnEndAbility
  (params (bWasCancelled :type Boolean)))

(fn FindNearestPlayer
  (LocalVariables|SetClosestActor 0)
  (LocalVariables|SetClosestDistance 9999999999.0)
  (bind _outactors (Actor|GetAllActorswithTag "Player"))
  (for _array_element _outactors
    (bind _output_get (LocalVariables|SetActor _array_element))
    (bind _output_get_2 (LocalVariables|SetCalculatedDistance (Transformation|GetDistanceTo _output_get (LocalVariables|GetActor))))
    (if (< _output_get_2 (LocalVariables|GetClosestDistance))
      (LocalVariables|SetClosestDistance (LocalVariables|GetCalculatedDistance))
      (bind _output_get_3 (LocalVariables|SetClosestActor (LocalVariables|GetActor)))
      (return (Transformation|GetActorLocation _output_get_3)))))