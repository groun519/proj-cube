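; Ancient Golem boss gameplay ability for the "Razer" ranged attack, firing a projectile at a player.
; Plays the attack montage at index 1, waits once for its tag event, then faces the combat target and spawns a pitch-overridden projectile from the montage's socket.
; FindNearestPlayer supplies the aim point, but measures each actor against itself, so it returns the first "Player"-tagged actor's location.
; No EndAbility call appears in the graph.
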(event Ability|EventActivateAbility
  (bind _returnvalue (Ability|GetAvatarActorfromActorInfo))
  (bind _returnvalue_2 (Class|CombatInterface|GetAttackMontages(Message) (Ability|GetAvatarActorfromActorInfo)))
  (bind (_array_element _array_index) (Utilities|Array|ForEachLoopwithBreak _returnvalue_2)
    (:LoopBody
      (if (== _array_index 1)
        (bind _output_get (Variables|Default|SetTaggedMontage _array_element))
        (|PlayMontageandWaitProxy "None" (.Montage (Utilities|Struct|BreakTaggedMontage _output_get)) 1.0 "None" true 1.0 0.0 false
          (:then
            (Ability|Tasks|WaitGameplayEvent (.MontageTag (Utilities|Struct|BreakTaggedMontage _output_get)) 0 true
              (:EventReceived
                (bind _returnvalue_3 (Class|CombatInterface|GetCombatTarget(Message) _returnvalue))
                (Class|CombatInterface|UpdateFacingTarget(Message) _returnvalue (Transformation|GetActorLocation _returnvalue_3))
                (bind _nearestplayerloc (CallFunction|FindNearestPlayer))
                (Class|CubeProjectileSkill|SpawnProjectile _nearestplayerloc (.SocketTag (Utilities|Struct|BreakTaggedMontage _output_get)) true 0.0 false 0.0 0 false 0)))))))))

(event Ability|EventOnEndAbility
  (params (bWasCancelled :type Boolean)))

(fn FindNearestPlayer
  (LocalVariables|SetClosestActor 0)
  (LocalVariables|SetClosestDistance 9999999999.0)
  (bind _outactors (Actor|GetAllActorswithTag "Player"))
  (for _array_element _outactors
    (bind _output_get (LocalVariables|SetActor _array_element))
    (bind _output_get_2 (LocalVariables|SetCalculatedDistance (Transformation|GetDistanceTo _output_get (LocalVariables|GetActor))))
    (if (< _output_get_2 (LocalVariables|GetClosestDistance))
      (LocalVariables|SetClosestDistance (LocalVariables|GetCalculatedDistance))
      (bind _output_get_3 (LocalVariables|SetClosestActor (LocalVariables|GetActor)))
      (return (Transformation|GetActorLocation _output_get_3)))))