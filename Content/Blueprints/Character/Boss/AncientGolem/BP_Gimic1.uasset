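; Timed area gimmick for the Ancient Golem boss, with a growing indicator that ends in a brief overlap window.
; Tick accumulates time and scales the flat Sec component in X and Y toward five times the Sphere's world scale.
; Once MaxTime passes, it enables overlap events on the Sphere and destroys the actor after a short delay.
; BeginPlay sets the Sphere's relative location to its world location; no overlap response is implemented here.
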(event EventBeginPlay
  (Variables|Default|SetYawRot 0.0)
  (Variables|Default|SetRollRot 0.0)
  (Variables|Default|SetPitchRot 0.0)
  (Transformation|SetRelativeLocation (Variables|Default|GetSphere) (Transformation|GetWorldLocation (Variables|Default|GetSphere)) false true))

(event Collision|EventActorBeginOverlap
  (params (OtherActor :type Actor%20Object%20Reference)))

(event EventTick
  (params (DeltaSeconds :type Float%20%28single-precision%29))
  (if (> (Variables|Default|GetTime) (Variables|Default|GetMaxTime))
    (Variables|/Script/Engine.PrimitiveComponent|SetbGenerateOverlapEvents (Variables|Default|GetSphere) true)
    (Utilities|FlowControl|Delay 0.1)
    (Actor|DestroyActor)
    (else
      (Variables|Default|SetTime (+ (Variables|Default|GetTime) DeltaSeconds))
      (Transformation|SetWorldScale3D (Variables|Default|GetSec) (Math|Vector|MakeVector (* (Variables|Default|GetTime) (/ (* (.x (Transformation|GetWorldScale (Variables|Default|GetSphere))) 5.0) (Variables|Default|GetMaxTime))) (* (Variables|Default|GetTime) (/ (* (.x (Transformation|GetWorldScale (Variables|Default|GetSphere))) 5.0) (Variables|Default|GetMaxTime))) 0.1)))))

(fn ConstructionScript)