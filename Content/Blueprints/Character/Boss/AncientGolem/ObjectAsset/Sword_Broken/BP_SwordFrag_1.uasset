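; Broken sword fragment for the Ancient Golem boss that rises, glows, then launches itself as a projectile at a nearby player.
; BeginPlay waits, then briefly enables a levitation flag, during which Tick boosts the mesh's emissive parameter and plays a Timeline that offsets its height.
; When levitation ends, FindPlayer searches a radius with a debug sphere, turns the fragment toward the player, and its look-at result sets the ProjectileMovement velocity.
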(event EventBeginPlay
  (Utilities|FlowControl|Delay 3.0)
  (Variables|Default|SetbIsLevitation true)
  (Utilities|FlowControl|Delay 2.0)
  (Variables|Default|SetbIsLevitation false)
  (bind _newparam (CallFunction|FindPlayer))
  (Variables|/Script/Engine.MovementComponent|SetVelocity (Variables|Default|GetProjectileMovement) (* _newparam 2e+04)))

(event EventTick
  (params (DeltaSeconds :type Float%20%28single-precision%29))
  (if (Variables|Default|GetbIsLevitation)
    (Rendering|Material|SetScalarParameterValueonMaterials (Variables|Default|GetStaticMesh) "EmissivePercent" 5.0)
    (bind _newtrack_0 (Timeline|Timeline Play)
      (:Update
        (Transformation|SetActorLocation (+ (Transformation|GetActorLocation) (Math|Vector|MakeVector 0.0 0.0 _newtrack_0)) false false)))))

(fn ConstructionScript)

(fn FindPlayer
  (bind _returnvalue (Class|CubeHitActor|FindNearestPlayers (Transformation|GetActorLocation) 1e+03 1 true))
  (for _array_element _returnvalue
    (Utilities|IsValid _array_element
      (:Is%20Valid
        (Transformation|SetActorRelativeRotation (Math|Rotator|FindLookatRotation (Transformation|GetActorLocation) (Transformation|GetActorLocation _array_element)))
        (return (Math|Rotator|FindLookatRotation (Transformation|GetActorLocation) (Transformation|GetActorLocation _array_element)))))))