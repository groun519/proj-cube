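; BP_BossTrail is a posed-mesh trail actor for the Ancient Golem boss, acting as a colored afterimage.
; CopyPose copies a skeletal component's pose onto its PoseableMesh, and SetColor stores the tint.
; BeginPlay runs the Opacity timeline, whose every update creates dynamic material instances on all material slots and sets their Opacity and Color parameters.
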(event Custom|CopyPose
  (params (InComponentToCopy :type Skeletal%20Mesh%20Component%20Object%20Reference))
  (Class|PoseableMeshComponent|CopyPosefromSkeletalComponent (Variables|Default|GetPoseableMesh) InComponentToCopy))

(event Custom|SetColor
  (params (Color :type Linear%20Color%20Structure))
  (Variables|Default|SetColor Color))

(event EventBeginPlay
  (bind _poseablemesh (Variables|Default|GetPoseableMesh))
  (bind _opacity (Timeline|Opacity Play)
    (:Update
      (for (_array_element _array_index) (Rendering|Material|GetMaterials _poseablemesh)
        (bind _returnvalue (Rendering|Material|CreateDynamicMaterialInstance _poseablemesh _array_index _array_element "None" :!class /Script/Engine.PrimitiveComponent))
        (Rendering|Material|SetScalarParameterValue _returnvalue "Opacity" _opacity :!class /Script/Engine.MaterialInstanceDynamic)
        (Rendering|Material|SetVectorParameterValue _returnvalue "Color" (Variables|Default|GetColor) :!class /Script/Engine.MaterialInstanceDynamic)))))

(event Collision|EventActorBeginOverlap
  (params (OtherActor :type Actor%20Object%20Reference)))

(event EventTick
  (params (DeltaSeconds :type Float%20%28single-precision%29)))

(fn ConstructionScript)