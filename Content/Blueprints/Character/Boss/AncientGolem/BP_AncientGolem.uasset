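; Ancient Golem boss character Blueprint, handling its entrance sequence and visual effect events.
; On BeginPlay it hides mesh and weapon, teleports far below and back, and plays an intro montage with walking disabled.
; When the montage completes, it restores base speed and sets a Blackboard bool.
; SpawnTrail spawns a tinted pose-copy trail, and EmissiveCharacter tints every material through dynamic instances, resetting after a delay.
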(event Custom|EmissiveCharacter
  (params (Color :type Linear%20Color%20Structure) (Emissive :type Float%20%28double-precision%29) (Time :type Float%20%28double-precision%29))
  ;[1 1 1] Character Emissive Event
  (Utilities|FlowControl|Sequence
    (:then_0
      (for (_array_element _array_index) (Rendering|Material|GetMaterials (Variables|Character|GetMesh))
        (bind _returnvalue (Rendering|Material|CreateDynamicMaterialInstance (Variables|Character|GetMesh) _array_index _array_element "None" :!class /Script/Engine.PrimitiveComponent))
        (Utilities|Array|Add (Variables|Default|GetMIDArr) _returnvalue)
        (Rendering|Material|SetVectorParameterValue _returnvalue "Color" Color :!class /Script/Engine.MaterialInstanceDynamic)
        (Rendering|Material|SetScalarParameterValue _returnvalue "Emissive" Emissive :!class /Script/Engine.MaterialInstanceDynamic))
      (Utilities|FlowControl|Delay Time)
      (for _array_element_2 (Variables|Default|GetMIDArr)
        (Rendering|Material|SetVectorParameterValue :self _array_element_2 :ParameterName "Color" :!class /Script/Engine.MaterialInstanceDynamic)
        (Rendering|Material|SetScalarParameterValue _array_element_2 "Emissive" 0.0 :!class /Script/Engine.MaterialInstanceDynamic)))))

(event Custom|SpawnTrail
  (params (Color :type Linear%20Color%20Structure))
  ;[1 1 1] Spawn Trail Event
  (bind _returnvalue (Game|SpawnActorfromClass "/Game/Blueprints/Character/Boss/AncientGolem/BP_BossTrail.BP_BossTrail_C" (Transformation|GetWorldTransform (Variables|Character|GetMesh)) "AlwaysSpawn" "MultiplyWithRoot" 0 0))
  (Default|CopyPose _returnvalue (Variables|Character|GetMesh))
  (Default|SetColor _returnvalue Color))

(event EventBeginPlay
  (Rendering|SetVisibility (Variables|Character|GetMesh) false false)
  (Utilities|FlowControl|Sequence
    (:then_0
      (Utilities|FlowControl|Delay 0.5)
      (Variables|Default|SetNewVar (Transformation|GetActorLocation))
      (Transformation|Teleport "0.000000,0.000000,-10000.000000" "0, 0, 0")
      (Rendering|SetVisibility (Variables|Character|GetMesh) true false)
      (Utilities|FlowControl|Delay 0.2)
      (Transformation|Teleport (Variables|Default|GetNewVar) "0.000000,180.000000,0.000000"))
    (:then_1
      (Variables|/Script/Engine.CharacterMovementComponent|SetMaxWalkSpeed (Variables|Character|GetCharacterMovement) 0.0)
      (Animation|Montage|PlayMontage (Variables|Character|GetMesh) "/Game/Blueprints/Character/Boss/AncientGolem/Alter/AM_Sohawn.AM_Sohawn" 0.65
        (:OnCompleted
          (Variables|/Script/Engine.CharacterMovementComponent|SetMaxWalkSpeed (Variables|Character|GetCharacterMovement) (Variables|Default|GetBaseSpeed))
          (AI|Components|Blackboard|SetValueasBool (AI|GetBlackboard (AI|GetAIController self)) (Variables|Default|GetKeyName) (Variables|Default|GetBoolValue)))))))

(fn ConstructionScript)