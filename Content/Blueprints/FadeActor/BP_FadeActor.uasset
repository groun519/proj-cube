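; Actor Blueprint set up to fade a mesh through a "Fade" material parameter driven by a timeline, though that logic is unconnected.
; The construction script stores the mesh's materials in OriginMaterials, but its instance-creation loop iterates the just-cleared dynamic instance array, leaving it empty.
; A helper function applies that array to the mesh slots but is not called here.
; BeginPlay, overlap and Tick do nothing.
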(event EventBeginPlay)

(event Collision|EventActorBeginOverlap
  (params (OtherActor :type Actor%20Object%20Reference)))

(event EventTick
  (params (DeltaSeconds :type Float%20%28single-precision%29)))

(fn ConstructionScript
  (Utilities|Array|Clear (Variables|Default|GetDynamicMaterialinstance))
  (Variables|Default|SetOriginMaterials (Rendering|Material|GetMaterials (Variables|Default|GetMesh)))
  (for _array_element (Variables|Default|GetDynamicMaterialinstance)
    (Rendering|Material|CreateDynamicMaterialInstance _array_element "None" "None" :!class /Script/Engine.KismetMaterialLibrary)
    (Utilities|Array|AddUnique (Variables|Default|GetDynamicMaterialinstance) 0)))

(fn SetMaterialsTODynamicMaterialinstance
  (for (_array_element _array_index) (Variables|Default|GetDynamicMaterialinstance)
    (Rendering|Material|SetMaterial (Variables|Default|GetMesh) _array_index _array_element)))