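; Light staff basic-attack projectile that redirects toward a nearby enemy and destroys itself shortly after spawning.
; After a brief delay, BeginPlay boosts its velocity and calls FindNearPlayer, which finds a nearby Enemy-tagged actor not in ActorsToIgnore and aims the velocity horizontally at it.
; The instigator-based "Last" branch is never requested, overlap is empty, and older homing, repeat-search and debug logic is disconnected.
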(event OnComponentBeginOverlap(Sphere)
  (params (OverlappedComponent :type Primitive%20Component%20Object%20Reference) (OtherActor :type Actor%20Object%20Reference) (OtherComp :type Primitive%20Component%20Object%20Reference) (OtherBodyIndex :type Integer) (bFromSweep :type Boolean) (SweepResult :type Hit%20Result%20Structure%20%28by%20ref%29)))

(event Custom|FindNearPlayer
  (params (Last :type Boolean))
  (bind _returnvalue (Class|CubeHitActor|GetInstigatorPlayer))
  (bind _returnvalue_2 (Transformation|GetActorLocation _returnvalue))
  (bind _returnvalue_3 (* _returnvalue_2 5e+03))
  (bind (_x _y) (Math|Vector|BreakVector _returnvalue_3))
  (if Last
    (Variables|/Script/Engine.ProjectileMovementComponent|SetHomingTargetComponent (Variables|Default|GetProjectileMovement) (Variables|Transformation|GetRootComponent))
    (Variables|/Script/Engine.MovementComponent|SetVelocity (Variables|Default|GetProjectileMovement) (Math|Vector|MakeVector _x _y 0.0))
    (else
      (bind _returnvalue_4 (Class|CubeHitActor|FindNearestActorsbyTag "Enemy" (Transformation|GetActorLocation) 1e+03 1 false :!label _label))
      (for _array_element _returnvalue_4
        (for _array_element_2 (Variables|Default|GetActorsToIgnore)
          (if (== _array_element _array_element_2)
            (goto _label)))
        (Variables|/Script/Engine.MovementComponent|SetVelocity (Variables|Default|GetProjectileMovement) (Math|Vector|MakeVector (.X (Math|Vector|BreakVector (* (Math|Rotator|GetRotationXVector (Math|Rotator|FindLookatRotation (Transformation|GetActorLocation) (Transformation|GetActorLocation _array_element))) 5e+03))) (.Y (Math|Vector|BreakVector (* (Math|Rotator|GetRotationXVector (Math|Rotator|FindLookatRotation (Transformation|GetActorLocation) (Transformation|GetActorLocation _array_element))) 5e+03))) 0.0))
        (Utilities|Array|Add (Variables|Default|GetActorsToIgnore) 0)))))

(event EventBeginPlay
  (bind _projectilemovement (Variables|Default|GetProjectileMovement))
  (Utilities|FlowControl|Delay 0.3)
  (Variables|/Script/Engine.MovementComponent|SetVelocity _projectilemovement (* (Variables|/Script/Engine.MovementComponent|GetVelocity _projectilemovement) 5e+03))
  (CallFunction|FindNearPlayer false)
  (Utilities|FlowControl|Delay 1.0)
  (Actor|DestroyActor))

(event EventTick
  (params (DeltaSeconds :type Float%20%28single-precision%29)))

(fn ConstructionScript)