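; Gameplay ability for the Light Staff basic attack, firing a light projectile toward the point under the mouse.
; On activation it commits, gets mouse target data, turns the avatar to face it and plays the attack montage.
; A montage gameplay event triggers the spawn from the weapon socket, and the ability ends when the montage finishes or is interrupted.
; A separate SpawnProject function, uncalled here, spawns a projectile restricted to one target actor.
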(event Ability|EventActivateAbility
  (Ability|CommitAbility)
  (bind _datahandle (|TargetDataUnderMouse)
    (:ValidData
      (Variables|Default|SetTargetLocation (.Location (Collision|BreakHitResult (Ability|TargetData|GetHitResultfromTargetData _datahandle))))
      (bind _ascombat_interface (Utilities|Casting|CastToCombatInterface (Ability|GetAvatarActorfromActorInfo)))
      (Class|CombatInterface|UpdateFacingTarget _ascombat_interface (Variables|Default|GetTargetLocation))
      (|PlayMontageandWaitProxy "FacingTarget" "/Game/Blueprints/AbilitySystem/Character/Abilities/LightStaff/Basic/AnimAsset/AM_LightStaff_Bagic.AM_LightStaff_Bagic" 1.0 "None" false 1.0 0.0 false
        (:then
          (Ability|Tasks|WaitGameplayEvent "(TagName=\"Event.Montage.LightStaff.Basic.Start\")" 0
            (:EventReceived
              (Class|CubeActiveSkill|SpawnProjectile "LightProjectile" "LightDamage" (Variables|Default|GetTargetLocation) (GameplayTags|MakeLiteralGameplayTag "(TagName=\"CombatSocket.Weapon\")") false 0.0 false 0.0 0 false 0))))
        (:OnCompleted
          (Ability|EndAbility :!label _label))
        (:OnBlendOut
          (goto _label))
        (:OnInterrupted
          (goto _label))
        (:OnCancelled
          (goto _label))))))

(fn SpawnProject
  (params (Pitch :type Float%20%28double-precision%29) (Yaw :type Float%20%28double-precision%29) (Target :type Actor%20Object%20Reference))
  (Class|CubeActiveSkill|SpawnProjectile "None" "None" (Variables|Default|GetTargetLocation) (GameplayTags|MakeLiteralGameplayTag "(TagName=\"CombatSocket.Weapon\")") true 0.0 false 0.0 (Ability|GetAvatarActorfromActorInfo) true Target))