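; Projectile for the Light Staff unique ability that homes in on a series of nearby actors.
; After a short launch delay it repeatedly sphere-searches, randomly tries to pick a homing target, and adds picks to an ignore list seeded with the instigator.
; A timeout stops movement, searching and overlap events.
; An overlap destroys it only when the ignore list holds exactly five entries.
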(event OnComponentBeginOverlap(Sphere)
  (params (OverlappedComponent :type Primitive%20Component%20Object%20Reference) (OtherActor :type Actor%20Object%20Reference) (OtherComp :type Primitive%20Component%20Object%20Reference) (OtherBodyIndex :type Integer) (bFromSweep :type Boolean) (SweepResult :type Hit%20Result%20Structure%20%28by%20ref%29))
  (if (== (Utilities|Array|Length (Variables|Default|GetActorsToIgnore)) 5)
    (Actor|DestroyActor)))

(event Custom|FindNearPlayer
  (if (Variables|Default|GetbIsFinding)
    (bind _outactors (Collision|SphereOverlapActors (Transformation|GetWorldLocation (Variables|Default|GetSphere)) 1e+03 (Variables|Default|GetObject%20Types) 0 (Variables|Default|GetActorsToIgnore)))
    (for (_array_element _array_index) _outactors
      (if (== _array_index (Math|Random|RandomInteger (Utilities|Array|Length _outactors)))
        (Variables|/Script/Engine.ProjectileMovementComponent|SetHomingTargetComponent (Variables|Default|GetProjectileMovement) (Variables|/Script/Engine.Actor|GetRootComponent _array_element))
        (Utilities|Array|Add (Variables|Default|GetActorsToIgnore) _array_element)))
    (Utilities|FlowControl|Delay 0.5)
    (CallFunction|FindNearPlayer)))

(event EventBeginPlay
  (bind _projectilemovement (Variables|Default|GetProjectileMovement))
  (bind _projectilemovement_2 (Variables|Default|GetProjectileMovement))
  (Utilities|FlowControl|Sequence
    (:then_0
      (Variables|Default|SetbIsFinding true)
      (Utilities|FlowControl|Delay 0.3)
      (Variables|/Script/Engine.MovementComponent|SetVelocity _projectilemovement (* (Variables|/Script/Engine.MovementComponent|GetVelocity _projectilemovement) 3e+03))
      (CallFunction|FindNearPlayer))
    (:then_1
      (Utilities|FlowControl|Delay 3.0)
      (Variables|/Script/Engine.MovementComponent|SetVelocity _projectilemovement_2 (* (Variables|/Script/Engine.MovementComponent|GetVelocity _projectilemovement_2) ""))
      (Variables|/Script/Engine.PrimitiveComponent|SetbGenerateOverlapEvents (Variables|Default|GetSphere) false)
      (Variables|Default|SetbIsFinding false))
    (:then_2
      (Utilities|Array|Add (Variables|Default|GetActorsToIgnore) (Class|CubeHitActor|GetInstigatorPlayer)))))

(fn ConstructionScript)