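; Light staff unique gameplay ability that fires a vertical fan of nine projectiles from the weapon socket toward the point under the mouse.
; It commits, gets cursor target data, turns the avatar through the combat interface and plays a staff montage.
; The montage's start event triggers the SpawnProject helper with stepped pitch overrides; the later wait for the end event drives nothing.
; The ability ends when the montage completes, blends out or is interrupted or cancelled.
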(event Ability|EventActivateAbility
  (Ability|CommitAbility)
  (bind _datahandle (|TargetDataUnderMouse)
    (:ValidData
      (Variables|Default|SetTargetLocation (.Location (Collision|BreakHitResult (Ability|TargetData|GetHitResultfromTargetData _datahandle))))
      (bind _ascombat_interface (Utilities|Casting|CastToCombatInterface (Ability|GetAvatarActorfromActorInfo)))
      (Class|CombatInterface|UpdateFacingTarget _ascombat_interface (Variables|Default|GetTargetLocation))
      (|PlayMontageandWaitProxy "FacingTarget" "/Game/Blueprints/AbilitySystem/Character/Abilities/LightStaff/Basic/AnimAsset/AM_LightStaff_Bagic.AM_LightStaff_Bagic" 1.0 "None" false 1.0 0.0 false
        (:then
          (Ability|Tasks|WaitGameplayEvent "(TagName=\"Event.Montage.LightStaff.Basic.Start\")" 0
            (:EventReceived
              (CallFunction|SpawnProject 0.0)
              (CallFunction|SpawnProject 1e+01)
              (CallFunction|SpawnProject 2e+01)
              (CallFunction|SpawnProject 3e+01)
              (CallFunction|SpawnProject 4e+01)
              (CallFunction|SpawnProject 5e+01)
              (CallFunction|SpawnProject 6e+01)
              (CallFunction|SpawnProject 7e+01)
              (CallFunction|SpawnProject 8e+01)
              (Ability|Tasks|WaitGameplayEvent "(TagName=\"Event.Montage.LightStaff.Basic.End\")" 0))))
        (:OnCompleted
          (Ability|EndAbility :!label _label))
        (:OnBlendOut
          (goto _label))
        (:OnInterrupted
          (goto _label))
        (:OnCancelled
          (goto _label))))))

(fn SpawnProject
  (params (Pitch :type Float%20%28double-precision%29))
  (Class|CubeProjectileSkill|SpawnProjectile "None" (Variables|Default|GetTargetLocation) (GameplayTags|MakeLiteralGameplayTag "(TagName=\"CombatSocket.Weapon\")") true Pitch false 0.0 (Ability|GetAvatarActorfromActorInfo) false 0))