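; Ninja unique gameplay ability that fires a projectile at the spot or enemy under the mouse.
; Mouse target data sets the target, snapping to the actor's location for enemies, and the avatar turns to face it through CombatInterface.
; A montage plays while a gameplay event triggers the projectile from the weapon socket with pitch override.
; The ability ends shortly after firing or when the montage finishes or is interrupted.
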(event Ability|EventActivateAbility
  (Ability|CommitAbility)
  (bind _datahandle (|TargetDataUnderMouse)
    (:ValidData
      (if (Actor|ActorHasTag (.HitActor (Collision|BreakHitResult (Ability|TargetData|GetHitResultfromTargetData _datahandle))) "Enemy")
        (Variables|Default|SetTargetLocation (Transformation|GetActorLocation (.HitActor (Collision|BreakHitResult (Ability|TargetData|GetHitResultfromTargetData _datahandle)))))
        (else
          (Variables|Default|SetTargetLocation (.Location (Collision|BreakHitResult (Ability|TargetData|GetHitResultfromTargetData _datahandle))))))
      (bind _ascombat_interface (Utilities|Casting|CastToCombatInterface (Ability|GetAvatarActorfromActorInfo)))
      (Class|CombatInterface|UpdateFacingTarget _ascombat_interface (Variables|Default|GetTargetLocation))
      (|PlayMontageandWaitProxy "FacingTarget" "/Game/Blueprints/AbilitySystem/Character/Abilities/Ninja/Unique/AM_Ninja_Unique.AM_Ninja_Unique" 1.0 "None" false 1.0 0.0 false
        (:then
          (Ability|Tasks|WaitGameplayEvent "(TagName=\"Event.Montage.Ninja.Unique\")" 0
            (:EventReceived
              (Class|CubeActiveSkill|SpawnProjectile "NinUni" "NinUni" (Variables|Default|GetTargetLocation) (GameplayTags|MakeLiteralGameplayTag "(TagName=\"CombatSocket.Weapon\")") true 0.0 false 0.0 0 false 0)
              (Ability|Tasks|WaitGameplayEvent "(TagName=\"Event.Montage.Ninja.Unique\")" 0
                (:then
                  (Utilities|FlowControl|Delay 0.2)
                  (Ability|EndAbility))))))
        (:OnCompleted
          (Ability|EndAbility :!label _label))
        (:OnBlendOut
          (goto _label))
        (:OnInterrupted
          (goto _label))
        (:OnCancelled
          (goto _label))))))