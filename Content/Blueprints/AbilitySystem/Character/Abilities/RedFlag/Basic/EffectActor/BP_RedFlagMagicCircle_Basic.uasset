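; Red Flag basic ability's magic circle, an effect actor that acts as a timed area zone and destroys itself after a fixed delay.
; Its box overlap events call OnOverlap and OnEndOverlap for any actor entering or leaving.
; Actors tagged Player also get a Niagara flag buff attached to their root, held in a single Effect variable and destroyed when a player exits.
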(event OnComponentBeginOverlap(Box)
  (params (OverlappedComponent :type Primitive%20Component%20Object%20Reference) (OtherActor :type Actor%20Object%20Reference) (OtherComp :type Primitive%20Component%20Object%20Reference) (OtherBodyIndex :type Integer) (bFromSweep :type Boolean) (SweepResult :type Hit%20Result%20Structure%20%28by%20ref%29))
  (Class|CubeEffectActor|OnOverlap OtherActor)
  (if (Actor|ActorHasTag OtherActor "Player")
    (bind _returnvalue (Niagara|SpawnSystemAttached "/Game/Blueprints/AbilitySystem/Character/Abilities/RedFlag/Basic/EffectActor/NS_FlagBuff.NS_FlagBuff" (Variables|/Script/Engine.Actor|GetRootComponent OtherActor) "EffectSocket" (Transformation|GetActorLocation OtherActor) "0, 0, 0" "KeepWorldPosition" false))
    (Variables|Default|SetEffect _returnvalue)))

(event OnComponentEndOverlap(Box)
  (params (OverlappedComponent :type Primitive%20Component%20Object%20Reference) (OtherActor :type Actor%20Object%20Reference) (OtherComp :type Primitive%20Component%20Object%20Reference) (OtherBodyIndex :type Integer))
  (Class|CubeEffectActor|OnEndOverlap OtherActor)
  (if (Actor|ActorHasTag OtherActor "Player")
    (Utilities|IsValid (Variables|Default|GetEffect)
      (:Is%20Valid
        (Components|DestroyComponent (Variables|Default|GetEffect))))))

(event EventBeginPlay
  (Utilities|FlowControl|Delay 15.0)
  (Actor|DestroyActor))

(fn ConstructionScript)