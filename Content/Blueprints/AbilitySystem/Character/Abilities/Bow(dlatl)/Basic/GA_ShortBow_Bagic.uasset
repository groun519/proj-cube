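; Gameplay ability for the short bow's basic attack, which fires a projectile at the point under the mouse.
; On activation it commits, takes target data from the cursor hit and turns the avatar toward it through CombatInterface.
; It plays the bow montage, whose gameplay event triggers the projectile spawn from the weapon socket with a pitch override.
; The ability ends when the montage completes, blends out, is interrupted or is cancelled.
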(event Ability|EventActivateAbility
  (Ability|CommitAbility)
  (bind _datahandle (|TargetDataUnderMouse)
    (:ValidData
      (Variables|Default|SetTargetLocation (.Location (Collision|BreakHitResult (Ability|TargetData|GetHitResultfromTargetData _datahandle))))
      (bind _ascombat_interface (Utilities|Casting|CastToCombatInterface (Ability|GetAvatarActorfromActorInfo)))
      (Class|CombatInterface|UpdateFacingTarget _ascombat_interface (Variables|Default|GetTargetLocation))
      (|PlayMontageandWaitProxy "FacingTarget" "/Game/Blueprints/AbilitySystem/Character/Abilities/Bow(dlatl)/Basic/AM_ShortBow_Bagic.AM_ShortBow_Bagic" 1.0 "None" false 1.0 0.0 false
        (:then
          (Ability|Tasks|WaitGameplayEvent "(TagName=\"Event.Montage.ShortBow.Basic\")" 0
            (:EventReceived
              (Class|CubeProjectileSkill|SpawnProjectile (Variables|Default|GetTargetLocation) (GameplayTags|MakeLiteralGameplayTag "(TagName=\"CombatSocket.Weapon\")") false 6e+01)
              (Ability|Tasks|WaitGameplayEvent "(TagName=\"\")" 0))))
        (:OnCompleted
          (Ability|EndAbility :!label _label))
        (:OnBlendOut
          (goto _label))
        (:OnInterrupted
          (goto _label))
        (:OnCancelled
          (goto _label))))))