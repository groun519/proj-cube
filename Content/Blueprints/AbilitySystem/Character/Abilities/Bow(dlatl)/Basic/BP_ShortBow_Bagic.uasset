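; BP_ShortBow_Bagic is the actor for the short bow's basic ability, with Niagara, collision sphere and projectile movement components.
; On BeginPlay it registers itself as the Niagara system's export callback.
; Received particle data enables the sphere's overlap events and teleports it through each particle position, so collision follows the effect.
; The actor's own overlap handler is empty, and the velocity-zeroing logic is disconnected.
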(event EventBeginPlay
  (Niagara|SetNiagaraVariable(Object) (Variables|Default|GetNiagara) "User.BPCallback" self))

(event Collision|EventActorBeginOverlap
  (params (OtherActor :type Actor%20Object%20Reference)))

(event EventTick
  (params (DeltaSeconds :type Float%20%28single-precision%29)))

(event EventParticleData
  (params (Data :type Array%20of%20Basic%20Particle%20Data%20Structures) (NiagaraSystem :type Niagara%20System%20Object%20Reference) (SimulationPositionOffset :type Vector%20%28by%20ref%29 :default "0, 0, 0"))
  (Variables|/Script/Engine.PrimitiveComponent|SetbGenerateOverlapEvents (Variables|Default|GetSphere) true)
  (for _array_element Data
    (Transformation|SetWorldLocation (Variables|Default|GetSphere) (.Position (Utilities|Struct|BreakBasicParticleData _array_element)) false true)))

(fn ConstructionScript)