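; Base auto-attack Gameplay Ability: attacks the Player- or Enemy-tagged actor under the cursor with fire staff projectiles.
; Out-of-range targets are approached by SimpleMoveToActor, polling distance every 0.1s.
; An attack-speed-scaled montage waits for Abilities.Attack to spawn a homing projectile, then delays, calls the empty SpawnSmallProj hook and repeats until death.
; Chained input release/press tasks cancel it for movement; CommitAbility is left unwired, so no cooldown applies.
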(event Custom|SpawnSmallProj
  ;[1 1 1] 작은 투사체 생성
)

(event Custom|ReStartAttack
  ;[1 1 1] 공격 몽타주 재생
  (if (not (Variables|UsefulVarriables|GetbIsTargetDead))
    (|PlayMontageandWaitProxy "FacingTarget" "/Game/Blueprints/AbilitySystem/Character/Abilities/FireStaff/Attack/Anim/AM_FireStaff_Attack.AM_FireStaff_Attack" (* (.ReturnValue (Ability|Attribute|GetFloatAttribute (Ability|GetAvatarActorfromActorInfo) "(AttributeName=\"AttackSpeed\",Attribute=/Script/P_Cube.CubeAttributeSet:AttackSpeed,AttributeOwner=\"/Script/CoreUObject.Class'/Script/P_Cube.CubeAttributeSet'\")")) (+ (Variables|Default|GetPreDelay) 0.1)) "None" true 1.0 0.0 true
      (:then
        (Ability|Tasks|WaitGameplayEvent "(TagName=\"Abilities.Attack\")" 0 true
          (:EventReceived
            ;[1 1 1] 큰 투사체 생성
            (Variables|UsefulVarriables|SetHomingFeacher (Utilities|Struct|MakeHomingFeacher true 2e+02 2e+04 (Variables|MouseData|GetHitTarget)))
            (Class|CubeActiveSkill|SpawnProjectile "AttackProj_Big" "FireStaff_Big_Attack" (Variables|MouseData|GetTargetLocation) (GameplayTags|MakeLiteralGameplayTag "(TagName=\"CombatSocket.Weapon\")") false 0.0 false 0.0 (Ability|GetAvatarActorfromActorInfo) true (Variables|MouseData|GetHitTarget) "(bUseMultipleProjectilesFeacher=False,ProjectileSpread=90.000000,NumProjectiles=1,MaxNumProjectiles=1,UpgradeProjectiles=1)" (Variables|UsefulVarriables|GetHomingFeacher))
            ;[1 1 1] 후딜레이 처리 / 작은 투사체 소환 / 다시 공격
            (Utilities|FlowControl|Delay (Variables|Default|GetPostDelay))
            (CallFunction|SpawnSmallProj)
            (bind _returnvalue (Class|CombatInterface|IsDead(Message) (Variables|MouseData|GetHitTarget)))
            (Variables|UsefulVarriables|SetbIsTargetDead _returnvalue)
            (if (< (Variables|MouseData|GetDistance) (Variables|Default|GetMaxDistance))
              (CallFunction|ReStartAttack)
              (else
                (CallFunction|MovetoTarget)))))))))

(event Custom|MoveToTarget
  (bind _returnvalue (Ability|GetAvatarActorfromActorInfo))
  (bind _returnvalue_2 (Ability|GetAvatarActorfromActorInfo))
  (bind _hittarget (Variables|MouseData|GetHitTarget))
  (bind _returnvalue_3 (Ability|Attribute|GetFloatAttribute _returnvalue "(AttributeName=\"AttackSpeed\",Attribute=/Script/P_Cube.CubeAttributeSet:AttackSpeed,AttributeOwner=\"/Script/CoreUObject.Class'/Script/P_Cube.CubeAttributeSet'\")"))
  (bind _returnvalue_4 (Transformation|GetDistanceTo _hittarget _returnvalue_2))
  ;[1 1 1] 타겟에게 이동
  (AI|Navigation|SimpleMovetoActor (Game|GetPlayerController 0) (Variables|MouseData|GetHitTarget))
  (Utilities|FlowControl|Delay 0.1)
  (bind _output_get (Variables|MouseData|SetDistance _returnvalue_4))
  (Development|PrintString (Utilities|String|Append "Dist : " (Utilities|String|ToString(Integer) (Math|Float|Truncate _returnvalue_4)) " : " (Utilities|String|ToString(Integer) (Math|Float|Truncate (Variables|Default|GetMaxDistance)))) (Variables|Debug|GetbShowDebug_Distance) false "(R=1.000000,G=0.000000,B=0.901964,A=1.000000)")
  (if (< _output_get (Variables|Default|GetMaxDistance))
    ;[1 1 1] 거리 계산
    (if (< (Variables|MouseData|GetDistance) (Variables|Default|GetMaxDistance))
      (Variables|MouseData|SetTargetLocation (.Location (Collision|BreakHitResult (Ability|TargetData|GetHitResultfromTargetData (stale Ability|EventActivateAbility _datahandle)))))
      ;[1 1 1] 플레이어/몬스터만 공격 가능하게 함.
      (if (or (Actor|ActorHasTag (Variables|MouseData|GetHitTarget) "Player") (Actor|ActorHasTag (Variables|MouseData|GetHitTarget) "Enemy"))
        ;[1 1 1] Facing Target
        (Class|CombatInterface|UpdateFacingTarget(Message) (Ability|GetAvatarActorfromActorInfo) (Variables|MouseData|GetTargetLocation))
        ;[1 1 1] 후딜레이가 0.03 아래로 가면 서버 딜레이 때문에 평타가 안나가기 때문에, 방지 차원에서 0.03을 최소치로 설정
        (Variables|Default|SetPostDelay (Math|Float|Max(Float) 0.03 (Math|Float|SafeDivide (Variables|Default|GetPostDelay) _returnvalue_3)))
        ;[1 1 1] 공격 몽타주 재생
        (|PlayMontageandWaitProxy "FacingTarget" "/Game/Blueprints/AbilitySystem/Character/Abilities/FireStaff/Attack/Anim/AM_FireStaff_Attack.AM_FireStaff_Attack" (* _returnvalue_3 (+ (Variables|Default|GetPreDelay) 0.1)) "None" true 1.0 0.0 true
          (:then
            (Ability|Tasks|WaitGameplayEvent "(TagName=\"Abilities.Attack\")" 0 true
              (:EventReceived
                ;[1 1 1] 큰 투사체 생성
                (Variables|UsefulVarriables|SetHomingFeacher (Utilities|Struct|MakeHomingFeacher true 2e+02 2e+04 (Variables|MouseData|GetHitTarget)))
                (Class|CubeActiveSkill|SpawnProjectile "AttackProj_Big" "FireStaff_Big_Attack" (Variables|MouseData|GetTargetLocation) (GameplayTags|MakeLiteralGameplayTag "(TagName=\"CombatSocket.Weapon\")") false 0.0 false 0.0 (Ability|GetAvatarActorfromActorInfo) true (Variables|MouseData|GetHitTarget) "(bUseMultipleProjectilesFeacher=False,ProjectileSpread=90.000000,NumProjectiles=1,MaxNumProjectiles=1,UpgradeProjectiles=1)" (Variables|UsefulVarriables|GetHomingFeacher))
                ;[1 1 1] 후딜레이 처리 / 작은 투사체 소환 / 다시 공격
                (Utilities|FlowControl|Delay (Variables|Default|GetPostDelay))
                (CallFunction|SpawnSmallProj)
                (bind _returnvalue_5 (Class|CombatInterface|IsDead(Message) (Variables|MouseData|GetHitTarget)))
                (Variables|UsefulVarriables|SetbIsTargetDead _returnvalue_5)
                (if (< (Variables|MouseData|GetDistance) (Variables|Default|GetMaxDistance))
                  (CallFunction|ReStartAttack)
                  (else
                    (CallFunction|MovetoTarget)))))))
        (else
          (Ability|CancelAbility)))
      (else
        (CallFunction|MovetoTarget)))
    (else
      (CallFunction|MovetoTarget))))

(event Ability|EventActivateAbility
  (bind _returnvalue (Ability|GetAvatarActorfromActorInfo))
  (bind _returnvalue_2 (Ability|Attribute|GetFloatAttribute _returnvalue "(AttributeName=\"AttackSpeed\",Attribute=/Script/P_Cube.CubeAttributeSet:AttackSpeed,AttributeOwner=\"/Script/CoreUObject.Class'/Script/P_Cube.CubeAttributeSet'\")"))
  (bind _datahandle (|TargetDataUnderMouse)
    (:ValidData
      ;[1 1 1] 타겟이 유효한가?
      (bind _output_get (Variables|MouseData|SetHitTarget (.HitActor (Collision|BreakHitResult (Ability|TargetData|GetHitResultfromTargetData _datahandle)))))
      (Utilities|IsValid _output_get
        (:Is%20Valid
          (bind _asbp_cube_character (Utilities|Casting|CastToBP_CubeCharacter (Ability|GetAvatarActorfromActorInfo)))
          (bind _output_get_2 (Variables|Default|SetCharacter _asbp_cube_character))
          (Variables|/Game/Blueprints/Character/PlayerCharacter/BP_CubeCharacter.BP_CubeCharacter_C|SetTargetCharacter _output_get_2 _output_get)
          (Utilities|FlowControl|Sequence
            (:then_0
              ;[1 1 1] 거리 계산
              (Variables|MouseData|SetDistance (Transformation|GetDistanceTo (Variables|MouseData|GetHitTarget) (Ability|GetAvatarActorfromActorInfo)))
              (if (< (Variables|MouseData|GetDistance) (Variables|Default|GetMaxDistance))
                (Variables|MouseData|SetTargetLocation (.Location (Collision|BreakHitResult (Ability|TargetData|GetHitResultfromTargetData _datahandle))))
                ;[1 1 1] 플레이어/몬스터만 공격 가능하게 함.
                (if (or (Actor|ActorHasTag (Variables|MouseData|GetHitTarget) "Player") (Actor|ActorHasTag (Variables|MouseData|GetHitTarget) "Enemy"))
                  ;[1 1 1] Facing Target
                  (Class|CombatInterface|UpdateFacingTarget(Message) (Ability|GetAvatarActorfromActorInfo) (Variables|MouseData|GetTargetLocation))
                  ;[1 1 1] 후딜레이가 0.03 아래로 가면 서버 딜레이 때문에 평타가 안나가기 때문에, 방지 차원에서 0.03을 최소치로 설정
                  (Variables|Default|SetPostDelay (Math|Float|Max(Float) 0.03 (Math|Float|SafeDivide (Variables|Default|GetPostDelay) _returnvalue_2)))
                  ;[1 1 1] 공격 몽타주 재생
                  (|PlayMontageandWaitProxy "FacingTarget" "/Game/Blueprints/AbilitySystem/Character/Abilities/FireStaff/Attack/Anim/AM_FireStaff_Attack.AM_FireStaff_Attack" (* _returnvalue_2 (+ (Variables|Default|GetPreDelay) 0.1)) "None" true 1.0 0.0 true
                    (:then
                      (Ability|Tasks|WaitGameplayEvent "(TagName=\"Abilities.Attack\")" 0 true
                        (:EventReceived
                          ;[1 1 1] 큰 투사체 생성
                          (Variables|UsefulVarriables|SetHomingFeacher (Utilities|Struct|MakeHomingFeacher true 2e+02 2e+04 (Variables|MouseData|GetHitTarget)))
                          (Class|CubeActiveSkill|SpawnProjectile "AttackProj_Big" "FireStaff_Big_Attack" (Variables|MouseData|GetTargetLocation) (GameplayTags|MakeLiteralGameplayTag "(TagName=\"CombatSocket.Weapon\")") false 0.0 false 0.0 (Ability|GetAvatarActorfromActorInfo) true (Variables|MouseData|GetHitTarget) "(bUseMultipleProjectilesFeacher=False,ProjectileSpread=90.000000,NumProjectiles=1,MaxNumProjectiles=1,UpgradeProjectiles=1)" (Variables|UsefulVarriables|GetHomingFeacher))
                          ;[1 1 1] 후딜레이 처리 / 작은 투사체 소환 / 다시 공격
                          (Utilities|FlowControl|Delay (Variables|Default|GetPostDelay))
                          (CallFunction|SpawnSmallProj)
                          (bind _returnvalue_3 (Class|CombatInterface|IsDead(Message) (Variables|MouseData|GetHitTarget)))
                          (Variables|UsefulVarriables|SetbIsTargetDead _returnvalue_3)
                          (if (< (Variables|MouseData|GetDistance) (Variables|Default|GetMaxDistance))
                            (CallFunction|ReStartAttack)
                            (else
                              (CallFunction|MovetoTarget)))))))
                  (else
                    (Ability|CancelAbility)))
                (else
                  (CallFunction|MovetoTarget))))
            (:then_1
              ;[1 1 1] 이게 왜 되는건지 모르겠지만 이동 평캔
              (Ability|Tasks|WaitInputRelease false
                (:OnRelease
                  (Development|PrintString "Release" (Variables|Debug|GetbShowDebug_CancelToMove) false "(R=0.000000,G=1.000000,B=0.003194,A=1.000000)")
                  (Ability|Tasks|WaitInputPress false
                    (:OnPress
                      (Development|PrintString "Wait" (Variables|Debug|GetbShowDebug_CancelToMove) false "(R=1.000000,G=0.957500,B=0.000000,A=1.000000)")
                      (Ability|Tasks|WaitInputPress false
                        (:OnPress
                          (Development|PrintString "Cancel" (Variables|Debug|GetbShowDebug_CancelToMove) false "(R=1.000000,G=0.016900,B=0.000000,A=1.000000)")
                          (AI|Navigation|StopMovement (Game|GetPlayerController 0))
                          (Ability|CancelAbility))))))))))
        (:Is%20Not%20Valid
          (Ability|CancelAbility))))))

(event Ability|EventOnEndAbility
  (params (bWasCancelled :type Boolean))
  (Variables|/Game/Blueprints/Character/PlayerCharacter/BP_CubeCharacter.BP_CubeCharacter_C|SetTargetCharacter (Variables|Default|GetCharacter) 0))