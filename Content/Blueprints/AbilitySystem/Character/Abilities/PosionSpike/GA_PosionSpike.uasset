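; Gameplay ability for Poison Spike, which fires a staff projectile toward the point or enemy under the cursor.
; On activation it commits, reads mouse target data, snaps to the actor location of Enemy-tagged hits and turns the avatar through CombatInterface.
; A fire-staff montage event triggers the projectile spawn from the weapon socket with a pitch override.
; The ability ends after a short delay once the montage finishes or is interrupted.
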(event Ability|EventActivateAbility
  (Ability|CommitAbility)
  (bind _datahandle (|TargetDataUnderMouse)
    (:ValidData
      (if (Actor|ActorHasTag (.HitActor (Collision|BreakHitResult (Ability|TargetData|GetHitResultfromTargetData _datahandle))) "Enemy")
        (Variables|Default|SetTargetLocation (Transformation|GetActorLocation (.HitActor (Collision|BreakHitResult (Ability|TargetData|GetHitResultfromTargetData _datahandle)))))
        (else
          (Variables|Default|SetTargetLocation (.Location (Collision|BreakHitResult (Ability|TargetData|GetHitResultfromTargetData _datahandle))))))
      (bind _ascombat_interface (Utilities|Casting|CastToCombatInterface (Ability|GetAvatarActorfromActorInfo)))
      (Class|CombatInterface|UpdateFacingTarget _ascombat_interface (Variables|Default|GetTargetLocation))
      (|PlayMontageandWaitProxy "FacingTarget" "/Game/Blueprints/AbilitySystem/Character/Abilities/FireStaff/Unique/AnimAsset/AM_FireStaff_Unique.AM_FireStaff_Unique" 1.0 "None" true 1.0 0.0 false
        (:then
          (Ability|Tasks|WaitGameplayEvent "(TagName=\"Event.Montage.FireStaff.Unique\")" 0
            (:EventReceived
              (Class|CubeActiveSkill|SpawnProjectile "Proj" "FireStaff_Unique_Damage" (Variables|Default|GetTargetLocation) (GameplayTags|MakeLiteralGameplayTag "(TagName=\"CombatSocket.Weapon\")") true -5.0 false 0.0 0 false 0 "(bUseMultipleProjectilesFeacher=False,ProjectileSpread=90.000000,NumProjectiles=1,MaxNumProjectiles=1,UpgradeProjectiles=1)" "(bUseHomingFeacher=False,HomingAccelerationMin=1600.000000,HomingAccelerationMax=3200.000000,HomingTarget=None)"))))
        (:OnCompleted
          (Utilities|FlowControl|Delay 3.0 :!label _label)
          (Ability|EndAbility))
        (:OnBlendOut
          (goto _label))
        (:OnInterrupted
          (goto _label))
        (:OnCancelled
          (goto _label))))))