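; Mana arrow projectile for a passive skill, which homes toward a target actor.
; Shortly after spawn it sets a very high homing acceleration on its ProjectileMovement.
; Each tick it asks the target whether it is dead and, if so, destroys itself after a short delay.
; A stall check that explodes the arrow with impact sound and Niagara effect, and a velocity boost, exist but are not connected.
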(event EventBeginPlay
  (Utilities|FlowControl|Delay 0.2)
  (Variables|/Script/Engine.ProjectileMovementComponent|SetHomingAccelerationMagnitude (Variables|Default|GetProjectileMovement) 1e+05))

(event EventTick
  (params (DeltaSeconds :type Float%20%28single-precision%29))
  (bind _returnvalue (Class|CombatInterface|IsDead(Message) (Class|CubeHitActor|GetTargetActor)))
  (if _returnvalue
    (Utilities|FlowControl|Delay 0.5)
    (Actor|DestroyActor)))

(fn ConstructionScript)

(fn MakeGoKaboomifNoMove
  (Variables|Default|SetLocationLastFrame (Variables|Default|GetLocationThisFrame))
  (Variables|Default|SetLocationThisFrame (Transformation|GetActorLocation))
  (if (<= (Math|Vector|VectorLength (- (Variables|Default|GetLocationThisFrame) (Variables|Default|GetLocationLastFrame))) (Variables|Default|GetMinDistancePerFrame))
    (Audio|SpawnSoundatLocation "/Game/Blueprints/AbilitySystem/Character/Abilities/FireStaff/Basic/Sound/FireStaff_Basic_Impact.FireStaff_Basic_Impact" (Variables|Default|GetLocationThisFrame) "0, 0, 0" 1.0 1.0 0.0 0 0)
    (Niagara|SpawnSystematLocation "/Game/Blueprints/AbilitySystem/Character/Abilities/LightStaff/Basic/EffectAsset/N_LightStaff_Bagic.N_LightStaff_Bagic" (Variables|Default|GetLocationThisFrame))
    (Actor|DestroyActor)))