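; Passive gameplay ability that fires a homing mana arrow on every third attack by the cube character.
; It listens for attack gameplay events with a one-shot wait task that re-arms itself after each event and increments a stack counter.
; At the threshold it launches a pitched projectile from the weapon socket that homes on and hits only the current attack target, then resets the counter.
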(event Ability|EventActivateAbility
  (Development|PrintString "Hello" true true "(R=1.000000,G=0.000000,B=0.894553,A=1.000000)")
  (bind _asbp_cube_character (Utilities|Casting|CastToBP_CubeCharacter (Ability|GetAvatarActorfromActorInfo)))
  (Variables|Default|SetCharacter _asbp_cube_character)
  (Ability|Tasks|WaitGameplayEvent "(TagName=\"Abilities.Attack\")" 0 true :!label _label
    (:EventReceived
      (Math|Integer|IncrementInt (Variables|Default|GetStack)
        (:%20%20
          (Utilities|FlowControl|Sequence
            (:then_0
              (goto _label))
            (:then_1
              (if (== (Variables|Default|GetStack) 3)
                (Class|CubeActiveSkill|SpawnProjectile "Projectile" "Damage" (Transformation|GetActorLocation (Variables|/Script/P_Cube.CubeCharacter|GetAttackTarget (Variables|Default|GetCharacter))) (GameplayTags|MakeLiteralGameplayTag "(TagName=\"CombatSocket.Weapon\")") true 5e+01 false 0.0 0 true (Variables|/Script/P_Cube.CubeCharacter|GetAttackTarget (Variables|Default|GetCharacter)) "(bUseMultipleProjectilesFeacher=False,ProjectileSpread=90.000000,NumProjectiles=1,MaxNumProjectiles=1,UpgradeProjectiles=1)" (Utilities|Struct|MakeHomingFeacher true 1.6e+03 3.2e+03 (Variables|/Script/P_Cube.CubeCharacter|GetAttackTarget (Variables|Default|GetCharacter))))
                (Variables|Default|SetStack 0)))))))))

(event Ability|EventOnEndAbility
  (params (bWasCancelled :type Boolean))
  (Development|PrintString "Hello" true true "(R=1.000000,G=0.000000,B=0.031401,A=1.000000)"))