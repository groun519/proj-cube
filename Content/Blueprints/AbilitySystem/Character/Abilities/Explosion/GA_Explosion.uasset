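; GA_Explosion is a gameplay ability that casts a mouse-targeted explosion.
; On activation it shows a scaled targeting decal, then on input release hides it, takes target data under the mouse and turns the avatar toward that point.
; A fire staff montage's gameplay event spawns the damage hitbox there, scaled by the same Size as the decal.
; Each hit then increments and prints Size before ending the ability after a short delay.
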(event Ability|EventActivateAbility
  (Utilities|FlowControl|Sequence
    (:then_0
      (Class|PlayerInterface|ShowDecalEffectActor(Message) (Ability|GetAvatarActorfromActorInfo) (Math|Vector|MakeVector (* (Variables|Default|GetSize) 0.75) (* (Variables|Default|GetSize) 0.75) (* (Variables|Default|GetSize) 0.75)) 0))
    (:then_1
      (Ability|Tasks|WaitInputRelease false
        (:OnRelease
          (Class|PlayerInterface|HideDecalEffectActor(Message) (Ability|GetAvatarActorfromActorInfo))
          (bind _datahandle (|TargetDataUnderMouse)
            (:ValidData
              (Variables|Default|SetSpawnLoc (.Location (Collision|BreakHitResult (Ability|TargetData|GetHitResultfromTargetData _datahandle))))
              (Class|CombatInterface|UpdateFacingTarget(Message) (Ability|GetAvatarActorfromActorInfo) (Variables|Default|GetSpawnLoc))
              (|PlayMontageandWaitProxy "None" "/Game/Blueprints/AbilitySystem/Character/Abilities/Explosion/AM_FireStaff_Bagic.AM_FireStaff_Bagic" 1.0 "None" false 1.0 0.0 false
                (:then
                  (Ability|Tasks|WaitGameplayEvent "(TagName=\"Event.Montage.Explosion\")" 0 true
                    (:EventReceived
                      (Class|CubeActiveSkill|SpawnHitBox "Hitbox" "Damage" (Math|Transform|MakeTransform (Variables|Default|GetSpawnLoc) "0, 0, 0" (Math|Vector|MakeVector (* (Variables|Default|GetSize) 0.75) (* (Variables|Default|GetSize) 0.75) (* (Variables|Default|GetSize) 0.75))) false 0 0)
                      (bind _output_get (Variables|Default|SetSize (+ (Variables|Default|GetSize) 0.1)))
                      (Development|PrintString (Utilities|String|ToString(Float) _output_get))
                      (Utilities|FlowControl|Delay 0.2)
                      (Ability|EndAbility))))))))))))