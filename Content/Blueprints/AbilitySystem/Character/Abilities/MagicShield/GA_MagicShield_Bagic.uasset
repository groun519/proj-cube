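; Gameplay ability that casts a temporary magic shield, which fires a projectile when hit.
; It faces the avatar toward the target under the mouse, plays a montage, and uses montage gameplay events to spawn the shield on player 0's left hand and later destroy it.
; Shield hits spawn a projectile from the weapon socket.
; Interruption or cancellation ends the ability after a short delay, without destroying the shield.
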(event Custom|CustomEvent
  (Class|CubeProjectileSkill|SpawnProjectile (+ (Transformation|GetSocketLocation (Variables|/Script/Engine.Character|GetMesh (Game|GetPlayerCharacter 0)) "None") "1.000000,0.000000,0.000000") (GameplayTags|MakeLiteralGameplayTag "(TagName=\"CombatSocket.Weapon\")")))

(event Ability|EventActivateAbility
  (bind _datahandle (|TargetDataUnderMouse)
    (:ValidData
      (Variables|Default|SetTargetLocation (.Location (Collision|BreakHitResult (Ability|TargetData|GetHitResultfromTargetData _datahandle))))
      (bind _ascombat_interface (Utilities|Casting|CastToCombatInterface (Ability|GetAvatarActorfromActorInfo)))
      (Class|CombatInterface|UpdateFacingTarget _ascombat_interface (Variables|Default|GetTargetLocation))
      (|PlayMontageandWaitProxy "FacingTarget" "/Game/Blueprints/AbilitySystem/Character/Abilities/MagicShield/AM_MagicShield_Bagic.AM_MagicShield_Bagic" 1.0 "None" true 1.0 0.0 false
        (:then
          (Ability|Tasks|WaitGameplayEvent "(TagName=\"Event.Montage.MagicShield.Basic.Start\")" 0
            (:EventReceived
              (bind _returnvalue (Game|SpawnActorfromClass "/Game/Blueprints/AbilitySystem/Character/Abilities/MagicShield/BP_MagicSheld.BP_MagicSheld_C" (Math|Transform|MakeTransform "0, 0, 0") "Undefined" "MultiplyWithRoot" 0 0))
              (bind _output_get (Variables|Default|SetMagicSheld _returnvalue))
              (Transformation|AttachComponentToComponent _output_get (Variables|/Script/Engine.Character|GetMesh (Game|GetPlayerCharacter 0)) "LeftHand" "SnapToTarget" "KeepRelative" "KeepRelative" true)
              (EventDispatchers|BindEventtoOnMagicShieldHit (Variables|Default|GetMagicSheld) (delegate Custom|CustomEvent))
              (Ability|Tasks|WaitGameplayEvent "(TagName=\"Event.Montage.MagicShield.Basic.End\")" 0
                (:EventReceived
                  (Actor|DestroyActor (Variables|Default|GetMagicSheld)))))))
        (:OnInterrupted
          _)
        (:OnCancelled
          _))
      (Utilities|FlowControl|Delay 0.5)
      (Ability|EndAbility))))