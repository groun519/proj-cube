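; Gameplay ability for the poison arrow, firing a seven-projectile longbow fan toward the point under the mouse.
; It turns the avatar to the target and plays the basic longbow montage, whose gameplay event spawns a weapon-socket hitbox and the arrows.
; Each activation appends symmetric yaw offsets to an array that SpawnArrow loops over.
; Montage, projectile and damage all use longbow names, with nothing poison-specific.
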(event Ability|EventActivateAbility
  (bind _yawoffset (Variables|Default|GetYawOffset))
  (Ability|CommitAbility)
  (bind _datahandle (|TargetDataUnderMouse)
    (:ValidData
      (Variables|Default|SetTargetLocation (.Location (Collision|BreakHitResult (Ability|TargetData|GetHitResultfromTargetData _datahandle))))
      (Utilities|Array|AppendArray (Variables|Default|GetYawOvrrides) (Utilities|Array|MakeArray (* _yawoffset -3.0) (* _yawoffset -2.0) (* _yawoffset -1.0) 0.0 _yawoffset (* _yawoffset 2.0) (* _yawoffset 3.0)))
      (bind _ascombat_interface (Utilities|Casting|CastToCombatInterface (Ability|GetAvatarActorfromActorInfo)))
      (Class|CombatInterface|UpdateFacingTarget _ascombat_interface (Variables|Default|GetTargetLocation))
      (|PlayMontageandWaitProxy "FacingTarget" "/Game/Blueprints/AbilitySystem/Character/Abilities/LongBow/Basic/AM_LongBow_Basic.AM_LongBow_Basic" 1.0 "None" true 1.0 0.0 false
        (:then
          (Ability|Tasks|WaitGameplayEvent "(TagName=\"Abilities.LongBow.Basic\")" 0
            (:EventReceived
              (bind _returnvalue (Class|CombatInterface|GetCombatSocketLocation(Message) (Ability|GetAvatarActorfromActorInfo) (GameplayTags|MakeLiteralGameplayTag "(TagName=\"CombatSocket.Weapon\")")))
              (Class|CubeActiveSkill|SpawnHitBox "LongBow" "D_LongBow_Basic" (Math|Conversions|ToTransform(Vector) _returnvalue) false 0 0)
              (CallFunction|SpawnArrow)
              (Utilities|FlowControl|Delay 0.2)
              (Ability|EndAbility))))
        (:OnCompleted
          (Ability|EndAbility :!label _label))
        (:OnBlendOut
          (goto _label))
        (:OnInterrupted
          (goto _label))
        (:OnCancelled
          (goto _label))))))

(fn SpawnArrow
  (for _array_element (Variables|Default|GetYawOvrrides)
    (Class|CubeActiveSkill|SpawnProjectile "PT_LongBow" "D_LongBow_Basic" (Variables|Default|GetTargetLocation) (GameplayTags|MakeLiteralGameplayTag "(TagName=\"CombatSocket.ActorLocation\")") true 0.0 true _array_element 0 false 0 "(bUseMultipleProjectilesFeacher=False,ProjectileSpread=90.000000,NumProjectiles=1,MaxNumProjectiles=1,UpgradeProjectiles=1)" "(bUseHomingFeacher=False,HomingAccelerationMin=1600.000000,HomingAccelerationMax=3200.000000,HomingTarget=None)")))