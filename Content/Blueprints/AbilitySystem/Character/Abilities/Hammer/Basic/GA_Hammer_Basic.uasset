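; Gameplay ability for the basic hammer attack, aimed at the target location under the mouse.
; It commits, turns the avatar toward the target and plays the hammer montage with scaled root motion.
; A montage gameplay event spawns a damage hitbox at the weapon socket, then the ability ends after a short delay.
; Interruption or cancellation also ends it after a delay; an unconnected two-hit event chain never runs.
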(event Ability|EventActivateAbility
  (Ability|CommitAbility)
  (bind _datahandle (|TargetDataUnderMouse)
    (:ValidData
      (Variables|Default|SetTargetLocation (.Location (Collision|BreakHitResult (Ability|TargetData|GetHitResultfromTargetData _datahandle))))
      (bind _ascombat_interface (Utilities|Casting|CastToCombatInterface (Ability|GetAvatarActorfromActorInfo)))
      (Class|CombatInterface|UpdateFacingTarget _ascombat_interface (Variables|Default|GetTargetLocation))
      (|PlayMontageandWaitProxy "FacingTarget" "/Game/Blueprints/AbilitySystem/Character/Abilities/Hammer/Basic/AM_Hammer_Basic.AM_Hammer_Basic" 1.0 "None" true 1.25 0.0 false
        (:then
          (Ability|Tasks|WaitGameplayEvent "(TagName=\"Abilities.Hammer.Basic\")" 0
            (:EventReceived
              (bind _returnvalue (Class|CombatInterface|GetCombatSocketLocation(Message) (Ability|GetAvatarActorfromActorInfo) (GameplayTags|MakeLiteralGameplayTag "(TagName=\"CombatSocket.Weapon\")")))
              (Class|CubeActiveSkill|SpawnHitBox "Hammer" "D_Hammer_Basic" (Math|Conversions|ToTransform(Vector) _returnvalue) false 0 0)
              (Utilities|FlowControl|Delay 0.25)
              (Ability|EndAbility))))
        (:OnInterrupted
          (Utilities|FlowControl|Delay 0.5 :!label _label)
          (Ability|EndAbility))
        (:OnCancelled
          (goto _label))))))