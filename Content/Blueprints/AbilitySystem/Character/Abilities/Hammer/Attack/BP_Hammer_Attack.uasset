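; Hammer attack projectile actor in the ability system, with its launched object held in a component named LongBow.
; On BeginPlay it waits a zero-length delay, then multiplies the ProjectileMovement velocity to launch speed.
; On any Sphere overlap it detaches LongBow, disables its collision and teleports it far below the world, then destroys the actor after a short delay.
; The graph applies no damage itself.
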(event OnComponentBeginOverlap(Sphere)
  (params (OverlappedComponent :type Primitive%20Component%20Object%20Reference) (OtherActor :type Actor%20Object%20Reference) (OtherComp :type Primitive%20Component%20Object%20Reference) (OtherBodyIndex :type Integer) (bFromSweep :type Boolean) (SweepResult :type Hit%20Result%20Structure%20%28by%20ref%29))
  (Transformation|DetachFromComponent (Variables|Default|GetLongBow) "KeepWorld" "KeepWorld" "KeepWorld" true)
  (Collision|SetCollisionEnabled (Variables|Default|GetLongBow) "NoCollision")
  (Transformation|SetWorldLocation (Variables|Default|GetLongBow) "0.000000,0.000000,-100000.000000" false true)
  (Utilities|FlowControl|Delay 1.0)
  (Actor|DestroyActor))

(event EventBeginPlay
  (bind _projectilemovement (Variables|Default|GetProjectileMovement))
  (Utilities|FlowControl|Delay 0.0)
  (Variables|/Script/Engine.MovementComponent|SetVelocity _projectilemovement (* (Variables|/Script/Engine.MovementComponent|GetVelocity _projectilemovement) 4e+03)))

(fn ConstructionScript)