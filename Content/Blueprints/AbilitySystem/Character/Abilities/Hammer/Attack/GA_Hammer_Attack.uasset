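; Gameplay ability for the hammer attack, which faces the avatar toward the point under the mouse and strikes.
; It commits, turns the avatar through the combat interface using mouse target data, then plays the attack montage.
; The montage's hammer attack gameplay event spawns a damage hitbox at the weapon socket and ends the ability.
; Interruption or cancellation only runs a short delay, without ending the ability.
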(event Ability|EventActivateAbility
  (Ability|CommitAbility)
  (bind _datahandle (|TargetDataUnderMouse)
    (:ValidData
      (Variables|Default|SetTargetLocation (.Location (Collision|BreakHitResult (Ability|TargetData|GetHitResultfromTargetData _datahandle))))
      (bind _ascombat_interface (Utilities|Casting|CastToCombatInterface (Ability|GetAvatarActorfromActorInfo)))
      (Class|CombatInterface|UpdateFacingTarget _ascombat_interface (Variables|Default|GetTargetLocation))
      (|PlayMontageandWaitProxy "FacingTarget" "/Game/Blueprints/AbilitySystem/Character/Abilities/Hammer/Attack/AM_Hammer_Attack.AM_Hammer_Attack" 1.0 "None" true 1.0 0.0 false
        (:then
          (Ability|Tasks|WaitGameplayEvent "(TagName=\"Abilities.Hammer.Attack\")" 0
            (:EventReceived
              (bind _returnvalue (Class|CombatInterface|GetCombatSocketLocation(Message) (Ability|GetAvatarActorfromActorInfo) (GameplayTags|MakeLiteralGameplayTag "(TagName=\"CombatSocket.Weapon\")")))
              (Class|CubeActiveSkill|SpawnHitBox "Hammer" "D_Hammer_Attack" (Math|Conversions|ToTransform(Vector) _returnvalue) false 0 0)
              (Ability|EndAbility))))
        (:OnInterrupted
          (Utilities|FlowControl|Delay 0.5 :!label _label))
        (:OnCancelled
          (goto _label))))))