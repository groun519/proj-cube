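; Gameplay ability for the hammer's unique attack, a montage-driven swing that deals four timed hits.
; On activation it commits, turns the avatar toward the target under the mouse through CombatInterface, and plays the montage with scaled root motion.
; Four chained gameplay event waits each spawn a damage hitbox at the weapon socket, and the last ends the ability.
; Montage interruption or cancellation only runs a short delay, without ending the ability.
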(event Ability|EventActivateAbility
  (Ability|CommitAbility)
  (bind _datahandle (|TargetDataUnderMouse)
    (:ValidData
      (Variables|Default|SetTargetLocation (.Location (Collision|BreakHitResult (Ability|TargetData|GetHitResultfromTargetData _datahandle))))
      (bind _ascombat_interface (Utilities|Casting|CastToCombatInterface (Ability|GetAvatarActorfromActorInfo)))
      (Class|CombatInterface|UpdateFacingTarget _ascombat_interface (Variables|Default|GetTargetLocation))
      (|PlayMontageandWaitProxy "FacingTarget" "/Game/Blueprints/AbilitySystem/Character/Abilities/Hammer/Unique/AM_Hammer_Unique.AM_Hammer_Unique" 1.0 "None" true 1.25 0.0 false
        (:then
          (Ability|Tasks|WaitGameplayEvent "(TagName=\"Abilities.Hammer.Unique\")" 0
            (:EventReceived
              (bind _returnvalue (Class|CombatInterface|GetCombatSocketLocation(Message) (Ability|GetAvatarActorfromActorInfo) (GameplayTags|MakeLiteralGameplayTag "(TagName=\"CombatSocket.Weapon\")")))
              (Class|CubeActiveSkill|SpawnHitBox "Hammer" "D_Hammer_Unique" _returnvalue 0 0)
              (Ability|Tasks|WaitGameplayEvent "(TagName=\"Abilities.Hammer.Unique\")" 0
                (:EventReceived
                  (bind _returnvalue_2 (Class|CombatInterface|GetCombatSocketLocation(Message) (Ability|GetAvatarActorfromActorInfo) (GameplayTags|MakeLiteralGameplayTag "(TagName=\"CombatSocket.Weapon\")")))
                  (Class|CubeActiveSkill|SpawnHitBox "Hammer" "D_Hammer_Unique" _returnvalue_2 0 0)
                  (Ability|Tasks|WaitGameplayEvent "(TagName=\"Abilities.Hammer.Unique\")" 0
                    (:EventReceived
                      (bind _returnvalue_3 (Class|CombatInterface|GetCombatSocketLocation(Message) (Ability|GetAvatarActorfromActorInfo) (GameplayTags|MakeLiteralGameplayTag "(TagName=\"CombatSocket.Weapon\")")))
                      (Class|CubeActiveSkill|SpawnHitBox "Hammer" "D_Hammer_Unique" _returnvalue_3 0 0)
                      (Ability|Tasks|WaitGameplayEvent "(TagName=\"Abilities.Hammer.Unique\")" 0
                        (:EventReceived
                          (bind _returnvalue_4 (Class|CombatInterface|GetCombatSocketLocation(Message) (Ability|GetAvatarActorfromActorInfo) (GameplayTags|MakeLiteralGameplayTag "(TagName=\"CombatSocket.Weapon\")")))
                          (Class|CubeActiveSkill|SpawnHitBox "Hammer" "D_Hammer_Unique" _returnvalue_4 0 0)
                          (Ability|EndAbility))))))))))
        (:OnInterrupted
          (Utilities|FlowControl|Delay 0.5 :!label _label))
        (:OnCancelled
          (goto _label))))))