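; Gameplay ability for the Scroll Blink: teleports the avatar a fixed horizontal distance toward the point under the mouse.
; Cursor target data sets a yaw-only direction, then the avatar updates its facing through CombatInterface and plays the blink montage.
; A montage gameplay event triggers an unswept teleport, spawning Blink hitboxes at both departure and arrival points.
; The ability ends shortly afterward, or when the montage completes or is interrupted.
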(event Ability|EventActivateAbility
  (Ability|CommitAbility)
  (bind _datahandle (|TargetDataUnderMouse)
    (:ValidData
      (Variables|Default|SetTargetLocation (.Location (Collision|BreakHitResult (Ability|TargetData|GetHitResultfromTargetData _datahandle))))
      (Variables|Default|SetMoveRatation (Math|Rotator|MakeRotator 0.0 0.0 (.Yaw (Math|Rotator|BreakRotator (Math|Rotator|FindLookatRotation (Transformation|GetActorLocation (Ability|GetAvatarActorfromActorInfo)) (Variables|Default|GetTargetLocation))))))
      (Variables|Default|SetMoveLocation (+ (Math|Vector|MakeVector (.X (Math|Vector|BreakVector (* (Math|Vector|Normalize (Math|Rotator|GetRotationXVector (Variables|Default|GetMoveRatation))) 5e+02))) (.Y (Math|Vector|BreakVector (* (Math|Vector|Normalize (Math|Rotator|GetRotationXVector (Variables|Default|GetMoveRatation))) 5e+02))) 0.0) (Transformation|GetActorLocation (Ability|GetAvatarActorfromActorInfo))))
      (bind _ascombat_interface (Utilities|Casting|CastToCombatInterface (Ability|GetAvatarActorfromActorInfo)))
      (Class|CombatInterface|UpdateFacingTarget _ascombat_interface (Variables|Default|GetMoveLocation))
      (|PlayMontageandWaitProxy "FacingTarget" "/Game/Blueprints/AbilitySystem/Character/Abilities/Blink/AM_Scroll_Blink.AM_Scroll_Blink" 1.0 "None" false 0.0 0.0 false
        (:then
          (Ability|Tasks|WaitGameplayEvent "(TagName=\"Event.Montage.Scroll.Blink\")" 0 true
            (:EventReceived
              (Class|CubeActiveSkill|SpawnHitBox "Blink" "Blink" (Math|Transform|MakeTransform (Transformation|GetActorLocation (Ability|GetAvatarActorfromActorInfo)) (Variables|Default|GetMoveRatation)) false 0 0)
              (Transformation|SetActorRelativeLocation (Ability|GetAvatarActorfromActorInfo) (Variables|Default|GetMoveLocation) false true)
              (Class|CubeActiveSkill|SpawnHitBox "Blink" "Blink" (Math|Transform|MakeTransform (Transformation|GetActorLocation (Ability|GetAvatarActorfromActorInfo)) (Variables|Default|GetMoveRatation)) false 0 0)
              (Utilities|FlowControl|Delay 0.2)
              (Ability|EndAbility))))
        (:OnCompleted
          (Ability|EndAbility :!label _label))
        (:OnInterrupted
          (goto _label))
        (:OnCancelled
          (goto _label))))))