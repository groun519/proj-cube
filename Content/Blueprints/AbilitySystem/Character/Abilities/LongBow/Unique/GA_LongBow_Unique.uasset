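; Longbow unique gameplay ability that fires repeated fan-shaped volleys of arrows toward the point under the mouse.
; On activation it commits, stores the target location, builds symmetric yaw offsets, turns the avatar via CombatInterface and plays the attack montage.
; A montage gameplay event triggers timed SpawnArrows bursts, each spawning one projectile per yaw override from the actor-location socket.
; The ability ends when the montage completes, blends out or is interrupted or cancelled.
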(event Ability|EventActivateAbility
  (bind _yawoffset (Variables|Default|GetYawOffset))
  (Ability|CommitAbility)
  (bind _datahandle (|TargetDataUnderMouse)
    (:ValidData
      (Variables|Default|SetTargetLocation (.Location (Collision|BreakHitResult (Ability|TargetData|GetHitResultfromTargetData _datahandle))))
      (Utilities|Array|AppendArray (Variables|Default|GetYawOvrrides) (Utilities|Array|MakeArray (* _yawoffset -3.0) (* _yawoffset -2.0) (* _yawoffset -1.0) 0.0 _yawoffset (* _yawoffset 2.0) (* _yawoffset 3.0)))
      (bind _ascombat_interface (Utilities|Casting|CastToCombatInterface (Ability|GetAvatarActorfromActorInfo)))
      (Class|CombatInterface|UpdateFacingTarget _ascombat_interface (Variables|Default|GetTargetLocation))
      (|PlayMontageandWaitProxy "FacingTarget" "/Game/Blueprints/AbilitySystem/Character/Abilities/LongBow/Unique/AM_LongBow_Unique.AM_LongBow_Unique" 1.0 "None" true 1.0 0.0 false
        (:then
          (Ability|Tasks|WaitGameplayEvent "(TagName=\"Abilities.LongBow.Unique\")" 0
            (:EventReceived
              (CallFunction|SpawnArrows)
              (Utilities|FlowControl|Delay 0.2)
              (CallFunction|SpawnArrows)
              (Utilities|FlowControl|Delay 0.2)
              (CallFunction|SpawnArrows)
              (Utilities|FlowControl|Delay 0.2)
              (CallFunction|SpawnArrows)
              (Utilities|FlowControl|Delay 0.2)
              (CallFunction|SpawnArrows))))
        (:OnCompleted
          (Ability|EndAbility :!label _label))
        (:OnBlendOut
          (goto _label))
        (:OnInterrupted
          (goto _label))
        (:OnCancelled
          (goto _label))))))

(fn SpawnArrows
  (for _array_element (Variables|Default|GetYawOvrrides)
    (Class|CubeProjectileSkill|SpawnProjectile (Variables|Default|GetTargetLocation) (GameplayTags|MakeLiteralGameplayTag "(TagName=\"CombatSocket.ActorLocation\")") true 0.0 true _array_element 0 false 0)))