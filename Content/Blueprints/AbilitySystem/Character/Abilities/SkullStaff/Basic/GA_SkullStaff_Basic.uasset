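; Basic attack ability for the Skull Staff that fires a projectile at the target under the mouse.
; On activation it commits, turns the avatar to the target via CombatInterface and plays the attack montage.
; The montage's attack event spawns the projectile from the weapon socket.
; The ability ends when the montage finishes or shortly after spawning, as the delay follows the end-event wait's immediate output, not its received event.
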(event Ability|EventActivateAbility
  (Ability|CommitAbility)
  (bind _datahandle (|TargetDataUnderMouse)
    (:ValidData
      (Variables|Default|SetTargetLocation (.Location (Collision|BreakHitResult (Ability|TargetData|GetHitResultfromTargetData _datahandle))))
      (bind _ascombat_interface (Utilities|Casting|CastToCombatInterface (Ability|GetAvatarActorfromActorInfo)))
      (Class|CombatInterface|UpdateFacingTarget _ascombat_interface (Variables|Default|GetTargetLocation))
      (|PlayMontageandWaitProxy "FacingTarget" "/Game/Blueprints/AbilitySystem/Character/Abilities/SkullStaff/Attack/AM_SkullStaff_Bagic.AM_SkullStaff_Bagic" 1.0 "None" false 1.0 0.0 false
        (:then
          (Ability|Tasks|WaitGameplayEvent "(TagName=\"Event.Montage.SkullStaff.Attack\")" 0
            (:EventReceived
              (Class|CubeProjectileSkill|SpawnProjectile (Variables|Default|GetTargetLocation) (GameplayTags|MakeLiteralGameplayTag "(TagName=\"CombatSocket.Weapon\")") false 0.0 false 0.0 (Ability|GetAvatarActorfromActorInfo) false 0)
              (Ability|Tasks|WaitGameplayEvent "(TagName=\"Event.Montage.FireStaff.Basic.End\")" 0
                (:then
                  (Utilities|FlowControl|Delay 0.2)
                  (Ability|EndAbility))))))
        (:OnCompleted
          (Ability|EndAbility :!label _label))
        (:OnBlendOut
          (goto _label))
        (:OnInterrupted
          (goto _label))
        (:OnCancelled
          (goto _label))))))