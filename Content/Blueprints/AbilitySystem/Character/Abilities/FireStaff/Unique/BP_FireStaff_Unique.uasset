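; Fire Staff unique-ability fireball projectile that charges up, flies, and spawns a damage hitbox when it expires.
; BeginPlay caches launch velocity and staggers cast VFX and sound, head visibility with sphere collision, then smoke and shot sound.
; A Timeline, played from Tick, drives head and sphere scale and multiplies the cached velocity.
; On finish it detaches smoke, spawns the hitbox through the linked CubeActiveSkill, ends the ability and destroys itself.
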(event EventBeginPlay
  (Variables|Default|SetFirstVel (Variables|/Script/Engine.MovementComponent|GetVelocity (Variables|Default|GetProjectileMovement)))
  (Collision|SetCollisionEnabled (Variables|Default|GetSphere) "NoCollision")
  (Utilities|FlowControl|Delay 0.22)
  (bind _returnvalue (Niagara|SpawnSystematLocation "/Game/Blueprints/AbilitySystem/Character/Abilities/FireStaff/Unique/EffectAsset/NS_FireBall_Cast_Unique.NS_FireBall_Cast_Unique" (Transformation|GetWorldLocation (Variables|Default|GetSphere))))
  (Transformation|AttachComponentToComponent _returnvalue 0 "None" "KeepRelative" "KeepRelative" "KeepRelative" true)
  (Audio|PlaySound2D "/Game/Blueprints/AbilitySystem/Character/Abilities/FireStaff/Unique/AnimAsset/FireStaff_Unique_Cast.FireStaff_Unique_Cast" 4.0 1.0 0.1 0 0)
  (Utilities|FlowControl|Delay 0.4)
  (Rendering|SetVisibility (Variables|Default|GetHead) true true)
  (Collision|SetCollisionEnabled (Variables|Default|GetSphere) "QueryAndPhysics")
  (Utilities|FlowControl|Delay 0.88)
  (Rendering|SetVisibility (Variables|Default|GetSmoke) true true)
  (Audio|PlaySound2D "/Game/Blueprints/AbilitySystem/Character/Abilities/FireStaff/Unique/AnimAsset/FireStaff_Unique_Shot.FireStaff_Unique_Shot" 3.0 0.75 0.0 0 0))

(event EventTick
  (params (DeltaSeconds :type Float%20%28single-precision%29))
  (bind _linkedability (Variables|Default|GetLinkedAbility))
  (bind (_direction _scale _velovity) (Timeline|Timeline Play)
    (:Update
      (Transformation|SetRelativeScale3D (Variables|Default|GetHead) (Math|Vector|MakeVector _scale _scale _scale))
      (Variables|/Script/Engine.MovementComponent|SetVelocity (Variables|Default|GetProjectileMovement) (* (Variables|Default|GetFirstVel) _velovity)))
    (:Finished
      (Transformation|DetachFromComponent (Variables|Default|GetSmoke) "KeepRelative" "KeepRelative" "KeepRelative" true)
      (bind _ascube_active_skill (Utilities|Casting|CastToCubeActiveSkill _linkedability))
      (Class|CubeActiveSkill|SpawnHitBox _ascube_active_skill "Hit" "Hitdam" (Math|Transform|MakeTransform (Transformation|GetActorLocation)) false 0 0)
      (Ability|EndAbility _linkedability)
      (Actor|DestroyActor))))

(fn ConstructionScript)