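; Fireball projectile actor for the fire staff's basic ability, with Niagara head and smoke effects and a sphere for hit detection.
; After a short delay it appears and launches by scaling its velocity, then stops and hides shortly afterwards.
; On overlap it halts, hides the head, moves the detached smoke far away and destroys itself after a delay.
; It also traces downward, but the BP_FireArea spawn using that hit is disconnected.
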(event OnComponentBeginOverlap(Sphere)
  (params (OverlappedComponent :type Primitive%20Component%20Object%20Reference) (OtherActor :type Actor%20Object%20Reference) (OtherComp :type Primitive%20Component%20Object%20Reference) (OtherBodyIndex :type Integer) (bFromSweep :type Boolean) (SweepResult :type Hit%20Result%20Structure%20%28by%20ref%29))
  (bind _sphere (Variables|Default|GetSphere))
  (bind _projectilemovement (Variables|Default|GetProjectileMovement))
  (bind _returnvalue (Transformation|GetWorldLocation _sphere))
  (Variables|/Script/Engine.MovementComponent|SetVelocity _projectilemovement (* (Variables|/Script/Engine.MovementComponent|GetVelocity _projectilemovement) ""))
  (Transformation|DetachFromComponent (Variables|Default|GetNS_FireBall_Smoke) "KeepWorld" "KeepWorld" "KeepWorld" true)
  (Collision|SetCollisionEnabled (Variables|Default|GetSphere) "NoCollision")
  (Rendering|SetVisibility (Variables|Default|GetNS_FireBall_Head) false false)
  (bind _outhit (Collision|LineTraceByChannel _returnvalue (- _returnvalue "0.000000,0.000000,500.000000") "TraceTypeQuery2" false 0 "ForDuration"))
  (Transformation|SetWorldLocation (Variables|Default|GetNS_FireBall_Smoke) "0.000000,0.000000,-10000.000000" false true)
  (Utilities|FlowControl|Delay 1.0)
  (Actor|DestroyActor))

(event EventBeginPlay
  (bind _projectilemovement (Variables|Default|GetProjectileMovement))
  (bind _projectilemovement_2 (Variables|Default|GetProjectileMovement))
  (Utilities|FlowControl|Delay 0.2)
  (Rendering|SetVisibility (Variables|Default|GetNS_FireBall_Head) true false)
  (Variables|/Script/Engine.MovementComponent|SetVelocity _projectilemovement (* (Variables|/Script/Engine.MovementComponent|GetVelocity _projectilemovement) 3e+03))
  (Utilities|FlowControl|Delay 0.3)
  (Rendering|SetVisibility (Variables|Default|GetNS_FireBall_Head) false false)
  (Variables|/Script/Engine.MovementComponent|SetVelocity _projectilemovement_2 (* (Variables|/Script/Engine.MovementComponent|GetVelocity _projectilemovement_2) "")))

(fn ConstructionScript)