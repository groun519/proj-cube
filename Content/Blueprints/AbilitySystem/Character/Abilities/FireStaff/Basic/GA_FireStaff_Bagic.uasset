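; Gameplay ability for the fire staff's basic attack, which fires a projectile toward the point under the mouse.
; On activation it commits, gets mouse target data, turns the avatar to face the hit location via CombatInterface, and plays the attack montage.
; A montage gameplay event triggers the projectile spawn from the weapon socket.
; The ability ends when the montage completes, blends out, is interrupted or is cancelled.
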(event Ability|EventActivateAbility
  (Ability|CommitAbility)
  (bind _datahandle (|TargetDataUnderMouse)
    (:ValidData
      (Variables|Default|SetTargetLocation (.Location (Collision|BreakHitResult (Ability|TargetData|GetHitResultfromTargetData _datahandle))))
      (bind _ascombat_interface (Utilities|Casting|CastToCombatInterface (Ability|GetAvatarActorfromActorInfo)))
      (Class|CombatInterface|UpdateFacingTarget _ascombat_interface (Variables|Default|GetTargetLocation))
      (|PlayMontageandWaitProxy "FacingTarget" "/Game/Blueprints/AbilitySystem/Character/Abilities/FireStaff/Basic/AnimAsset/AM_FireStaff_Bagic.AM_FireStaff_Bagic" 1.0 "None" false 1.0 0.0 false
        (:then
          (Ability|Tasks|WaitGameplayEvent "(TagName=\"Event.Montage.FireStaff.Basic.Start\")" 0
            (:EventReceived
              (Class|CubeActiveSkill|SpawnProjectile "Projectile" "Projectile" (Variables|Default|GetTargetLocation) (GameplayTags|MakeLiteralGameplayTag "(TagName=\"CombatSocket.Weapon\")") false 0.0 false 0.0 0 false 0))))
        (:OnCompleted
          (Ability|EndAbility :!label _label))
        (:OnBlendOut
          (goto _label))
        (:OnInterrupted
          (goto _label))
        (:OnCancelled
          (goto _label))))))