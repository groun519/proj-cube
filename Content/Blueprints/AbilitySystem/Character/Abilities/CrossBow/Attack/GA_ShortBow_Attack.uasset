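; Short bow attack gameplay ability that fires a projectile at the location under the mouse.
; Target data under the mouse sets the target, which the avatar turns toward through the CombatInterface while the attack montage plays.
; A montage gameplay event spawns the projectile from the weapon socket.
; The ability ends after a short delay following the shot, or following montage interruption or cancellation.
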(event Ability|EventActivateAbility
  (bind _datahandle (|TargetDataUnderMouse)
    (:ValidData
      (Variables|Default|SetTargetLocation (.Location (Collision|BreakHitResult (Ability|TargetData|GetHitResultfromTargetData _datahandle))))
      (bind _ascombat_interface (Utilities|Casting|CastToCombatInterface (Ability|GetAvatarActorfromActorInfo)))
      (Class|CombatInterface|UpdateFacingTarget _ascombat_interface (Variables|Default|GetTargetLocation))
      (|PlayMontageandWaitProxy "FacingTarget" "/Game/Blueprints/AbilitySystem/Character/Abilities/CrossBow/Attack/AM_ShortBow_Attack.AM_ShortBow_Attack" 1.0 "None" true 1.0 0.0 false
        (:then
          (Ability|Tasks|WaitGameplayEvent "(TagName=\"Event.Montage.ShortBow.Attack\")" 0
            (:EventReceived
              (Class|CubeProjectileSkill|SpawnProjectile (Variables|Default|GetTargetLocation) (GameplayTags|MakeLiteralGameplayTag "(TagName=\"CombatSocket.Weapon\")") false 0.0))))
        (:OnInterrupted
          _)
        (:OnCancelled
          _))
      (Utilities|FlowControl|Delay 0.5)
      (Ability|EndAbility))))