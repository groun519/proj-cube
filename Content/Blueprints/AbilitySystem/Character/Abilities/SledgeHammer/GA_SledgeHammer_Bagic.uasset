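; Sledgehammer gameplay ability: a hold-to-charge attack that faces the point under the mouse and swaps in the hammer mesh during its montage.
; Chained montage events raise the charge count to three with emissive flashes, the last also locking movement and adding a looping shock cue.
; Input release or a timeout jumps to the Charged section, damages the clicked actor, applies a self effect, then restores the weapon and ends.
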(event Custom|ChargeEnd
  (Variables|Default|SetCharged true)
  (Variables|/Script/Engine.PlayerController|SetbShowMouseCursor (Variables|Default|GetOwnerPlayerController) true)
  (Pawn|Components|CharacterMovement|SetMovementMode (Variables|/Script/Engine.Character|GetCharacterMovement (Variables|Default|GetOwnerCharacter)) "MOVE_Walking" 0)
  (GameplayCue|RemoveGameplayCue "(TagName=\"GameplayCue.ShockLoop\")")
  (Ability|Animation|MontageJumptoSection "Charged")
  (Development|PrintString "Jump" true true "(R=0.057249,G=1.000000,B=0.000000,A=1.000000)")
  (Class|CubeActiveSkill|ApplyDamagebyName (Variables|Default|GetMouseHitActor) "SledgeHammer_Basic_Damage_Hitbox_1")
  (Ability|ApplyGameplayEffectToOwner "/Game/Blueprints/AbilitySystem/Character/Abilities/SledgeHammer/GE_Fuck.GE_Fuck_C")
  (Utilities|FlowControl|Delay 1.0)
  (Class|CombatInterface|ResetWeapon(Message) (Ability|GetAvatarActorfromActorInfo))
  (Ability|EndAbility))

(event Ability|EventActivateAbility
  (CallFunction|EnforceImplementsCombatInterface)
  (bind _asbp_cube_character (Utilities|Casting|CastToBP_CubeCharacter (Ability|GetAvatarActorfromActorInfo)))
  (Variables|Default|SetBPCubeCharacter _asbp_cube_character)
  ;[1 1 1] Store Mouse Data Variables
  (bind _datahandle (|TargetDataUnderMouse)
    (:ValidData
      (Class|CubeActiveSkill|StoreMouseDataInfo (Ability|TargetData|GetHitResultfromTargetData _datahandle))
      (Class|CubeActiveSkill|StoreOwnerVariables)
      (Utilities|FlowControl|Sequence
        (:then_0
          (Variables|/Script/Engine.PlayerController|SetbShowMouseCursor (Variables|Default|GetOwnerPlayerController) false)
          ;[1 1 1] Update Facing Target
          (Class|CombatInterface|UpdateFacingTarget(Message) (Ability|GetAvatarActorfromActorInfo) (Variables|Default|GetMouseHitLocation))
          (GameplayCue|ExecuteGameplayCue :GameplayCueTag "(TagName=\"GameplayCue.ShockBurst\")")
          (|PlayMontageandWaitProxy "None" (Variables|Default|GetMontage_SledgeHammer) 1.0 "None" true 1.0 0.0 false
            (:then
              (Utilities|FlowControl|Sequence
                (:then_0
                  (Class|CombatInterface|ChangeWeapon(Message) (Ability|GetAvatarActorfromActorInfo) (Variables|Default|GetWeapon) (Math|Transform|MakeTransform "0.000000,0.000000,-100.000000" "0.000000,90.000000,0.000000" "2.000000,2.000000,2.000000"))
                  (Utilities|FlowControl|Delay 1.5)
                  (if (not (Variables|Default|GetCharged))
                    (CallFunction|ChargeEnd)
                    (Development|PrintString "Charged" true true "(R=1.000000,G=0.005162,B=0.000000,A=1.000000)")))
                (:then_1
                  (Ability|Tasks|WaitGameplayEvent "(TagName=\"Event.Montage.SledgeHammer.Basic.Charge.1\")" 0 true
                    (:EventReceived
                      (Variables|Default|SetChargeCount 1)
                      (Default|EmissiveCharacter (Variables|Default|GetBPCubeCharacter) "(R=1.000000,G=0.271328,B=0.000000,A=1.000000)" 3e+03 0.3)
                      (Ability|Tasks|WaitGameplayEvent "(TagName=\"Event.Montage.SledgeHammer.Basic.Charge.2\")" 0 true
                        (:EventReceived
                          (Variables|Default|SetChargeCount 2)
                          (Default|EmissiveCharacter (Variables|Default|GetBPCubeCharacter) "(R=1.000000,G=0.271328,B=0.000000,A=1.000000)" 3e+03 0.3)
                          (Ability|Tasks|WaitGameplayEvent "(TagName=\"Event.Montage.SledgeHammer.Basic.Charge.3\")" 0 true
                            (:EventReceived
                              (Variables|Default|SetChargeCount 3)
                              (Default|EmissiveCharacter (Variables|Default|GetBPCubeCharacter) "(R=1.000000,G=0.271328,B=0.000000,A=1.000000)" 3e+03 0.3)
                              (Utilities|FlowControl|Sequence
                                (:then_1
                                  (Pawn|Components|CharacterMovement|DisableMovement (Variables|/Script/Engine.Character|GetCharacterMovement (Variables|Default|GetOwnerCharacter)))
                                  (bind _returnvalue (Class|CombatInterface|GetWeapon(Message) (Ability|GetAvatarActorfromActorInfo)))
                                  (GameplayCue|AddGameplayCueOnActor(Looping) (Ability|GetAvatarActorfromActorInfo) "(TagName=\"GameplayCue.ShockLoop\")" (Ability|GameplayCue|MakeGameplayCueParameters :SourceObject _returnvalue)))))))))))))))
        (:then_1
          (Ability|Tasks|WaitInputRelease false
            (:OnRelease
              (if (not (Variables|Default|GetCharged))
                (CallFunction|ChargeEnd)))))))))

(fn EnforceImplementsCombatInterface
  (if (not (Utilities|DoesObjectImplementInterface (Ability|GetAvatarActorfromActorInfo) "/Script/P_Cube.CombatInterface"))
    (Ability|EndAbility)))