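; Gameplay ability for the gravity staff's basic attack, firing a projectile at the location under the mouse.
; It lowers the hit point on Z, turns the avatar toward it through CombatInterface, then plays the attack montage.
; A montage gameplay event triggers the projectile spawn from the weapon socket.
; The ability ends after a short delay following the spawn, or following montage interruption or cancellation.
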(event Ability|EventActivateAbility
  (bind _datahandle (|TargetDataUnderMouse)
    (:ValidData
      (Variables|Default|SetTargetLocation (Math|Vector|MakeVector (.X (Math|Vector|BreakVector (.Location (Collision|BreakHitResult (Ability|TargetData|GetHitResultfromTargetData _datahandle))))) (.Y (Math|Vector|BreakVector (.Location (Collision|BreakHitResult (Ability|TargetData|GetHitResultfromTargetData _datahandle))))) (- (.Z (Math|Vector|BreakVector (.Location (Collision|BreakHitResult (Ability|TargetData|GetHitResultfromTargetData _datahandle))))) 3e+02)))
      (bind _ascombat_interface (Utilities|Casting|CastToCombatInterface (Ability|GetAvatarActorfromActorInfo)))
      (Class|CombatInterface|UpdateFacingTarget _ascombat_interface (Variables|Default|GetTargetLocation))
      (|PlayMontageandWaitProxy "FacingTarget" "/Game/Blueprints/AbilitySystem/Character/Abilities/GravityStaff/Basic/AM_GravityStaff_Bagic.AM_GravityStaff_Bagic" 1.0 "None" true 1.0 0.0 false
        (:then
          (Ability|Tasks|WaitGameplayEvent "(TagName=\"Event.Montage.GravityStaff.Basic\")" 0
            (:EventReceived
              (Class|CubeProjectileSkill|SpawnProjectile (Variables|Default|GetTargetLocation) (GameplayTags|MakeLiteralGameplayTag "(TagName=\"CombatSocket.Weapon\")")))))
        (:OnInterrupted
          _)
        (:OnCancelled
          _))
      (Utilities|FlowControl|Delay 0.5)
      (Ability|EndAbility))))