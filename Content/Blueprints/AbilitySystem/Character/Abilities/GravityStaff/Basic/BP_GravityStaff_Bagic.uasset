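; Projectile actor for the Gravity Staff's basic ability, launched after a short hover.
; On BeginPlay it teleports itself upward, waits briefly, then scales its ProjectileMovement velocity by a large factor to fire along the existing direction.
; Destroyed is empty, and the nodes that would reset rotation and spawn a BP_GravityArea are disconnected, so they never run.
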(event EventBeginPlay
  (bind _returnvalue (Transformation|GetActorLocation))
  (bind _projectilemovement (Variables|Default|GetProjectileMovement))
  (bind (_x _y _z) (Math|Vector|BreakVector _returnvalue))
  (Transformation|SetActorLocation (Math|Vector|MakeVector _x _y (+ _z 3e+02)) false true)
  (Utilities|FlowControl|Delay 0.7)
  (Variables|/Script/Engine.MovementComponent|SetVelocity _projectilemovement (* (Variables|/Script/Engine.MovementComponent|GetVelocity _projectilemovement) 2e+03)))

(event EventDestroyed)

(fn ConstructionScript)