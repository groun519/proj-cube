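; Gameplay ability for the World Tree's Branch basic attack, firing a projectile at the Player- or Enemy-tagged actor under the mouse.
; It commits, reads cursor target data, turns the avatar through CombatInterface and plays the attack montage.
; A montage gameplay event spawns the projectile from the weapon socket, restricted to that target and using the FireStaff_Attack damage name.
; The ability ends shortly after firing or montage end, or immediately for other targets.
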(event Ability|EventActivateAbility
  (bind _returnvalue (Ability|GetAvatarActorfromActorInfo))
  (Ability|CommitAbility)
  (bind _datahandle (|TargetDataUnderMouse)
    (:ValidData
      (Variables|Default|SetTargetLocation (.Location (Collision|BreakHitResult (Ability|TargetData|GetHitResultfromTargetData _datahandle))))
      (if (or (Actor|ActorHasTag (.HitActor (Collision|BreakHitResult (Ability|TargetData|GetHitResultfromTargetData _datahandle))) "Player") (Actor|ActorHasTag (.HitActor (Collision|BreakHitResult (Ability|TargetData|GetHitResultfromTargetData _datahandle))) "Enemy"))
        (bind _ascombat_interface (Utilities|Casting|CastToCombatInterface _returnvalue))
        (Class|CombatInterface|UpdateFacingTarget _ascombat_interface (Variables|Default|GetTargetLocation))
        (|PlayMontageandWaitProxy "FacingTarget" "/Game/Blueprints/AbilitySystem/Character/Abilities/WorldTreesBranch/Attack/AM_WTB_Attack.AM_WTB_Attack" 1.0 "None" false 1.0 0.0 true
          (:then
            (Ability|Tasks|WaitGameplayEvent "(TagName=\"Event.Montage.WorldTreesBranch.Attack\")" 0
              (:EventReceived
                (Class|CubeActiveSkill|SpawnProjectile "AttackProj" "FireStaff_Attack" (Variables|Default|GetTargetLocation) (GameplayTags|MakeLiteralGameplayTag "(TagName=\"CombatSocket.Weapon\")") false 0.0 false 0.0 _returnvalue true (.HitActor (Collision|BreakHitResult (Ability|TargetData|GetHitResultfromTargetData _datahandle))))
                (Utilities|FlowControl|Delay 0.2)
                (Ability|EndAbility))))
          (:OnCompleted
            (Utilities|FlowControl|Delay 0.2 :!label _label)
            (Ability|EndAbility))
          (:OnInterrupted
            (goto _label))
          (:OnCancelled
            (goto _label)))
        (else
          (Ability|EndAbility))))))