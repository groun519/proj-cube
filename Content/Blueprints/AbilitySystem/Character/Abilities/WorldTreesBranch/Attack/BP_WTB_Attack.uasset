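; Attack projectile for the World Tree's Branch ability that heals players near its spawn point, excluding the caster.
; On BeginPlay it scales its velocity, then uses the linked CubeActiveSkill to find nearby Player-tagged actors and spawn a player-only heal hitbox on each.
; The search sphere and a print are leftover debug output, and the homing-target logic is unconnected, so it never runs.
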(event EventBeginPlay
  (bind _projectilemovement (Variables|Default|GetProjectileMovement))
  (Variables|/Script/Engine.MovementComponent|SetVelocity _projectilemovement (* (Variables|/Script/Engine.MovementComponent|GetVelocity _projectilemovement) 3e+03))
  (bind _ascube_active_skill (Utilities|Casting|CastToCubeActiveSkill (Variables|Default|GetLinkedAbility)))
  (bind _returnvalue (Class|CubeActiveSkill|FindNearestActorsbyTag _ascube_active_skill "Player" (Transformation|GetActorLocation) 2e+03 10 true))
  (for _array_element _returnvalue
    (if (not (== (Ability|GetAvatarActorfromActorInfo _ascube_active_skill) _array_element))
      (Class|CubeActiveSkill|SpawnHitBox _ascube_active_skill "HealHitbox" "HealDamage" (Math|Transform|MakeTransform (Transformation|GetActorLocation _array_element)) true 0 0)
      (Development|PrintString "Hello"))))

(event Collision|EventActorBeginOverlap
  (params (OtherActor :type Actor%20Object%20Reference)))

(event EventTick
  (params (DeltaSeconds :type Float%20%28single-precision%29)))

(fn ConstructionScript)