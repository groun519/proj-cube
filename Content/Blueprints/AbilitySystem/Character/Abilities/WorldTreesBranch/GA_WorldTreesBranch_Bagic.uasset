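; Gameplay ability for the World Tree's Branch basic cast, which creates a heal area and fires projectiles at nearby players.
; It turns the avatar toward the cursor target, then plays a montage whose gameplay event spawns the area at the caster's feet.
; Five one-second-spaced pulses sphere-overlap for other Player-tagged actors and launch projectiles at them, with debug drawing left in.
; The ability ends when the montage finishes or breaks off.
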(event Ability|EventActivateAbility
  (bind _returnvalue (Ability|GetAvatarActorfromActorInfo))
  (bind _returnvalue_2 (Transformation|GetActorLocation _returnvalue))
  (bind (_x _y _z) (Math|Vector|BreakVector _returnvalue_2))
  (Ability|CommitAbility)
  (bind _datahandle (|TargetDataUnderMouse)
    (:ValidData
      (Variables|Default|SetTargetLocation (.Location (Collision|BreakHitResult (Ability|TargetData|GetHitResultfromTargetData _datahandle))))
      (bind _ascombat_interface (Utilities|Casting|CastToCombatInterface (Ability|GetAvatarActorfromActorInfo)))
      (Class|CombatInterface|UpdateFacingTarget _ascombat_interface (Variables|Default|GetTargetLocation))
      (|PlayMontageandWaitProxy "FacingTarget" "/Game/Blueprints/AbilitySystem/Character/Abilities/WorldTreesBranch/AM_WorldTreesBranch_Bagic.AM_WorldTreesBranch_Bagic" 1.0 "None" false 1.0 0.0 false
        (:then
          (Ability|Tasks|WaitGameplayEvent "(TagName=\"Event.Montage.WorldTreesBranch.Basic\")" 0
            (:EventReceived
              (Game|SpawnActorfromClass "/Game/Blueprints/AbilitySystem/Character/Abilities/WorldTreesBranch/BP_WorldTreesBranch_HealArea.BP_WorldTreesBranch_HealArea_C" (Math|Transform|MakeTransform (Math|Vector|MakeVector _x _y (- _z 95.0))) "AlwaysSpawn" "MultiplyWithRoot" 0 0)
              (CallFunction|FindNearPlayersandSpawnProj)
              (Utilities|FlowControl|Delay 1.0)
              (CallFunction|FindNearPlayersandSpawnProj)
              (Utilities|FlowControl|Delay 1.0)
              (CallFunction|FindNearPlayersandSpawnProj)
              (Utilities|FlowControl|Delay 1.0)
              (CallFunction|FindNearPlayersandSpawnProj)
              (Utilities|FlowControl|Delay 1.0)
              (CallFunction|FindNearPlayersandSpawnProj)
              (Utilities|FlowControl|Delay 1.0))))
        (:OnCompleted
          (Ability|EndAbility :!label _label))
        (:OnBlendOut
          (goto _label))
        (:OnInterrupted
          (goto _label))
        (:OnCancelled
          (goto _label))))))

(fn FindNearPlayers
  (params (SphereRadius :type Float%20%28double-precision%29))
  (bind _returnvalue (Ability|GetAvatarActorfromActorInfo))
  (bind _returnvalue_2 (Transformation|GetActorLocation _returnvalue))
  (Utilities|Array|AppendArray (LocalVariables|GetActorsToIgnore) (Utilities|Array|MakeArray (Ability|GetAvatarActorfromActorInfo)))
  (bind _outactors (Collision|SphereOverlapActors _returnvalue_2 SphereRadius (LocalVariables|GetObject%20Types) 0 (LocalVariables|GetActorsToIgnore)))
  (Rendering|Debug|DrawDebugSphere _returnvalue_2 SphereRadius 12 "(R=1.000000,G=1.000000,B=1.000000,A=1.000000)" 1e+01)
  (for _array_element _outactors
    (if (Actor|ActorHasTag _array_element "Player")
      (Utilities|Array|AppendArray (LocalVariables|GetNearPls) (Utilities|Array|MakeArray _array_element))))
  (return (LocalVariables|GetNearPls)))

(fn FindNearPlayersandSpawnProj
  (bind _nearplayers (CallFunction|FindNearPlayers 3.5e+02))
  (for _array_element _nearplayers
    (Utilities|IsValid _array_element
      (:Is%20Valid
        (Development|PrintString (Utilities|GetDisplayName _array_element))
        (Class|CubeActiveSkill|SpawnProjectile "None" "None" (Transformation|GetActorLocation _array_element) (GameplayTags|MakeLiteralGameplayTag "(TagName=\"CombatSocket.Weapon\")") false 0.0 false 0.0 (Ability|GetAvatarActorfromActorInfo) false _array_element)))))