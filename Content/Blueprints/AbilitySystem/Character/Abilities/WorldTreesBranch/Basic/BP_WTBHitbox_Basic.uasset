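; Short-lived hitbox actor for the basic ability of World Tree's Branch, pairing a sphere collision with a Niagara effect.
; On BeginPlay it registers the sphere through SetHitboxCollision, then plays a timeline that drives the effect's opacity and uniform scale.
; In parallel, a delay chain disables the collision halfway through its roughly one-second lifetime, then destroys the actor.
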(event EventBeginPlay
  ;[1 1 1] 1. 콜리전 컴포넌트를 하나 생성하고, 생성된 콜리전을 SetHitboxCollision 함수를 통해 등록함.
  (Class|CubeHitbox|SetHitboxCollision (Variables|Default|GetSphere))
  (Utilities|FlowControl|Sequence
    (:then_0
      (bind (_direction _scale _opacity) (Timeline|Timeline Play)
        (:Update
          (Niagara|SetNiagaraVariable(Float) (Variables|Default|GetNiagara) "Opacity" _opacity)
          (Transformation|SetRelativeScale3D (Variables|Default|GetNiagara) (Math|Vector|MakeVector _scale _scale _scale)))))
    (:then_1
      (Utilities|FlowControl|Delay 0.5)
      (Collision|SetCollisionEnabled (Variables|Default|GetSphere) "NoCollision")
      (Utilities|FlowControl|Delay 0.5)
      (Actor|DestroyActor))))

(fn ConstructionScript)