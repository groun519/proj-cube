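; Gameplay ability for the World Tree's Branch unique skill, a pulsed area heal for players.
; It faces the mouse target, plays a montage, then on its gameplay event spawns a player-only heal hitbox at the caster's feet.
; Five one-second-spaced pulses launch upward, random-yaw heal projectiles, each restricted to one other nearby player.
; The ability ends with the montage; the Enemy-filtering FindNearPlayers helper is not called here.
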(event Ability|EventActivateAbility
  (bind _returnvalue (Ability|GetAvatarActorfromActorInfo))
  (bind _returnvalue_2 (Transformation|GetActorLocation _returnvalue))
  (bind (_x _y _z) (Math|Vector|BreakVector _returnvalue_2))
  (Ability|CommitAbility)
  (bind _datahandle (|TargetDataUnderMouse)
    (:ValidData
      (Variables|Default|SetTargetLocation (.Location (Collision|BreakHitResult (Ability|TargetData|GetHitResultfromTargetData _datahandle))))
      (bind _ascombat_interface (Utilities|Casting|CastToCombatInterface (Ability|GetAvatarActorfromActorInfo)))
      (Class|CombatInterface|UpdateFacingTarget _ascombat_interface (Variables|Default|GetTargetLocation))
      (|PlayMontageandWaitProxy "FacingTarget" "/Game/Blueprints/AbilitySystem/Character/Abilities/WorldTreesBranch/Unique/Anim/AM_WorldTreesBranch_Unique.AM_WorldTreesBranch_Unique" 1.0 "None" true 1.0 0.0 false
        (:then
          (Ability|Tasks|WaitGameplayEvent "(TagName=\"Event.Montage.WorldTreesBranch.Unique\")" 0 true
            (:EventReceived
              (Class|CubeActiveSkill|SpawnHitBox "HealBox" "HealBox" (Math|Transform|MakeTransform (Math|Vector|MakeVector _x _y (- _z 95.0))) true 0 0)
              (CallFunction|FindNearPlayersandSpawnProj)
              (Utilities|FlowControl|Delay 1.0)
              (CallFunction|FindNearPlayersandSpawnProj)
              (Utilities|FlowControl|Delay 1.0)
              (CallFunction|FindNearPlayersandSpawnProj)
              (Utilities|FlowControl|Delay 1.0)
              (CallFunction|FindNearPlayersandSpawnProj)
              (Utilities|FlowControl|Delay 1.0)
              (CallFunction|FindNearPlayersandSpawnProj)
              (Utilities|FlowControl|Delay 1.0))))
        (:OnCompleted
          (Ability|EndAbility :!label _label))
        (:OnBlendOut
          (goto _label))
        (:OnInterrupted
          (goto _label))
        (:OnCancelled
          (goto _label))))))

(fn FindNearPlayers
  (params (SphereRadius :type Float%20%28double-precision%29))
  (Utilities|Array|AppendArray (LocalVariables|GetActorsToIgnore) (Utilities|Array|MakeArray (Ability|GetAvatarActorfromActorInfo)))
  (bind _outactors (Collision|SphereOverlapActors (Transformation|GetActorLocation (Ability|GetAvatarActorfromActorInfo)) SphereRadius (LocalVariables|GetObject%20Types) 0 (LocalVariables|GetActorsToIgnore)))
  (for _array_element _outactors
    (if (Actor|ActorHasTag _array_element "Enemy")
      (Utilities|Array|AppendArray (LocalVariables|GetNearPls) (Utilities|Array|MakeArray _array_element))))
  (return (LocalVariables|GetNearPls)))

(fn FindNearPlayersandSpawnProj
  (bind _returnvalue (Class|CubeActiveSkill|FindNearestActorsbyTag "Player" (Transformation|GetActorLocation (Ability|GetAvatarActorfromActorInfo)) 7e+02 100 false))
  (for _array_element _returnvalue
    (if (!= _array_element (Ability|GetAvatarActorfromActorInfo))
      (Utilities|IsValid _array_element
        (:Is%20Valid
          (Class|CubeActiveSkill|SpawnProjectile "HealProj" "HealDamage" (Transformation|GetActorLocation _array_element) (GameplayTags|MakeLiteralGameplayTag "(TagName=\"CombatSocket.Weapon\")") true 75.0 true (Math|Random|RandomFloatinRange 0.0 3.6e+02) (Ability|GetAvatarActorfromActorInfo) true _array_element))))))