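; Projectile actor for the WorldTreesBranch ability that homes in on a target.
; On BeginPlay it turns on homing in its ProjectileMovement and locks onto the root component of the actor returned by GetTargetActor.
; The sphere overlap handler is empty.
; Disconnected leftover nodes, which never run, would trace to the ground, spawn an actor at the impact point, then teleport the projectile away and destroy it after a delay.
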(event OnComponentBeginOverlap(Sphere)
  (params (OverlappedComponent :type Primitive%20Component%20Object%20Reference) (OtherActor :type Actor%20Object%20Reference) (OtherComp :type Primitive%20Component%20Object%20Reference) (OtherBodyIndex :type Integer) (bFromSweep :type Boolean) (SweepResult :type Hit%20Result%20Structure%20%28by%20ref%29)))

(event EventBeginPlay
  (bind _projectilemovement (Variables|Default|GetProjectileMovement))
  (Variables|/Script/Engine.ProjectileMovementComponent|SetbIsHomingProjectile _projectilemovement true)
  (Variables|/Script/Engine.ProjectileMovementComponent|SetHomingTargetComponent _projectilemovement (Variables|/Script/Engine.Actor|GetRootComponent (Class|CubeProjectile|GetTargetActor))))

(fn ConstructionScript)