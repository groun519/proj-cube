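; BP_RangedEnemyProjectile is a homing projectile for a ranged enemy ability.
; On BeginPlay it sets the projectile movement's homing target to the target actor's root component, or prints a red warning if that component is invalid.
; Tick spins the static mesh by per-axis rates picked at BeginPlay, though all random ranges are zero, so it currently does not rotate.
; The overlap event is empty.
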(event EventBeginPlay
  (bind _returnvalue (Math|Random|RandomFloatinRange 0.0 0.0))
  (Variables|Default|SetYawRot _returnvalue)
  (Variables|Default|SetRollRot _returnvalue)
  (Variables|Default|SetPitchRot _returnvalue)
  (bind _rootcomponent (Variables|/Script/Engine.Actor|GetRootComponent (Class|CubeHitActor|GetTargetActor))
    (:then
      (Variables|/Script/Engine.ProjectileMovementComponent|SetHomingTargetComponent (Variables|Default|GetProjectileMovement) _rootcomponent))
    (:else
      (Development|PrintString "Target in None ! ! !" true true "(R=1.000000,G=0.000000,B=0.000000,A=1.000000)"))))

(event Collision|EventActorBeginOverlap
  (params (OtherActor :type Actor%20Object%20Reference)))

(event EventTick
  (params (DeltaSeconds :type Float%20%28single-precision%29))
  (Transformation|AddLocalRotation (Variables|Default|GetStaticMesh) (Math|Rotator|MakeRotator (* DeltaSeconds (Variables|Default|GetRollRot)) (* DeltaSeconds (Variables|Default|GetPitchRot)) (* DeltaSeconds (Variables|Default|GetYawRot))) false false))

(fn ConstructionScript)