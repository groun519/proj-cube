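; Enemy summon gameplay ability that spawns random minions at shuffled spawn locations around a montage cue.
; On activation it plays a ground Niagara effect at every location and starts the summon montage, then waits for the Montage.Attack.1 event.
; A delayed loop then spreads spawns over about a second, facing minions away from the summoner, before ending.
; Spawns and deaths update the summoner's minion count, with deaths also decrementing the spawn index.
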(event Custom|OnDestroyed_Event
  (params (DestroyedActor :type Actor%20Object%20Reference))
  (Class|CombatInterface|IncremenetMinionCount(Message) (Ability|GetAvatarActorfromActorInfo) -1)
  (Math|Integer|DecrementInt (Variables|Default|GetSpawnLocationIndex)))

(event Ability|EventActivateAbility
  (bind _returnvalue (Class|CubeSummonAbility|GetSpawnLocations))
  (bind _output_get (Variables|Default|SetSpawnLocations _returnvalue))
  (Utilities|Array|Shuffle _output_get)
  (for _array_element _output_get
    (Niagara|SpawnSystematLocation "/Game/Assets/EffectAsset/GAS_Aura_Effects/Combat/NS_GroundSummon.NS_GroundSummon" _array_element))
  (|PlayMontageandWaitProxy "None" "/Game/Blueprints/AbilitySystem/Enemies/Abilities/AM_Summon.AM_Summon" 1.0 "None" false 1.0 0.0 false
    (:then
      (Ability|Tasks|WaitGameplayEvent "(TagName=\"Montage.Attack.1\")" 0 true
        (:EventReceived
          (if (< (Variables|Default|GetSpawnLocationIndex) (Utilities|Array|Length (Variables|Default|GetSpawnLocations))) :!label _label
            (Rendering|Debug|DrawDebugSphere (Utilities|Array|Get(acopy) (Variables|Default|GetSpawnLocations) (Variables|Default|GetSpawnLocationIndex)) 25.0 12 "(R=1.000000,G=0.000000,B=0.000000,A=1.000000)" 1e+01)
            (bind _returnvalue_2 (Game|SpawnActorfromClass (Class|CubeSummonAbility|GetRandomMinionClass) (Math|Transform|MakeTransform (+ (Utilities|Array|Get(acopy) (Variables|Default|GetSpawnLocations) (Variables|Default|GetSpawnLocationIndex)) "0.000000,0.000000,90.000000") (Math|Rotator|FindLookatRotation (Transformation|GetActorLocation (Ability|GetAvatarActorfromActorInfo)) (+ (Utilities|Array|Get(acopy) (Variables|Default|GetSpawnLocations) (Variables|Default|GetSpawnLocationIndex)) "0.000000,0.000000,90.000000")) "1.000000,1.000000,1.000000") "AlwaysSpawn" "MultiplyWithRoot" 0 0))
            (Game|AssignOnDestroyed _returnvalue_2 (delegate Custom|OnDestroyed_Event))
            (Pawn|SpawnDefaultController _returnvalue_2)
            (Class|CombatInterface|IncremenetMinionCount(Message) (Ability|GetAvatarActorfromActorInfo) 1)
            (Math|Integer|IncrementInt (Variables|Default|GetSpawnLocationIndex)
              (:%20%20
                (Utilities|FlowControl|Delay (/ 1.0 (Math|Conversions|ToFloat(Integer) (Utilities|Array|Length (Variables|Default|GetSpawnLocations)))))
                (goto _label)))
            (else
              (Ability|EndAbility))))))))