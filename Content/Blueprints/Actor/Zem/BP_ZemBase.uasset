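; Base actor for Zem objects, which spins continuously and reacts when the player enters or leaves its sphere.
; Tick accumulates scaled delta time and applies it as the actor's yaw.
; Sphere begin and end overlaps filter on the "Player" tag, then pass the actor to OnOverlap and OnEndOverlap, whose logic is not defined in these graphs.
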(event OnComponentBeginOverlap(Sphere)
  (params (OverlappedComponent :type Primitive%20Component%20Object%20Reference) (OtherActor :type Actor%20Object%20Reference) (OtherComp :type Primitive%20Component%20Object%20Reference) (OtherBodyIndex :type Integer) (bFromSweep :type Boolean) (SweepResult :type Hit%20Result%20Structure%20%28by%20ref%29))
  (if (Actor|ActorHasTag OtherActor "Player")
    (Class|CubeEffectActor|OnOverlap OtherActor)))

(event OnComponentEndOverlap(Sphere)
  (params (OverlappedComponent :type Primitive%20Component%20Object%20Reference) (OtherActor :type Actor%20Object%20Reference) (OtherComp :type Primitive%20Component%20Object%20Reference) (OtherBodyIndex :type Integer))
  (if (Actor|ActorHasTag OtherActor "Player")
    (Class|CubeEffectActor|OnEndOverlap OtherActor)))

(event EventBeginPlay)

(event Collision|EventActorBeginOverlap
  (params (OtherActor :type Actor%20Object%20Reference)))

(event EventTick
  (params (DeltaSeconds :type Float%20%28single-precision%29))
  (Variables|Default|SetTime (+ (Variables|Default|GetTime) (* DeltaSeconds 2e+01)))
  (Transformation|SetActorRotation (Math|Rotator|MakeRotator 0.0 0.0 (Variables|Default|GetTime))))

(fn ConstructionScript)