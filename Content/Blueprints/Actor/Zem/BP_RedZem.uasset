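; BP_RedZem is the red Zem actor, a child Blueprint that handles its own delayed reveal when spawned.
; After the parent BeginPlay and a short random delay, it activates its Niagara effect, shows the Zem component and enables overlap events on its Sphere.
; It then plays a drop sound at its location with a randomized pitch.
; It adds no overlap, tick or construction logic of its own.
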(event EventBeginPlay
  (|CallParentFunction)
  (Utilities|FlowControl|Delay (Math|Random|RandomFloatinRange 0.2 0.8))
  (Components|Activation|Activate (Variables|Default|GetNiagara) true)
  (Rendering|SetVisibility (Variables|Default|GetZem) true false)
  (Variables|/Script/Engine.PrimitiveComponent|SetbGenerateOverlapEvents (Variables|Default|GetSphere) true)
  (Variables|Default|SetRandPitch (Math|Float|Max(Float) (/ (Math|Conversions|ToFloat(Integer) (Math|Random|RandomIntegerinRange 0 8)) 2.0) 0.01))
  (Audio|PlaySoundatLocation (Variables|Default|GetDropSounds) (Transformation|GetActorLocation) "0, 0, 0" 0.75 (Variables|Default|GetRandPitch) 0.0 0 0 0 0))

(event Collision|EventActorBeginOverlap
  (params (OtherActor :type Actor%20Object%20Reference))
  (|CallParentFunction OtherActor) ; This node is disabled and will not be called.\nDrag off pins to build functionality.
)

(event EventTick
  (params (DeltaSeconds :type Float%20%28single-precision%29))
  (|CallParentFunction DeltaSeconds) ; This node is disabled and will not be called.\nDrag off pins to build functionality.
)

(fn ConstructionScript
  (|CallParentFunction))