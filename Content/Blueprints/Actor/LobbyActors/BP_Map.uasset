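; BP_Map is a lobby map actor that displays connected versus maximum players and triggers travel when enough players are ready.
; The server updates the text every Tick, with OnRep_LobbyText updating clients, and calls the game mode's GoTravel when ReadyPlayers equals a hard-coded four.
; Player-tagged overlaps with Range increment ReadyPlayers, with no end-overlap decrement.
; SetMat toggles a mesh's OnOff material parameter and adjusts the count, but has no caller here.
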(event OnComponentBeginOverlap(Range)
  (params (OverlappedComponent :type Primitive%20Component%20Object%20Reference) (OtherActor :type Actor%20Object%20Reference) (OtherComp :type Primitive%20Component%20Object%20Reference) (OtherBodyIndex :type Integer) (bFromSweep :type Boolean) (SweepResult :type Hit%20Result%20Structure%20%28by%20ref%29))
  (if (Actor|ActorHasTag OtherActor "Player")
    (Variables|Default|SetReadyPlayers (+ (Variables|Default|GetReadyPlayers) 1))))

(event Custom|CustomEvent
  (params (Text :type Text))
  (Rendering|Components|TextRender|SetText (Variables|Default|Get_Text) Text))

(event EventTick
  (params (DeltaSeconds :type Float%20%28single-precision%29))
  (Networking|SwitchHasAuthority
    (:Authority
      (Utilities|FlowControl|Sequence
        (:then_0
          (bind _asbp_lobby_game_mode (Utilities|Casting|CastToBP_LobbyGameMode (Game|GetGameMode)))
          (Variables|Default|SetLobbyText (Utilities|Text|ToText(String) (Utilities|String|Append (Utilities|String|ToString(Integer) (Utilities|Array|Length (Variables|/Script/Engine.GameStateBase|GetPlayerArray (Game|GetGameState)))) " / " (Utilities|String|ToString(Integer) (Variables|/Script/P_Cube.LobbyGameMode|GetMaxTravelPlayers _asbp_lobby_game_mode)))))
          (if (== (Variables|Default|GetReadyPlayers) 4)
            (Class|LobbyGameMode|GoTravel _asbp_lobby_game_mode 4)))
        (:then_1
          (CallFunction|CustomEvent (Variables|Default|GetLobbyText)))))))

(fn ConstructionScript)

(fn SetMat
  (params (OnLight :type Boolean) (Mesh :type Static%20Mesh%20Component%20Object%20Reference))
  (if OnLight
    (LocalVariables|SetValue 0.0)
    (Rendering|Material|SetScalarParameterValueonMaterials Mesh "OnOff" 1.0)
    (Variables|Default|SetReadyPlayers (+ (Variables|Default|GetReadyPlayers) 1))
    (else
      (LocalVariables|SetValue 0.0)
      (Rendering|Material|SetScalarParameterValueonMaterials Mesh "OnOff" 0.0)
      (Variables|Default|SetReadyPlayers (+ (Variables|Default|GetReadyPlayers) -1)))))

(fn OnRepReadyPlayers)

(fn OnRepLobbyText
  (Rendering|Components|TextRender|SetText (Variables|Default|Get_Text) (Variables|Default|GetLobbyText)))